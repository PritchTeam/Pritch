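; AI debug actor that visualizes extreme-close, too-close and too-far distance thresholds as three translucent colored spheres.
; The construction script gives each sphere a dynamic instance of a transparent debug material with its own color and opacity (red, orange, green).
; SetRadiusSizes resets all spheres to the default scale, then scales each by the radius passed in.
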(event `SetRadiusSizes`
  (params (ExtremeCloseRadius :type "Float (double-precision)") (TooCloseRadius :type "Float (double-precision)") (TooFarRadius :type "Float (double-precision)"))
  (`|ExecutionSequence`
    (:`then_0`
      ;[1 1 1] ResetSize
      (`SceneComponent.SetWorldScale3D` (`self.ExtremeClose`) (`self.DefaultSphereScale`))
      (`SceneComponent.SetWorldScale3D` (`self.TooClose`) (`self.DefaultSphereScale`))
      (`SceneComponent.SetWorldScale3D` (`self.TooFar`) (`self.DefaultSphereScale`)))
    (:`then_1`
      (`SceneComponent.SetWorldScale3D` (`self.ExtremeClose`) (* (`self.DefaultSphereScale`) ExtremeCloseRadius)))
    (:`then_2`
      (`SceneComponent.SetWorldScale3D` (`self.TooClose`) (* (`self.DefaultSphereScale`) TooCloseRadius)))
    (:`then_3`
      (`SceneComponent.SetWorldScale3D` (`self.TooFar`) (* (`self.DefaultSphereScale`) TooFarRadius)))))

(fn `UserConstructionScript`
  (`|ExecutionSequence`
    (:`then_0`
      (bind _returnvalue (`PrimitiveComponent.CreateDynamicMaterialInstance` (`self.ExtremeClose`) 0 "/Game/0000_Pritch/04_Materials/01_Parent_Materials/DebugMaterials/Transparent_DebugMAT.Transparent_DebugMAT" "None"))
      (`MaterialInstanceDynamic.SetScalarParameterValue` _returnvalue "Transparency" 0.3)
      (`MaterialInstanceDynamic.SetVectorParameterValue` _returnvalue "Color" (struct :`R` 1.0 :`B` 0.054821 :`A` 1.0)))
    (:`then_1`
      (bind _returnvalue_2 (`PrimitiveComponent.CreateDynamicMaterialInstance` (`self.TooClose`) 0 "/Game/0000_Pritch/04_Materials/01_Parent_Materials/DebugMaterials/Transparent_DebugMAT.Transparent_DebugMAT" "None"))
      (`MaterialInstanceDynamic.SetScalarParameterValue` _returnvalue_2 "Transparency" 0.2)
      (`MaterialInstanceDynamic.SetVectorParameterValue` _returnvalue_2 "Color" (struct :`R` 1.0 :`G` 0.366374 :`A` 1.0)))
    (:`then_2`
      (bind _returnvalue_3 (`PrimitiveComponent.CreateDynamicMaterialInstance` (`self.TooFar`) 0 "/Game/0000_Pritch/04_Materials/01_Parent_Materials/DebugMaterials/Transparent_DebugMAT.Transparent_DebugMAT" "None"))
      (`MaterialInstanceDynamic.SetScalarParameterValue` _returnvalue_3 "Transparency" 0.2)
      (`MaterialInstanceDynamic.SetVectorParameterValue` _returnvalue_3 "Color" (struct :`R` 0.18035 :`G` 1.0 :`A` 1.0)))))