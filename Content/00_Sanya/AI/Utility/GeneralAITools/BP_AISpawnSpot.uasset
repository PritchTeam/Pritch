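; AI spawn spot actor that spawns BP_BaseShooterNPC enemies at its location and initializes their setup and blackboard info.
; BeginPlay builds its spawn list from either a handpicked array or shuffled multiclass wave data.
; Events spawn the whole list with delays, one entry per call, or a class passed by a spawner.
; The construction script tints a debug sphere to match its linked spawner, clearing links the spawner doesn't list.
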(event `self.ReceiveBeginPlay`
  ;[1 1 1] SpawnArraySetup
  (`|ExecutionSequence`
    (:`then_0`
      (if (`self.UseHandpickedArray`)
        (`KismetArrayLibrary.Array_Clear` (`self.DynamicSpawnContents`))
        (for _array_element (`self.HandpickedArray`)
          (`KismetArrayLibrary.Array_Add` (`self.DynamicSpawnContents`) _array_element))
        (else
          (for _array_element_2 (`.MulticlassWave_10_6042BA8A4D1E1F4D56CDCB89097CCB95` (break `/Game/00_Sanya/AI/Utility/Structs/S_MulticlassEnemyWave` (`self.InstantSpawnContents`)))
            (bind (_enemyclass _numberofenemies) (break `/Game/00_Sanya/AI/Utility/Structs/S_EnemyWave` _array_element_2))
            (for _ (range 1 (+ _numberofenemies 1))
              (`KismetArrayLibrary.Array_Add` (`self.DynamicSpawnContents`) _enemyclass)))
          (`KismetArrayLibrary.Array_Shuffle` (`self.DynamicSpawnContents`)))))
    (:`then_1`
      (set `self.Empty` (== (`KismetArrayLibrary.Array_Length` (`self.DynamicSpawnContents`)) 0)))
    (:`then_2`
      (if (== (`KismetArrayLibrary.Array_Length` (`self.AvailableClasses`)) 0)
        (set `self.HasSpawnLimits` false)
        (else
          (set `self.HasSpawnLimits` true))))))

(event `SpawnFromSelf`
  (bind _returnvalue (`KismetArrayLibrary.Array_Length` (`self.DynamicSpawnContents`)))
  ;[1 1 1] Instant Spawn of All Enemies From This Spot's Array
  (if (>= _returnvalue 0)
    (if (not (`self.SpawningNow`))
      (set `self.SpawningNow` true)
      (set `self.ActorsLeftToSpawn` _returnvalue)
      (bind _returnvalue_2 (`|SpawnActorFromClass` (`|GetArrayItem` (`self.DynamicSpawnContents`) (`self.CurrentIndexInstant`)) (`KismetMathLibrary.Conv_VectorToTransform` (`self.K2_GetActorLocation`)) "AdjustIfPossibleButAlwaysSpawn" "OverrideRootScale" null null :!label _label))
      (bind _asbp_base_shooter_npc (cast `/Game/00_Sanya/AI/NPCCharacters/BaseNPC/BP_BaseShooterNPC` _returnvalue_2))
      (`/Game/00_Sanya/AI/NPCCharacters/BaseNPC/BP_BaseShooterNPC.InitialSetupExternal` _asbp_base_shooter_npc)
      (`/Game/00_Sanya/AI/NPCCharacters/BaseNPC/BP_BaseShooterNPC.PassInfoToBB` _asbp_base_shooter_npc)
      (`KismetSystemLibrary.Delay` (`self.InstantSpawnDelay`))
      (bind _output_get (set `self.ActorsLeftToSpawn` (- (`self.ActorsLeftToSpawn`) 1)))
      (if (> _output_get 0)
        (set `self.CurrentIndexInstant` (+ (`self.CurrentIndexInstant`) 1))
        (goto _label)
        (else
          (set `self.SpawningNow` false))))))

(event `SpawnSingleFromLocalArray`
  ;[1 1 1] SpawnSingleFromLocalArray
  (if (not (`self.Empty`))
    (bind _returnvalue (`|SpawnActorFromClass` (`|GetArrayItem` (`self.DynamicSpawnContents`) (`self.CurrentIndexContinuous`)) (`KismetMathLibrary.Conv_VectorToTransform` (`self.K2_GetActorLocation`)) "AdjustIfPossibleButAlwaysSpawn" "OverrideRootScale" null null))
    (bind _asbp_base_shooter_npc (cast `/Game/00_Sanya/AI/NPCCharacters/BaseNPC/BP_BaseShooterNPC` _returnvalue))
    (`/Game/00_Sanya/AI/NPCCharacters/BaseNPC/BP_BaseShooterNPC.InitialSetupExternal` _asbp_base_shooter_npc)
    (`/Game/00_Sanya/AI/NPCCharacters/BaseNPC/BP_BaseShooterNPC.PassInfoToBB` _asbp_base_shooter_npc)
    (bind _output_get (set `self.CurrentIndexContinuous` (+ (`self.CurrentIndexContinuous`) 1)))
    (if (> _output_get (`KismetArrayLibrary.Array_LastIndex` (`self.DynamicSpawnContents`)))
      (set `self.Empty` true))))

(event `SpawnFromSpawner`
  (params (Enemies :type "Actor Class Reference"))
  ;[1 1 1] Spawn from spawner
  (if (not (`self.Empty`))
    (bind _returnvalue (`|SpawnActorFromClass` Enemies (`KismetMathLibrary.Conv_VectorToTransform` (`self.K2_GetActorLocation`)) "AdjustIfPossibleButAlwaysSpawn" "OverrideRootScale" null null))
    (bind _asbp_base_shooter_npc (cast `/Game/00_Sanya/AI/NPCCharacters/BaseNPC/BP_BaseShooterNPC` _returnvalue))
    (`/Game/00_Sanya/AI/NPCCharacters/BaseNPC/BP_BaseShooterNPC.InitialSetupExternal` _asbp_base_shooter_npc)
    (`/Game/00_Sanya/AI/NPCCharacters/BaseNPC/BP_BaseShooterNPC.PassInfoToBB` _asbp_base_shooter_npc)))

(event `ClearIndexes`
  ;[1 1 1] Clears Spot Data - use when transferring ownership to another Spawner
  (set `self.CurrentIndexInstant` 0)
  (set `self.CurrentIndexContinuous` 0)
  (set `self.CurrentIndexFromSpawner` 0)
  (set `self.ActorsLeftToSpawn` 0))

(fn `UserConstructionScript`
  (`/Engine/EditorBlueprintResources/StandardMacros.IsValid` (`self.LinkedToSpawner`)
    (:`Is Valid`
      (if (`KismetArrayLibrary.Array_Contains` (`/Game/00_Sanya/AI/Utility/GeneralAITools/BP_AISpawner.SpawnSpots` (`self.LinkedToSpawner`)) self)
        (bind _returnvalue (`PrimitiveComponent.CreateDynamicMaterialInstance` (`self.Sphere`) 0 "/Game/0000_Pritch/04_Materials/01_Parent_Materials/DebugMaterials/M_Unlit_Debug.M_Unlit_Debug" "None"))
        (`MaterialInstanceDynamic.SetVectorParameterValue` _returnvalue "Color" (`/Game/00_Sanya/AI/Utility/GeneralAITools/BP_AISpawner.DisplayClolor` (`self.LinkedToSpawner`)))
        (else
          (bind _returnvalue_2 (`PrimitiveComponent.CreateDynamicMaterialInstance` (`self.Sphere`) 0 "/Game/0000_Pritch/04_Materials/01_Parent_Materials/DebugMaterials/M_Unlit_Debug.M_Unlit_Debug" "None"))
          (`MaterialInstanceDynamic.SetVectorParameterValue` _returnvalue_2 "Color" (`self.DisplayColor`))
          (set `self.LinkedToSpawner` (`self.NoSpot`)))))
    (:`Is Not Valid`
      (bind _returnvalue_3 (`PrimitiveComponent.CreateDynamicMaterialInstance` (`self.Sphere`) 0 "/Game/0000_Pritch/04_Materials/01_Parent_Materials/DebugMaterials/M_Unlit_Debug.M_Unlit_Debug" "None"))
      (`MaterialInstanceDynamic.SetVectorParameterValue` _returnvalue_3 "Color" (`self.DisplayColor`)))))