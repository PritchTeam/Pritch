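; AI spawner that activates once when the main character enters its radius or box trigger, then spawns enemies through linked spawn spots.
; Enemies come from a handpicked array, a shuffled multiclass wave, or each spot's own contents.
; Instant mode spawns across all spots.
; Continuous mode runs an EQS query around the player, takes the first available linked spot, and spawns delayed, random-sized waves until contents run out.
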(event `self.ReceiveBeginPlay`
  ;[1 1 1] Setup
  (`|ExecutionSequence`
    (:`then_0`
      ;;[0.5729 1 0.1458] Collision Setup
      (switch `/Game/00_Sanya/AI/Utility/GeneralAITools/SpawnerEnums/E_SpawnerActivationType` (`self.ActivationType`)
        (:`NewEnumerator0`
          (`PrimitiveComponent.SetCollisionResponseToAllChannels` (`self.RadiusTrigger`) "ECR_Ignore")
          (`PrimitiveComponent.SetCollisionResponseToChannel` (`self.RadiusTrigger`) "ECC_Pawn" "ECR_Overlap"))
        (:`NewEnumerator1`
          (`PrimitiveComponent.SetCollisionResponseToAllChannels` (`self.BoxTrigger`) "ECR_Ignore")
          (`PrimitiveComponent.SetCollisionResponseToChannel` (`self.BoxTrigger`) "ECC_Pawn" "ECR_Overlap"))))
    (:`then_1`
      ;;[1 0.7349 0.1367] SpawnerArraySetup
      (if (`self.UseHandpickedArray`)
        (`KismetArrayLibrary.Array_Clear` (`self.DynamicSpawnContents`))
        (for _array_element (`self.HandpickedArray`)
          (`KismetArrayLibrary.Array_Add` (`self.DynamicSpawnContents`) _array_element))
        (else
          (for _array_element_2 (`.MulticlassWave_10_6042BA8A4D1E1F4D56CDCB89097CCB95` (break `/Game/00_Sanya/AI/Utility/Structs/S_MulticlassEnemyWave` (`self.EnemiesToSpawn`)))
            (bind (_enemyclass _numberofenemies) (break `/Game/00_Sanya/AI/Utility/Structs/S_EnemyWave` _array_element_2))
            (for _ (range 1 (+ _numberofenemies 1))
              (`KismetArrayLibrary.Array_Add` (`self.DynamicSpawnContents`) _enemyclass)))
          (`KismetArrayLibrary.Array_Shuffle` (`self.DynamicSpawnContents`)))))
    (:`then_2`
      (set `self.Player` (`GameplayStatics.GetPlayerCharacter` 0))
      (if (`self.InheritSpots`)
        (set `self.SpawnSpots` (`/Game/00_Sanya/AI/Utility/GeneralAITools/BP_AISpawner.SpawnSpots` (`self.PreviousSpawner`)))))))

(event `self.RadiusTrigger.OnComponentBeginOverlap`
  (params (OverlappedComponent :type "PrimitiveComponent Object Reference") (OtherActor :type "Actor Object Reference") (OtherComp :type "PrimitiveComponent Object Reference") (OtherBodyIndex :type Integer) (bFromSweep :type Boolean) (SweepResult :type "HitResult Structure (by ref)"))
  ;[1 1 1] SpawnerActivation
  (cast `/Game/00_Lin/Character/BP_MainCharacter` OtherActor)
  (`/Engine/EditorBlueprintResources/StandardMacros.DoOnce` false
    (:`Completed`
      (`PrimitiveComponent.SetCollisionResponseToChannel` (`self.RadiusTrigger`) "ECC_Pawn" "ECR_Ignore")
      (`KismetSystemLibrary.Delay` (`self.StartDelay`))
      (`self.Activation`))))

(event `self.BoxTrigger.OnComponentBeginOverlap`
  (params (OverlappedComponent :type "PrimitiveComponent Object Reference") (OtherActor :type "Actor Object Reference") (OtherComp :type "PrimitiveComponent Object Reference") (OtherBodyIndex :type Integer) (bFromSweep :type Boolean) (SweepResult :type "HitResult Structure (by ref)"))
  ;[1 1 1] SpawnerActivation
  (cast `/Game/00_Lin/Character/BP_MainCharacter` OtherActor)
  (`/Engine/EditorBlueprintResources/StandardMacros.DoOnce` false
    (:`Completed`
      (`PrimitiveComponent.SetCollisionResponseToChannel` (`self.BoxTrigger`) "ECC_Pawn" "ECR_Ignore")
      (`KismetSystemLibrary.Delay` (`self.StartDelay`))
      (`self.Activation`))))

(event `Activation`
  (bind _output (`|GetArrayItem` (`self.DynamicSpawnContents`) (`self.CurrentSpawnerArrayIndex`)))
  (`KismetSystemLibrary.PrintString` "SPAWNER ACTIVE" true false)
  (`KismetSystemLibrary.Delay` (`self.StartDelay`))
  (switch `/Game/00_Sanya/AI/Utility/GeneralAITools/SpawnerEnums/E_SpawnStyle` (`self.SpawnStyle`)
    (:`NewEnumerator0`
      ;[1 1 1] InstantSpawn
      (switch `/Game/00_Sanya/AI/Utility/GeneralAITools/SpawnerEnums/E_SpawnSource` (`self.EnemySource`)
        (:`NewEnumerator0`
          (for _array_element (`self.SpawnSpots`) :!label _label
            (if (`KismetSystemLibrary.IsValidClass` _output)
              (`/Game/00_Sanya/AI/Utility/GeneralAITools/BP_AISpawnSpot.SpawnFromSpawner` _array_element _output (`KismetMathLibrary.RandomFloatInRange` 0.0 0.5))
              (set `self.CurrentSpawnerArrayIndex` (+ (`self.CurrentSpawnerArrayIndex`) 1))))
          (bind _spawnfinished (`self.CheckSpawnContents`))
          (if (not _spawnfinished)
            (`KismetSystemLibrary.Delay` 0.5)
            (goto _label)))
        (:`NewEnumerator1`
          (for _array_element_2 (`self.SpawnSpots`)
            (`/Game/00_Sanya/AI/Utility/GeneralAITools/BP_AISpawnSpot.SpawnFromSelf` _array_element_2)))))
    (:`NewEnumerator1`
      ;[1 1 1] ContinuousSpawn
      (`|ExecutionSequence`
        (:`then_0`
          ;;[0.3889 1 0.3093] Mark available spots
          (for _array_element_3 (`self.SpawnSpots`)
            (set `/Game/00_Sanya/AI/Utility/GeneralAITools/BP_AISpawnSpot.AvailableForContSpawn` true _array_element_3)))
        (:`then_1`
          (`self.FindSpot`))))))

(event `FindSpot`
  ;[1 1 1] Find Continuous spawn spot
  (bind _returnvalue (`EnvQueryManager.RunEQSQuery` "/Game/00_Sanya/AI/Utility/EQS/ReadyEQS/BestSpawnSpot_EQS.BestSpawnSpot_EQS" (`GameplayStatics.GetPlayerCharacter` 0) "AllMatching"))
  (add `EnvQueryInstanceBlueprintWrapper.OnQueryFinishedEvent` _returnvalue (delegate `QueryFinished`)))

(event `QueryFinished`
  (params (QueryInstance :type "EnvQueryInstanceBlueprintWrapper Object Reference") (QueryStatus :type "EEnvQueryStatus Enum" :default "Processing"))
  ;[1 1 1] Find Continuous spawn spot
  (bind (_outspot _spotfound) (`self.SelectSpawnSpot` QueryInstance))
  (if _spotfound
    (`KismetSystemLibrary.PrintString` (`KismetSystemLibrary.GetDisplayName` (`self.MatchingSpot`)))
    (switch `/Game/00_Sanya/AI/Utility/GeneralAITools/SpawnerEnums/E_SpawnSource` (`self.EnemySource`)
      (:`NewEnumerator0`
        (`self.ForLoopWithDelay` 1 (`KismetMathLibrary.RandomIntegerInRange` (`self.EnemyInWaveMin`) (`self.EnemyInWaveMax`)) (`self.DelayBetweenEnemies`)
          (:`LoopBody`
            (`/Game/00_Sanya/AI/Utility/GeneralAITools/BP_AISpawnSpot.SpawnFromSpawner` (`self.MatchingSpot`) (`|GetArrayItem` (`self.DynamicSpawnContents`) (`self.CurrentSpawnerArrayIndex`)) 0.0)
            (set `self.CurrentSpawnerArrayIndex` (+ (`self.CurrentSpawnerArrayIndex`) 1)))
          (:`Completed`
            (bind _spawnfinished (`self.CheckSpawnContents`))
            (if (not _spawnfinished)
              (`KismetSystemLibrary.Delay` (`self.DelayBetweenWaves`))
              (`self.FindSpot`)))))
      (:`NewEnumerator1`
        (`self.ForLoopWithDelay` 1 (`KismetMathLibrary.RandomIntegerInRange` (`self.EnemyInWaveMin`) (`self.EnemyInWaveMax`)) (`self.DelayBetweenEnemies`)
          (:`LoopBody`
            (`/Game/00_Sanya/AI/Utility/GeneralAITools/BP_AISpawnSpot.SpawnSingleFromLocalArray` (`self.MatchingSpot`)))
          (:`Completed`
            (bind _spawnfinished_2 (`self.CheckSpawnContents`))
            (if (not _spawnfinished_2)
              (`KismetSystemLibrary.Delay` (`self.DelayBetweenWaves`))
              (`self.FindSpot`))))))
    (else
      (`KismetSystemLibrary.PrintString` "NO SPOT")
      (`KismetSystemLibrary.Delay` 0.2)
      (`self.FindSpot`))))

(fn `CheckSpawnContents`
  (returns (SpawnFinished :type Boolean))
  (locals (NotEmptyDetected :type Boolean))
  (switch `/Game/00_Sanya/AI/Utility/GeneralAITools/SpawnerEnums/E_SpawnSource` (`self.EnemySource`)
    (:`NewEnumerator0`
      (if (> (`self.CurrentSpawnerArrayIndex`) (`KismetArrayLibrary.Array_LastIndex` (`self.DynamicSpawnContents`)))
        (return true)
        (else
          (return false))))
    (:`NewEnumerator1`
      (for _array_element (`self.SpawnSpots`)
        (if (not (`/Game/00_Sanya/AI/Utility/GeneralAITools/BP_AISpawnSpot.Empty` _array_element))
          (set `local.NotEmptyDetected` true)
          (break)))
      (if (`local.NotEmptyDetected`)
        (return false)
        (else
          (return true))))))

(fn `ResetRadiusSize`
  (params (NewRadius :type "Float (double-precision)"))
  (`SceneComponent.SetWorldScale3D` (`self.RadiusTrigger`) (`KismetMathLibrary.Conv_DoubleToVector` (`self.ActivationRadius`)))
  (`SceneComponent.SetWorldScale3D` (`self.DebugSphere`) (* (`SceneComponent.K2_GetComponentScale` (`self.DebugSphere`)) (`self.ActivationRadius`)))
  (bind _returnvalue (`PrimitiveComponent.CreateDynamicMaterialInstance` (`self.DebugSphere`) 0 "/Game/0000_Pritch/04_Materials/01_Parent_Materials/DebugMaterials/Transparent_DebugMAT.Transparent_DebugMAT" "None"))
  (`MaterialInstanceDynamic.SetVectorParameterValue` _returnvalue "Color" (`self.DisplayClolor`)))

(fn `SelectSpawnSpot`
  (params (QueryResults :type "EnvQueryInstanceBlueprintWrapper Object Reference"))
  (returns (OutSpot :type "/Game/00_Sanya/AI/Utility/GeneralAITools/BP_AISpawnSpot Object Reference") (SpotFound :type Boolean))
  (locals (RawSpots :type "Array of /Game/00_Sanya/AI/Utility/GeneralAITools/BP_AISpawnSpot Object Reference") (AvailableSpots :type "Array of /Game/00_Sanya/AI/Utility/GeneralAITools/BP_AISpawnSpot Object Reference"))
  (bind _output (`|GetArrayItem` (`local.AvailableSpots`)))
  ;[1 1 1] Get Spots Matching Requirements
  (`KismetArrayLibrary.Array_Clear` (`local.AvailableSpots`))
  (`KismetArrayLibrary.Array_Clear` (`local.RawSpots`))
  (bind _resultactors (`EnvQueryInstanceBlueprintWrapper.GetQueryResultsAsActors` QueryResults))
  (for _array_element _resultactors
    (bind _asbp_aispawn_spot (cast `/Game/00_Sanya/AI/Utility/GeneralAITools/BP_AISpawnSpot` _array_element))
    (`KismetArrayLibrary.Array_Add` (`local.RawSpots`) _asbp_aispawn_spot))
  ;[1 1 1] Filter out inactive and busy spots
  (for _array_element_2 (`local.RawSpots`)
    (if (`KismetArrayLibrary.Array_Contains` (`self.SpawnSpots`) _array_element_2)
      (if (`/Game/00_Sanya/AI/Utility/GeneralAITools/BP_AISpawnSpot.AvailableForContSpawn` _array_element_2)
        (`KismetArrayLibrary.Array_Add` (`local.AvailableSpots`) _array_element_2))))
  (`KismetSystemLibrary.PrintString` (`KismetStringLibrary.Concat_StrStr` "Matching Spots: " (`KismetStringLibrary.Conv_IntToString` (`KismetArrayLibrary.Array_Length` (`local.AvailableSpots`)))))
  ;[1 1 1] Pass Results
  (bind _output_get (set `self.MatchingSpot` _output))
  (`KismetSystemLibrary.PrintString` (`KismetSystemLibrary.GetDisplayName` _output))
  (return _output_get (> (`KismetArrayLibrary.Array_Length` (`local.AvailableSpots`)) 0)))

(fn `UserConstructionScript`
  (`|ExecutionSequence`
    (:`then_0`
      (`SceneComponent.SetWorldScale3D` (`self.RadiusTrigger`) (`KismetMathLibrary.Conv_DoubleToVector` (`self.ActivationRadius`)))
      (`SceneComponent.SetWorldScale3D` (`self.DebugSphere`) (* (`SceneComponent.K2_GetComponentScale` (`self.DebugSphere`)) (`self.ActivationRadius`))))
    (:`then_1`
      (bind _returnvalue (`PrimitiveComponent.CreateDynamicMaterialInstance` (`self.Billboard`) 0 "/Game/0000_Pritch/04_Materials/01_Parent_Materials/DebugMaterials/M_Billboard_Debug.M_Billboard_Debug" "None"))
      (`MaterialInstanceDynamic.SetVectorParameterValue` _returnvalue "Color" (`self.DisplayClolor`)))
    (:`then_3`
      (bind _returnvalue_2 (`PrimitiveComponent.CreateDynamicMaterialInstance` (`self.DebugCube`) 0 "/Game/0000_Pritch/04_Materials/01_Parent_Materials/DebugMaterials/Transparent_DebugMAT.Transparent_DebugMAT" "None"))
      (`MaterialInstanceDynamic.SetVectorParameterValue` _returnvalue_2 "Color" (`self.DisplayClolor`))
      (bind _returnvalue_3 (`PrimitiveComponent.CreateDynamicMaterialInstance` (`self.DebugSphere`) 0 "/Game/0000_Pritch/04_Materials/01_Parent_Materials/DebugMaterials/Transparent_DebugMAT.Transparent_DebugMAT" "None"))
      (`MaterialInstanceDynamic.SetVectorParameterValue` _returnvalue_3 "Color" (`self.DisplayClolor`)))))