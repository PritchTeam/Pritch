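; BP_RatManager is an NPC director that tracks active rats and holds a shared grenade-throw cooldown.
; AddRat and RemoveRat maintain the ActiveRats list without duplicates.
; ThrowCooldown clears CanThrowGrenade for GrenadeCooldown, then restores it, with a DoOnce ignoring repeat calls until the delay ends.
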(event `AddRat`
  (params (Rat :type "/Game/00_Sanya/AI/NPCCharacters/UsableNPC/OrdinaryNPC/Rat/BP_Rat Object Reference"))
  (`KismetArrayLibrary.Array_AddUnique` (`self.ActiveRats`) Rat))

(event `RemoveRat`
  (params (Rat :type "/Game/00_Sanya/AI/NPCCharacters/UsableNPC/OrdinaryNPC/Rat/BP_Rat Object Reference"))
  (`KismetArrayLibrary.Array_RemoveItem` (`self.ActiveRats`) Rat))

(event `ThrowCooldown`
  (`/Engine/EditorBlueprintResources/StandardMacros.DoOnce` false :!label _label
    (:`Completed`
      (set `self.CanThrowGrenade` false)
      (`KismetSystemLibrary.Delay` (`self.GrenadeCooldown`))
      (set `self.CanThrowGrenade` true)
      (goto _label :!via `Reset`))))

(fn `UserConstructionScript`)