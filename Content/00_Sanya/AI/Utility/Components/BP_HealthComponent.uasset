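; Actor health component that subtracts incoming damage from hit points and reports the result to its owner.
; TakeDamage notifies owners implementing BPI_HitPointsInterface with the damage taken and current hit points.
; For such owners other than the main character, it first calls HitVFX, which only affects BP_BaseShooterNPC.
; HitVFX alternates Bam and White Niagara bursts above the NPC, plus a punch effect at its gun and blood at its location.
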(event `TakeDamage`
  (params (IncomingDamage :type Integer))
  (bind _returnvalue (`self.GetOwner`))
  (set `self.DamageTaken` IncomingDamage)
  (set `self.HitPoints` (- (`self.HitPoints`) IncomingDamage))
  (if (`KismetSystemLibrary.DoesImplementInterface` _returnvalue "/Game/00_Sanya/AI/Utility/Components/BPI_HitPointsInterface.BPI_HitPointsInterface_C")
    (if (not (== _returnvalue "/Game/00_Lin/Character/BP_MainCharacter.BP_MainCharacter"))
      (`self.Hit VFX` (`Actor.K2_GetActorLocation` _returnvalue) (`Actor.GetActorForwardVector` _returnvalue) _returnvalue))
    (message `/Game/00_Sanya/AI/Utility/Components/BPI_HitPointsInterface.HealthComponentOutput` _returnvalue (`self.DamageTaken`) (`self.HitPoints`))))

(fn `Hit VFX`
  (params (Location :type "Vector Structure") (forw :type "Vector Structure") (NewParam :type "Actor Object Reference"))
  (bind _returnvalue (`KismetMathLibrary.MakeVector` (.x Location) (.y Location) (+ (.z Location) 100.0)))
  (bind _asbp_base_shooter_npc (cast `/Game/00_Sanya/AI/NPCCharacters/BaseNPC/BP_BaseShooterNPC` NewParam))
  (`/Engine/EditorBlueprintResources/StandardMacros.FlipFlop`
    (:`A`
      (`NiagaraFunctionLibrary.SpawnSystemAtLocation` "/Game/00_Lin/VFX/Enemy/NS_Bam.NS_Bam" _returnvalue (struct) (0.7 0.7 0.7)))
    (:`B`
      (`NiagaraFunctionLibrary.SpawnSystemAtLocation` "/Game/00_Lin/VFX/Enemy/NS_White.NS_White" _returnvalue (struct) (0.7 0.7 0.7))))
  (`NiagaraFunctionLibrary.SpawnSystemAtLocation` "/Game/00_Lin/VFX/Enemy/NS_Punch.NS_Punch" (`SceneComponent.K2_GetComponentLocation` (`/Game/00_Sanya/AI/NPCCharacters/BaseNPC/BP_BaseShooterNPC.Gun` _asbp_base_shooter_npc)) (struct) (0.2 0.2 0.2))
  (`NiagaraFunctionLibrary.SpawnSystemAtLocation` "/Game/00_Lin/VFX/Enemy/NS_Blood.NS_Blood" Location (struct) (0.2 0.2 0.2)))