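; Base gun actor that wraps an EBBarrel component for shooting, ammo and reloading.
; Shoot passes spread and trigger state to the barrel; each shot plays a sound and launches the parent Character along the barrel axis as blowback.
; The mesh's BodyColor shows ammo state, using the debug color when loaded and a desaturated version when empty.
; AIShoot is an empty stub, and TickDebug draws a short barrel trace.
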(event `self.ReceiveBeginPlay`
  ;[1 1 1] Setup
  (set `self.UsedBlowbackMultiplier` (`self.BlowbackMultiplier`)))

(event `Setup`
  (params (AmmoInChamber :type Integer))
  (bind _ebbarrel (`self.EBBarrel`))
  ;[1 1 1] Setup
  (`EBBarrel.SetAmmo` _ebbarrel AmmoInChamber true false false (`EBBarrel.Ammo` _ebbarrel))
  (if (<= (`EBBarrel.CycleAmmoCount` _ebbarrel) 0)
    (if (`EBBarrel.CycleAmmoUnlimited` (`self.EBBarrel`))
      (`MeshComponent.SetVectorParameterValueOnMaterials` (`self.SkeletalMesh`) "BodyColor" (`KismetMathLibrary.Conv_LinearColorToVector` (`self.DebugColor`)) :!label _label)
      (else
        (`MeshComponent.SetVectorParameterValueOnMaterials` (`self.SkeletalMesh`) "BodyColor" (`KismetMathLibrary.Conv_LinearColorToVector` (`KismetMathLibrary.LinearColor_Desaturated` (`self.DebugColor`) 0.5)))))
    (else
      (goto _label))))

(event `Shoot`
  (params (TriggerDown :type Boolean) (Spread :type "Float (double-precision)"))
  ;[1 1 1] Shoot
  (set `EBBarrel.Spread` Spread (`self.EBBarrel`))
  (`EBBarrel.Shoot` (`self.EBBarrel`) TriggerDown))

(event `AIShoot`
  (params (TriggerDown :type Boolean) (Target :type "Actor Object Reference"))
  ;[1 1 1] AI Shoot
)

(event `Reload`
  (bind _ebbarrel (`self.EBBarrel`))
  ;[1 1 1] Reload
  (`EBBarrel.SetAmmo` _ebbarrel (`self.ClipSize`) true false false (`EBBarrel.Ammo` _ebbarrel))
  (`MeshComponent.SetVectorParameterValueOnMaterials` (`self.SkeletalMesh`) "BodyColor" (`KismetMathLibrary.Conv_LinearColorToVector` (`self.DebugColor`))))

(event `self.EBBarrel.AmmoDepleted`
  ;[1 1 1] Show Unloaded
  (`MeshComponent.SetVectorParameterValueOnMaterials` (`self.SkeletalMesh`) "BodyColor" (`KismetMathLibrary.Conv_LinearColorToVector` (`KismetMathLibrary.LinearColor_Desaturated` (`self.DebugColor`) 0.5))))

(event `BlowBack`
  ;[1 1 1] Blowback
  (bind _ascharacter (cast `Character` (`self.GetParentActor`)))
  (`Character.LaunchCharacter` _ascharacter (`KismetMathLibrary.MakeVector` (.x (* (`SceneComponent.GetForwardVector` (`self.EBBarrel`)) (`self.UsedBlowbackMultiplier`))) (.y (* (`SceneComponent.GetForwardVector` (`self.EBBarrel`)) (`self.UsedBlowbackMultiplier`))) (* (.z (* (`SceneComponent.GetForwardVector` (`self.EBBarrel`)) (`self.UsedBlowbackMultiplier`))) 1.0)) false false))

(event `self.EBBarrel.ShotFired`
  ;[1 1 1] ShotFired
  (`self.BlowBack`)
  (`GameplayStatics.PlaySoundAtLocation` (`self.ShotSound`) (`self.K2_GetActorLocation`) (struct) 1.0 1.0 0.0 null null null))

(event `TickDebug`
  (bind _ebbarrel (`self.EBBarrel`))
  (bind _returnvalue (`SceneComponent.K2_GetComponentLocation` _ebbarrel))
  (`KismetSystemLibrary.LineTraceSingle` :`Start` _returnvalue :`End` (+ _returnvalue (* (`SceneComponent.GetForwardVector` _ebbarrel) 100.0)) :`TraceChannel` "TraceTypeQuery1" :`DrawDebugType` "ForDuration")
  (`KismetSystemLibrary.PrintString` "Trace"))

(fn `UserConstructionScript`
  (`MeshComponent.SetVectorParameterValueOnMaterials` (`self.SkeletalMesh`) "BodyColor" (`KismetMathLibrary.Conv_LinearColorToVector` (`self.DebugColor`))))