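; BP_BaseGrenade is a base thrown grenade that explodes once, on impact or after a fallback delay.
; In flight it uses CCD, plays a sound, animates a pulsing, rotating mesh, and adds per-tick force from gravity scaled to the throw multiplier at construction.
; The explosion damages overlapping Characters through BPI_HitPointsInterface, fires a radial impulse, plays a sound and briefly flashes a light before destroying the actor.
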(event `self.ReceiveTick`
  (params (DeltaSeconds :type "Float (single-precision)"))
  (`PrimitiveComponent.AddForce` (`self.StaticMesh`) (`self.AdditionalGravity`) "None" false))

(event `self.ReceiveBeginPlay`
  (`PrimitiveComponent.SetUseCCD` (`self.StaticMesh`) true "None")
  (`AudioComponent.SetSound` (`self.Audio`) (`self.GrenadeFlightSound`))
  (`AudioComponent.Play` (`self.Audio`) 0.0)
  (`self.Pulsate`)
  (`KismetSystemLibrary.Delay` 20.0)
  (`self.Explosion`))

(event `Explosion`
  (`/Engine/EditorBlueprintResources/StandardMacros.DoOnce` false
    (:`Completed`
      (for _array_element (`PrimitiveComponent.GetOverlappingActors` (`self.Sphere`) "/Script/Engine.Character")
        (if (`KismetSystemLibrary.DoesImplementInterface` _array_element "/Game/00_Sanya/AI/Utility/Components/BPI_HitPointsInterface.BPI_HitPointsInterface_C")
          (message `/Game/00_Sanya/AI/Utility/Components/BPI_HitPointsInterface.ReceiveDamage` _array_element (`self.Damage`))))
      (`RadialForceComponent.FireImpulse` (`self.RadialForce`))
      (`AudioComponent.Stop` (`self.Audio`))
      (`GameplayStatics.PlaySoundAtLocation` (`self.ExplosionSound`) (`self.K2_GetActorLocation`) (struct) 1.0 1.0 0.0 null null null)
      (`SceneComponent.SetVisibility` (`self.StaticMesh`) false false)
      (`SceneComponent.SetVisibility` (`self.PointLight`) true false)
      (`KismetSystemLibrary.Delay` 0.1)
      (`self.K2_DestroyActor`))))

(event `self.StaticMesh.OnComponentHit`
  (params (HitComponent :type "PrimitiveComponent Object Reference") (OtherActor :type "Actor Object Reference") (OtherComp :type "PrimitiveComponent Object Reference") (NormalImpulse :type "Vector Structure") (Hit :type "HitResult Structure (by ref)"))
  (`KismetSystemLibrary.PrintString` "HIT" :!label _label)
  (`self.Explosion`))

(event `self.ReceiveHit`
  (params (MyComp :type "PrimitiveComponent Object Reference") (Other :type "Actor Object Reference") (OtherComp :type "PrimitiveComponent Object Reference") (bSelfMoved :type Boolean) (HitLocation :type "Vector Structure") (HitNormal :type "Vector Structure") (NormalImpulse :type "Vector Structure") (Hit :type "HitResult Structure (by ref)"))
  (goto _label))

(event `Pulsate`
  (`|ExecutionSequence`
    (:`then_0`
      (bind (_direction _newtrack_0) (`Timeline|Pulse`)
        (:`Update`
          (`SceneComponent.SetWorldScale3D` (`self.PulseMesh`) (`KismetMathLibrary.Conv_DoubleToVector` _newtrack_0)))))
    (:`then_1`
      (bind (_direction_2 _z_azis _newtrack_0_2) (`Timeline|Rotate`)
        (:`Update`
          (`SceneComponent.K2_SetWorldRotation` (`self.PulseMesh`) (`KismetMathLibrary.MakeRotator` _newtrack_0_2 _newtrack_0_2 _z_azis) false false))))))

(fn `UserConstructionScript`
  (set `self.AdditionalGravity` (* (`self.GravityNeededFor1`) (- (`self.ThrowForceMultiplier`) 1.0))))