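; Base bullet actor for NPC characters that delivers damage on impact and destroys itself after a short fixed lifetime.
; On impact, it sends its Damage value to the hit actor through BPI_HitPointsInterface, if implemented, without destroying itself.
; The construction script tints the Sphere's materials from SphereColor through the Color parameter.
; Its own ReceiveDamage is an empty stub, and leftover velocity-print and health-component nodes never run.
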(event `self.ReceiveBeginPlay`
  (`KismetSystemLibrary.Delay` 3.0)
  (`self.K2_DestroyActor`))

(event `self.OnImpact`
  (params (Ricochet :type Boolean) (PassedThrough :type Boolean) (Location :type "Vector Structure") (IncomingVelocity :type "Vector Structure") (Normal :type "Vector Structure") (ExitLocation :type "Vector Structure") (ExitVelocity :type "Vector Structure") (Impulse :type "Vector Structure") (PenetrationDepth :type "Float (single-precision)") (Actor :type "Actor Object Reference") (Component :type "SceneComponent Object Reference") (BoneName :type Name) (PhysMaterial :type "PhysicalMaterial Object Reference") (HitResult :type "HitResult Structure"))
  (bind (_bblockinghit _binitialoverlap _time _distance _location _impactpoint _normal _impactnormal _physmat _hitactor) (`GameplayStatics.BreakHitResult` HitResult))
  (`/Engine/EditorBlueprintResources/StandardMacros.IsValid` _hitactor
    (:`Is Valid`
      (if (`KismetSystemLibrary.DoesImplementInterface` _hitactor "/Game/00_Sanya/AI/Utility/Components/BPI_HitPointsInterface.BPI_HitPointsInterface_C")
        (message `/Game/00_Sanya/AI/Utility/Components/BPI_HitPointsInterface.ReceiveDamage` _hitactor (`self.Damage`))))))

(fn `ReceiveDamage`
  (params (IncomingDamage :type Integer)))

(fn `UserConstructionScript`
  (`MeshComponent.SetVectorParameterValueOnMaterials` (`self.Sphere`) "Color" (`KismetMathLibrary.Conv_LinearColorToVector` (`self.SphereColor`))))