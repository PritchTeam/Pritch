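; Base shooter NPC that drives a child-actor gun, lobs arc-predicted grenades, reports player sightings to its blackboard and ragdolls on death.
; Events expose shooting, aiming, sounds and behavior cooldowns, with range values read from the gun.
; A looping timer sets spread by whether the NPC is within the player's view.
; Attacks spend timed-return tokens from BP_GlobalAIManager, which overrides per-class stats; close, in-view NPCs can overdraw tokens.
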(event `AfterActivation`
  ;[1 1 1] AdditionalSetup
)

(event `self.ReceiveBeginPlay`
  (bind _returnvalue (`GameplayStatics.GetPlayerCharacter` 0))
  (bind _globalmanagerref (`self.GlobalManagerRef`))
  (bind _asbp_base_gun (cast `/Game/00_Sanya/AI/NPCCharacters/BaseNPC/BP_BaseGun` (`ChildActorComponent.ChildActor` (`self.Gun`)) :!pure true))
  ;[1 1 1] Initial Setup
  (`/Engine/EditorBlueprintResources/StandardMacros.IsValid` _returnvalue :!label _label
    (:`Is Valid`
      (set `self.Player` _returnvalue)
      (`ChildActorComponent.SetChildActorClass` (`self.Gun`) (`self.GunClass`))
      (set `self.MaxRange` (`/Game/00_Sanya/AI/NPCCharacters/BaseNPC/BP_BaseGun.TooFar` _asbp_base_gun))
      (set `self.MinRange` (`/Game/00_Sanya/AI/NPCCharacters/BaseNPC/BP_BaseGun.TooClose` _asbp_base_gun))
      (set `self.ExtremeMinRange` (`/Game/00_Sanya/AI/NPCCharacters/BaseNPC/BP_BaseGun.ExtremeClose` _asbp_base_gun))
      (`/Game/00_Sanya/AI/NPCCharacters/BaseNPC/AIC_BaseAI.ControllerSetup` (cast `/Game/00_Sanya/AI/NPCCharacters/BaseNPC/AIC_BaseAI` (`self.GetController`) :!pure true))
      (set `self.CurrentSpread` (`self.NormalSpread`))
      (`|ExecutionSequence`
        (:`then_0`
          (if (`self.ShowDebugRange`)
            (bind _returnvalue_2 (`|SpawnActorFromClass` "/Game/00_Sanya/AI/Utility/AIDebug/BP_AIDistanceDebug.BP_AIDistanceDebug_C" (`KismetMathLibrary.Conv_VectorToTransform` (`self.K2_GetActorLocation`)) "AlwaysSpawn" "OverrideRootScale" null null))
            (`self.K2_AttachToActor` _returnvalue_2 self "None" "SnapToTarget" "SnapToTarget" "SnapToTarget" true)
            (`/Game/00_Sanya/AI/Utility/AIDebug/BP_AIDistanceDebug.SetRadiusSizes` _returnvalue_2 (`self.ExtremeMinRange`) (`self.MinRange`) (`self.MaxRange`))))
        (:`then_1`
          ;[1 1 1] Find Global Manager and Override stats if specified
          (`|ExecutionSequence`
            (:`then_0`
              (bind _outactors (`GameplayStatics.GetAllActorsOfClass` "/Game/00_Sanya/AI/Utility/NPCDirectors/BP_GlobalAIManager.BP_GlobalAIManager_C"))
              (if (> (`KismetArrayLibrary.Array_Length` _outactors) 0)
                (for _array_element _outactors
                  (if (`/Game/00_Sanya/AI/Utility/NPCDirectors/BP_GlobalAIManager.IsActive` _array_element)
                    (set `self.GlobalManagerRef` _array_element)
                    (break)))))
            (:`then_1`
              (`/Engine/EditorBlueprintResources/StandardMacros.IsValid` _globalmanagerref
                (:`Is Valid`
                  (for _array_element_2 (`/Game/00_Sanya/AI/Utility/NPCDirectors/BP_GlobalAIManager.EnemyStatOverrides` _globalmanagerref)
                    (bind (_enemyclass _normalatackweight _normaltokenreturntime _sattackweight _stokenreturntime) (break `/Game/00_Sanya/AI/Utility/Structs/S_EnemyAttackWeights` _array_element_2))
                    (if (== (`GameplayStatics.GetObjectClass` self) _enemyclass)
                      (`|ExecutionSequence`
                        (:`then_0`
                          (set `self.AttackWeight` _normalatackweight))
                        (:`then_1`
                          (set `self.NormalTokenReturnTime` _normaltokenreturntime))
                        (:`then_2`
                          (set `self.SAttackWeight` _sattackweight))
                        (:`then_3`
                          (set `self.STokenReturnTime` _stokenreturntime))
                        (:`then_4`
                          (break))))))))))
        (:`then_2`
          ;[1 1 1] Accuracy adjustment
          (`KismetSystemLibrary.K2_SetTimerDelegate` (delegate `AimAccuracyAdjustment`) 0.1 true))))))

(event `InitialSetupExternal`
  ;[1 1 1] Initial Setup
  (goto _label))

(event `TickMessage`
  (`KismetSystemLibrary.PrintString` (`KismetStringLibrary.Conv_DoubleToString` (`self.CurrentSpread`))))

(event `AimAccuracyAdjustment`
  ;[1 1 1] Accuracy adjustment
  (if (>= (`KismetMathLibrary.Dot_VectorVector` (`KismetMathLibrary.Normal` (`KismetMathLibrary.GetForwardVector` (`PlayerCameraManager.GetCameraRotation` (`GameplayStatics.GetPlayerCameraManager` 0)))) (`KismetMathLibrary.Normal` (- (`self.K2_GetActorLocation`) (`self.K2_GetActorLocation` (`self.Player`))))) 0.5)
    (set `self.CurrentSpread` (`self.NormalSpread`))
    (else
      (set `self.CurrentSpread` (`self.AltSpread`)))))

(event `PlayDamageSound`
  ;[0.7438 0.2276 1] Sounds
  ;;[1 1 1] DamagedSound
  (`GameplayStatics.PlaySoundAtLocation` (`self.DamagedSound`) (`self.K2_GetActorLocation`) (struct) 1.0 1.0 0.0 null null null null))

(event `JumpCooldown`
  ;[1 0.5147 0] Timers
  ;;[1 1 1] JumpCooldown
  (`/Engine/EditorBlueprintResources/StandardMacros.DoOnce` false :!label _label_2
    (:`Completed`
      (set `self.JumpAvailable` false)
      (`KismetSystemLibrary.Delay` (`self.JumpCooldownTime`))
      (set `self.JumpAvailable` true)
      (goto _label_2 :!via `Reset`))))

(event `StartShooting`
  (bind _asbp_base_gun (cast `/Game/00_Sanya/AI/NPCCharacters/BaseNPC/BP_BaseGun` (`ChildActorComponent.ChildActor` (`self.Gun`)) :!pure true))
  ;[1 1 1] StartShooting
  (if (not (`self.IsDead`))
    (`/Engine/EditorBlueprintResources/StandardMacros.IsValid` _asbp_base_gun
      (:`Is Valid`
        ;[0.1451 0.01961 0.05882] Create UI Arrows
        (`/Game/00_Sanya/AI/NPCCharacters/BaseNPC/BP_BaseGun.Shoot` _asbp_base_gun true (`self.CurrentSpread`))
        (bind _asbp_main_character (cast `/Game/00_Lin/Character/BP_MainCharacter` (`GameplayStatics.GetPlayerCharacter` 0)))
        (message `/Game/00_Lin/Weapon/Enums/BPI_CreateArrow.Create UI Arrow` _asbp_main_character (`self.K2_GetActorLocation`) 2.0 self)))))

(event `PlayDeathSound`
  ;[0.7438 0.2276 1] Sounds
  ;;[1 1 1] DeadSound
  (`GameplayStatics.PlaySoundAtLocation` (`self.DeathSound`) (`self.K2_GetActorLocation`) (struct) 1.0 1.0 0.0 null null null null))

(event `GrenadeCooldown`
  ;[1 0.5147 0] Timers
  ;;[1 1 1] GrenadeCooldown
  (set `self.CanThrowGrenade` false)
  (`KismetSystemLibrary.Delay` (`self.GrenadeCooldownTime`))
  (set `self.CanThrowGrenade` true))

(event `ObjectThrow`
  (bind _returnvalue (`KismetMathLibrary.RandomFloatInRange` (* (`self.ThrownSpread`) -1.0) (`self.ThrownSpread`)))
  (bind _returnvalue_2 (`KismetMathLibrary.MakeVector` (+ (.x (`self.K2_GetActorLocation` (`GameplayStatics.GetPlayerCharacter` 0))) _returnvalue) (+ (.y (`self.K2_GetActorLocation` (`GameplayStatics.GetPlayerCharacter` 0))) _returnvalue) (.z (`self.K2_GetActorLocation` (`GameplayStatics.GetPlayerCharacter` 0)))))
  ;[1 1 1] ObjectThrow
  (if (not (`self.IsDead`))
    (`KismetSystemLibrary.PrintString` "GRENADE")
    (bind _outlaunchvelocity (`GameplayStatics.SuggestProjectileVelocity_CustomArc` (`SceneComponent.K2_GetComponentLocation` (`self.ThrowStart`)) _returnvalue_2 0.0 (`self.ThrowArcParam`)))
    (if (`self.AlwaysThrow`)
      (bind _returnvalue_3 (`|SpawnActorFromClass` (`self.ThrownClass`) (`KismetMathLibrary.Conv_VectorToTransform` (`SceneComponent.K2_GetComponentLocation` (`self.ThrowStart`))) "AdjustIfPossibleButAlwaysSpawn" "OverrideRootScale" null null :!label _label_3))
      (bind _asbp_base_grenade (cast `/Game/00_Sanya/AI/NPCCharacters/BaseNPC/BP_BaseGrenade` _returnvalue_3 :!pure true))
      (`PrimitiveComponent.SetPhysicsLinearVelocity` (`/Game/00_Sanya/AI/NPCCharacters/BaseNPC/BP_BaseGrenade.StaticMesh` _asbp_base_grenade) (* _outlaunchvelocity (`/Game/00_Sanya/AI/NPCCharacters/BaseNPC/BP_BaseGrenade.ThrowForceMultiplier` _asbp_base_grenade)) false "None")
      (set `self.GrenadeCount` (- (`self.GrenadeCount`) 1))
      (`self.GrenadeCooldown`)
      (else
        (bind _landontarget (`self.WillProjectileLandOnTarget` _returnvalue_2 _outlaunchvelocity))
        (if _landontarget
          (goto _label_3))))))

(event `StopShooting`
  (bind _asbp_base_gun (cast `/Game/00_Sanya/AI/NPCCharacters/BaseNPC/BP_BaseGun` (`ChildActorComponent.ChildActor` (`self.Gun`)) :!pure true))
  ;[1 1 1] StopShooting
  (`/Engine/EditorBlueprintResources/StandardMacros.IsValid` _asbp_base_gun
    (:`Is Valid`
      (`/Game/00_Sanya/AI/NPCCharacters/BaseNPC/BP_BaseGun.Shoot` _asbp_base_gun false (`self.CurrentSpread`)))))

(event `PlayMeeleeLandedSound`
  ;[0.7438 0.2276 1] Sounds
  ;;[1 1 1] Meelee Landed Sound
  (`GameplayStatics.PlaySoundAtLocation` (`self.MeeleeLandedSound`) (`self.K2_GetActorLocation`) (struct) 1.0 1.0 0.0 null null null null))

(event `BehaviorChangeCooldown`
  ;[1 0.5147 0] Timers
  ;;[1 1 1] Behavior Change Cooldown
  (`/Engine/EditorBlueprintResources/StandardMacros.DoOnce` false :!label _label_4
    (:`Completed`
      (set `self.BehaviorChangeTimerDone` false)
      (`KismetSystemLibrary.Delay` (`self.TimeTillBehaviorChange`))
      (set `self.BehaviorChangeTimerDone` true)
      (goto _label_4 :!via `Reset`))))

(event `PlayMileeMissedSound`
  ;[0.7438 0.2276 1] Sounds
  ;;[1 1 1] Meelee Missed Sound
  (`GameplayStatics.PlaySoundAtLocation` (`self.MeeleeMissedSound`) (`self.K2_GetActorLocation`) (struct) 1.0 1.0 0.0 null null null null))

(event `Reload`
  (bind _asbp_base_gun (cast `/Game/00_Sanya/AI/NPCCharacters/BaseNPC/BP_BaseGun` (`ChildActorComponent.ChildActor` (`self.Gun`)) :!pure true))
  ;[1 1 1] Reload
  (`/Engine/EditorBlueprintResources/StandardMacros.IsValid` _asbp_base_gun
    (:`Is Valid`
      (`/Game/00_Sanya/AI/NPCCharacters/BaseNPC/BP_BaseGun.Reload` _asbp_base_gun))))

(event `EscapeTimer`
  ;[1 0.5147 0] Timers
  ;;[1 1 1] EscapeTimer
  (`/Engine/EditorBlueprintResources/StandardMacros.DoOnce` false :!label _label_5
    (:`Completed`
      (set `self.BehaviorChangeTimerDone` false)
      (`KismetSystemLibrary.Delay` (`self.EscapeTime`))
      (set `self.BehaviorChangeTimerDone` true)
      (goto _label_5 :!via `Reset`))))

(event `AimAtTarget`
  (params (Target :type "Actor Object Reference"))
  ;[1 1 1] AimGunAtTarget
  (`SceneComponent.K2_SetWorldRotation` (`self.Gun`) (`KismetMathLibrary.Conv_VectorToRotator` (- (+ (`self.K2_GetActorLocation` Target) (0.0 0.0 90.0)) (`SceneComponent.K2_GetComponentLocation` (`self.Gun`)))) false true))

(event `PlayObjectThrowSound`
  ;[0.7438 0.2276 1] Sounds
  ;;[1 1 1] ObjectThrowSound
  (`GameplayStatics.PlaySoundAtLocation` (`self.ObjectThrowSound`) (`self.K2_GetActorLocation`) (struct) 1.0 1.0 0.0 null null null null))

(event `VisibilityReactionTimer`
  ;[1 0.5147 0] Timers
  ;;[1 1 1] Visibility Reaction Timer
  (set `self.CanReactToVisibility` false)
  (`KismetSystemLibrary.Delay` (`self.VisibilityReactionCooldown`))
  (set `self.CanReactToVisibility` true))

(event `ImprfectShootingCooldown`
  ;[1 0.5147 0] Timers
  ;;[1 1 1] Imperfect Shooting Timer
  (`/Engine/EditorBlueprintResources/StandardMacros.DoOnce` false :!label _label_6
    (:`Completed`
      (set `self.BehaviorChangeTimerDone` false)
      (`KismetSystemLibrary.Delay` (`self.ImperfectShootingTime`))
      (set `self.BehaviorChangeTimerDone` true)
      (goto _label_6 :!via `Reset`))))

(event `PlayJumpDodgeSound`
  ;[0.7438 0.2276 1] Sounds
  ;;[1 1 1] JumpDodgeSound
  (`GameplayStatics.PlaySoundAtLocation` (`self.JumpDodgeSound`) (`self.K2_GetActorLocation`) (struct) 1.0 1.0 0.0 null null null null))

(event `ResetGunDirection`
  ;[1 1 1] ResetGunRotation
  (`SceneComponent.K2_SetWorldRotation` (`self.Gun`) (`SceneComponent.K2_GetComponentRotation` (`self.CapsuleComponent`)) false false))

(event `TokenReturnTimer`
  (params (Weight :type Integer))
  (bind _globalmanagerref (`self.GlobalManagerRef`))
  ;[1 0.5147 0] Timers
  ;;[1 1 1] Normal Token Return
  (`/Engine/EditorBlueprintResources/StandardMacros.DoOnce` false :!label _label_7
    (:`Completed`
      (set `self.AttackAllowed` false)
      (`KismetSystemLibrary.Delay` (`self.NormalTokenReturnTime`))
      (set `/Game/00_Sanya/AI/Utility/NPCDirectors/BP_GlobalAIManager.AttackTokenAmount` (+ (`/Game/00_Sanya/AI/Utility/NPCDirectors/BP_GlobalAIManager.AttackTokenAmount` _globalmanagerref) Weight) _globalmanagerref)
      (set `self.AttackAllowed` true)
      (goto _label_7 :!via `Reset`))))

(event `PlayLungeDodgeSound`
  ;[0.7438 0.2276 1] Sounds
  ;;[1 1 1] LungeDodgeSound
  (`GameplayStatics.PlaySoundAtLocation` (`self.LungeDodgeSound`) (`self.K2_GetActorLocation`) (struct) 1.0 1.0 0.0 null null null null))

(event `DamagedFX`
  ;[1 1 1] Damage FeedBack
)

(event `STokenReturnTimer`
  (params (Weight :type Integer))
  (bind _globalmanagerref (`self.GlobalManagerRef`))
  ;[1 0.5147 0] Timers
  ;;[1 1 1] SpecialTokenReturn
  (`/Engine/EditorBlueprintResources/StandardMacros.DoOnce` false :!label _label_8
    (:`Completed`
      (set `self.SAttackAllowed` false)
      (`KismetSystemLibrary.Delay` (`self.STokenReturnTime`))
      (set `/Game/00_Sanya/AI/Utility/NPCDirectors/BP_GlobalAIManager.SAttackTokenAmount` (+ (`/Game/00_Sanya/AI/Utility/NPCDirectors/BP_GlobalAIManager.SAttackTokenAmount` _globalmanagerref) Weight) _globalmanagerref)
      (set `self.SAttackAllowed` true)
      (goto _label_8 :!via `Reset`))))

(event `self.OnLanded`
  (params (Hit :type "HitResult Structure (by ref)"))
  ;[0.7438 0.2276 1] Sounds
  ;;[1 1 1] LandingSound
  (`GameplayStatics.PlaySoundAtLocation` (`self.LandingSound`) (`self.K2_GetActorLocation`) (struct) 1.0 1.0 0.0 null null null null))

(event `Death`
  (params (BoneName :type Name) (VelocityVector :type "Vector Structure"))
  (bind _capsulecomponent (`self.CapsuleComponent`))
  ;[1 1 1] Death
  (if (not (`self.IsDead`))
    (set `self.IsDead` true)
    (`self.K2_DestroyActor` (`self.GetController`))
    (`self.K2_DestroyActor` (`ChildActorComponent.ChildActor` (`self.Gun`)))
    (`PrimitiveComponent.SetSimulatePhysics` (`self.CapsuleComponent`) true)
    (`CharacterMovementComponent.DisableMovement` (`self.CharacterMovement`))
    (`PrimitiveComponent.SetSimulatePhysics` (`self.Mesh`) true)
    (`CapsuleComponent.SetCapsuleSize` _capsulecomponent 0.0 0.0 true)
    (`SceneComponent.K2_SetWorldLocation` _capsulecomponent (+ (`SceneComponent.K2_GetComponentLocation` _capsulecomponent) (0.0 0.0 -100000.0)) false true)
    (`PrimitiveComponent.AddImpulseAtLocation` (`self.Mesh`) (* (`KismetMathLibrary.Normal` VelocityVector) 50000.0) (0.0 0.0 0.0) BoneName)
    (`SkeletalMeshComponent.SetAnimationMode` (`self.Mesh`) "AnimationCustomMode")
    (`KismetSystemLibrary.Delay` 20.0)
    (for _array_element (`self.GetAttachedActors` true)
      (`self.K2_DestroyActor` _array_element))
    (`self.K2_DestroyActor`)))

(event `/Game/00_Sanya/AI/Utility/Components/BPI_HitPointsInterface.DeathOutput`
  (`self.Death` "None")
  (`KismetSystemLibrary.PrintString` "DEATH" true false (struct :`R` 1.0 :`G` 0.958333 :`B` 0.958333 :`A` 1.0)))

(event `/Game/00_Sanya/AI/Utility/Components/BPI_HitPointsInterface.DamageOutput`
  (params (DamageTaken :type Integer) (CurrentHitPoints :type Integer) (BoneName :type Name) (VelocityVector :type "Vector Structure"))
  ;[1 1 1] ReceiveDamage
  (`KismetSystemLibrary.PrintString` "INJURY" true false (struct :`R` 1.0 :`G` 0.958333 :`B` 0.958333 :`A` 1.0))
  (`self.StatusCheck` 0)
  (`self.PassInfoToBB`))

(event `ShootingMontage`
  ;[1 0 0] Delete if/when I can find a better solution
)

(event `self.AIPerception.OnTargetPerceptionUpdated`
  (params (Actor :type "Actor Object Reference") (Stimulus :type "AIStimulus Structure"))
  ;[1 1 1] Perception
  (if (== Actor (`self.Player`))
    (`/Engine/EditorBlueprintResources/StandardMacros.DoOnce` false
      (:`Completed`
        (`KismetSystemLibrary.PrintString` "SEEN PLAYER" true true (struct :`R` 1.0 :`B` 0.14193 :`A` 1.0))
        (`self.PassInfoToBB`)
        (`self.AfterActivation`)))))

(event `PassInfoToBB`
  ;[1 1 1] Pass Info to Blackboard
  (bind _asaic_base_ai (cast `/Game/00_Sanya/AI/NPCCharacters/BaseNPC/AIC_BaseAI` (`self.GetController`)))
  (`BlackboardComponent.SetValueAsBool` (`/Game/00_Sanya/AI/NPCCharacters/BaseNPC/AIC_BaseAI.CurrentBlackboard` _asaic_base_ai) "SeenEnemy" true))

(event `StatsChange`
  ;[1 1 1] Stats changed due to status, customize in child classes
  (set `self.NormalSpeed` (* (`self.NormalSpeed`) (`self.SpeedMultiplier`)))
  (set `self.StrafeSpeed` (* (`self.StrafeSpeed`) (`self.SpeedMultiplier`)))
  (`/Game/00_Sanya/AI/NPCCharacters/BaseNPC/AIC_BaseAI.VariableRefresh` (cast `/Game/00_Sanya/AI/NPCCharacters/BaseNPC/AIC_BaseAI` (`self.GetController`) :!pure true)))

(event `StatusCheck`
  (params (CurrentHitpoints :type Integer))
  ;[1 1 1] Status Changes
  (if (not (> CurrentHitpoints (`self.InjuredThreshold`)))
    (`self.StatsChange`)))

(fn `AskManagerPermission`
  (params (TokenType :type "/Game/00_Sanya/AI/Utility/NPCDirectors/E_TokenType Enum" :default "NewEnumerator0"))
  (returns (PermissionGranted :type Boolean) (TokenTypeToReturn :type "/Game/00_Sanya/AI/Utility/NPCDirectors/E_TokenType Enum"))
  (locals (Token :type "/Game/00_Sanya/AI/Utility/NPCDirectors/E_TokenType Enum" :default "NewEnumerator0"))
  (bind _globalmanagerref (`self.GlobalManagerRef`))
  (bind _globalmanagerref_2 (`self.GlobalManagerRef`))
  (bind _globalmanagerref_3 (`self.GlobalManagerRef`))
  (bind _globalmanagerref_4 (`self.GlobalManagerRef`))
  (bind _output_get (set `local.Token` TokenType))
  (switch `/Game/00_Sanya/AI/Utility/NPCDirectors/E_TokenType` _output_get
    (:`NewEnumerator0`
      ;[1 0.1039 0.1238] Check Timers
      (if (`self.AttackAllowed`)
        _
        (else
          (return false (`local.Token`)))))
    (:`NewEnumerator1`
      (if (`self.SAttackAllowed`)
        _
        (else
          (return false (`local.Token`))))))
  (`/Engine/EditorBlueprintResources/StandardMacros.IsValid` (`self.GlobalManagerRef`)
    (:`Is Valid`
      (if (<= (`KismetMathLibrary.VSize` (- (`self.K2_GetActorLocation` (`self.Player`)) (`self.K2_GetActorLocation` self))) (`/Game/00_Sanya/AI/Utility/NPCDirectors/BP_GlobalAIManager.StealTokenRadius` (`self.GlobalManagerRef`)))
        (if (>= (`KismetMathLibrary.Dot_VectorVector` (`KismetMathLibrary.Normal` (`KismetMathLibrary.GetForwardVector` (`PlayerCameraManager.GetCameraRotation` (`GameplayStatics.GetPlayerCameraManager` 0)))) (`KismetMathLibrary.Normal` (- (`self.K2_GetActorLocation`) (`self.K2_GetActorLocation` (`self.Player`))))) (`/Game/00_Sanya/AI/Utility/NPCDirectors/BP_GlobalAIManager.StealTokenDot` (`self.GlobalManagerRef`)))
          ;[0.7739 0.1864 1] Token "stolen" – ignores current token count, might tip it below 0
          (switch `/Game/00_Sanya/AI/Utility/NPCDirectors/E_TokenType` (`local.Token`)
            (:`NewEnumerator0`
              (set `/Game/00_Sanya/AI/Utility/NPCDirectors/BP_GlobalAIManager.AttackTokenAmount` (- (`/Game/00_Sanya/AI/Utility/NPCDirectors/BP_GlobalAIManager.AttackTokenAmount` _globalmanagerref_2) (`self.AttackWeight`)) _globalmanagerref_2)
              (`self.TokenReturnTimer` (`self.AttackWeight`)))
            (:`NewEnumerator1`
              (set `/Game/00_Sanya/AI/Utility/NPCDirectors/BP_GlobalAIManager.SAttackTokenAmount` (- (`/Game/00_Sanya/AI/Utility/NPCDirectors/BP_GlobalAIManager.SAttackTokenAmount` _globalmanagerref_3) (`self.SAttackWeight`)) _globalmanagerref_3)
              (`self.STokenReturnTimer` (`self.SAttackWeight`))))
          (return true (`local.Token`))
          (else
            _)))
      ;[0.1448 0.5143 1] Take token normally, fail if no tokens available
      (switch `/Game/00_Sanya/AI/Utility/NPCDirectors/E_TokenType` (`local.Token`)
        (:`NewEnumerator0`
          (if (>= (`/Game/00_Sanya/AI/Utility/NPCDirectors/BP_GlobalAIManager.AttackTokenAmount` (`self.GlobalManagerRef`)) (`self.AttackWeight`))
            (set `/Game/00_Sanya/AI/Utility/NPCDirectors/BP_GlobalAIManager.AttackTokenAmount` (- (`/Game/00_Sanya/AI/Utility/NPCDirectors/BP_GlobalAIManager.AttackTokenAmount` _globalmanagerref_4) (`self.AttackWeight`)) _globalmanagerref_4)
            (`self.TokenReturnTimer` (`self.AttackWeight`))
            (return true (`local.Token`))
            (else
              (return false (`local.Token`)))))
        (:`NewEnumerator1`
          (if (>= (`/Game/00_Sanya/AI/Utility/NPCDirectors/BP_GlobalAIManager.SAttackTokenAmount` (`self.GlobalManagerRef`)) (`self.SAttackWeight`))
            (set `/Game/00_Sanya/AI/Utility/NPCDirectors/BP_GlobalAIManager.SAttackTokenAmount` (- (`/Game/00_Sanya/AI/Utility/NPCDirectors/BP_GlobalAIManager.SAttackTokenAmount` _globalmanagerref) (`self.SAttackWeight`)) _globalmanagerref)
            (`self.STokenReturnTimer` (`self.SAttackWeight`))
            (return true (`local.Token`))
            (else
              (return false (`local.Token`)))))))
    (:`Is Not Valid`
      (return true (`local.Token`)))))

(fn `GetShootingTime1`
  (params (Gun :type "Actor Object Reference"))
  (returns (ShootingTime :type "Float (double-precision)"))
  (bind (_asbp_base_gun _bsuccess) (cast `/Game/00_Sanya/AI/NPCCharacters/BaseNPC/BP_BaseGun` Gun :!pure true))
  (`/Engine/EditorBlueprintResources/StandardMacros.IsValid` Gun
    (:`Is Valid`
      (if _bsuccess
        (return (`/Game/00_Sanya/AI/NPCCharacters/BaseNPC/BP_BaseGun.MaxShootingTime` _asbp_base_gun))))
    (:`Is Not Valid`
      (return 0.0))))

(fn `ReceiveDamage`
  (params (IncomingDamage :type Integer) (BoneName :type Name) (HitLoc :type "Vector Structure") (Hit :type "HitResult Structure") (ArrowActor :type "Actor Object Reference"))
  (returns (DidInteract :type Boolean))
  (`/Game/00_Sanya/AI/Utility/Components/BP_HealthComponent.DamageCalculation` (`self.HealthComponent`) IncomingDamage Hit ArrowActor "NewEnumerator0")
  (return false))

(fn `UserConstructionScript`)

(fn `WillProjectileLandOnTarget`
  (params (DesiredLocation :type "Vector Structure") (LaunchVelocity :type "Vector Structure"))
  (returns (LandOnTarget :type Boolean))
  (locals (DesiredPosition :type "Vector Structure") (LandPosition :type "Vector Structure"))
  (set `local.DesiredPosition` DesiredLocation)
  (bind _outhit (`GameplayStatics.Blueprint_PredictProjectilePath_ByTraceChannel` (`SceneComponent.K2_GetComponentLocation` (`self.ThrowStart`)) LaunchVelocity true 40.0 "ECC_WorldStatic" true (`|MakeArray` self :!type "Actor Object Reference") "None" 5.0 15.0 20.0))
  (set `local.LandPosition` (`.Location` (`GameplayStatics.BreakHitResult` _outhit)))
  (return (> (`self.GrenadeLandingTolerance`) (`KismetMathLibrary.VSize` (- (`local.DesiredPosition`) (`local.LandPosition`))))))