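; BP_SpiderBoss is a spider boss NPC that shoots and periodically rams the player, built on a parent class's shooting and aiming events.
; A looping timer fires Ram, which draws an unused debug trace toward the player, raises speed and acceleration, and moves to the player's location.
; StartShooting adds a reload, and AimatTarget replaces parent aiming by rotating the Gun toward the target.
; SummonEnemies is empty, and the normal-speed reset is unwired.
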(event `self.ReceiveBeginPlay`
  (`parent.ReceiveBeginPlay`)
  (`KismetSystemLibrary.K2_SetTimerDelegate` (delegate `Ram`) 2.0 true))

(event `Ram`
  (bind _charactermovement (`self.CharacterMovement`))
  (`KismetSystemLibrary.LineTraceSingle` :`Start` (+ (`self.K2_GetActorLocation`) (0.0 0.0 60.0)) :`End` (+ (`self.K2_GetActorLocation`) (* (`KismetMathLibrary.Normal` (- (+ (`self.K2_GetActorLocation` (`GameplayStatics.GetPlayerCharacter` 0)) (0.0 0.0 60.0)) (`self.K2_GetActorLocation`))) (`self.RamDistance`))) :`TraceChannel` "TraceTypeQuery1" :`DrawDebugType` "ForDuration")
  (set `CharacterMovementComponent.MaxWalkSpeed` (`self.RamSpeed`) _charactermovement)
  (set `CharacterMovementComponent.MaxAcceleration` 5000.0 _charactermovement)
  (`AIBlueprintHelperLibrary.SimpleMoveToLocation` (`self.GetController`) (`self.K2_GetActorLocation` (`GameplayStatics.GetPlayerCharacter` 0))))

(event `self.StartShooting`
  ;[1 1 1] Reload
  (`parent.StartShooting`)
  (`self.Reload`))

(event `self.AimAtTarget`
  (params (Target :type "Actor Object Reference"))
  ;[1 1 1] Aim Override
  (`SceneComponent.K2_SetWorldRotation` (`self.Gun`) (`KismetMathLibrary.Conv_VectorToRotator` (- (+ (`self.K2_GetActorLocation` Target) (0.0 0.0 90.0)) (+ (`self.K2_GetActorLocation`) (`SceneComponent.RelativeLocation` (`self.Gun`))))) false true))

(event `SummonEnemies`)

(fn `UserConstructionScript`
  (`parent.UserConstructionScript`))