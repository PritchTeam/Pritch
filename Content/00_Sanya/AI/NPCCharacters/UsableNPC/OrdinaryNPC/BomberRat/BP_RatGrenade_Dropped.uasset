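; BP_RatGrenade_Dropped is the dropped variant of the BomberRat NPC's grenade, a child Blueprint that explodes after landing in the world.
; BeginPlay skips the parent logic, enables CCD on the mesh, removes the trail and calls Explosion after a random delay of a few seconds.
; DeathOutput triggers the explosion immediately.
; Hit events are overridden empty, so impacts trigger nothing here.
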(event `self.ReceiveBeginPlay`
  (`PrimitiveComponent.SetUseCCD` (`self.StaticMesh`) true "None")
  (`ActorComponent.K2_DestroyComponent` (`self.GrenadeTrail`))
  (`KismetSystemLibrary.Delay` (`KismetMathLibrary.RandomFloatInRange` 3.0 8.0))
  (`self.Explosion`))

(event `/Game/00_Sanya/AI/Utility/Components/BPI_HitPointsInterface.DeathOutput`
  (`self.Explosion`))

(event `self.StaticMesh.OnComponentHit`
  (params (HitComponent :type "PrimitiveComponent Object Reference") (OtherActor :type "Actor Object Reference") (OtherComp :type "PrimitiveComponent Object Reference") (NormalImpulse :type "Vector Structure") (Hit :type "HitResult Structure (by ref)")))

(event `self.ReceiveHit`
  (params (MyComp :type "PrimitiveComponent Object Reference") (Other :type "Actor Object Reference") (OtherComp :type "PrimitiveComponent Object Reference") (bSelfMoved :type Boolean) (HitLocation :type "Vector Structure") (HitNormal :type "Vector Structure") (NormalImpulse :type "Vector Structure") (Hit :type "HitResult Structure (by ref)")))

(fn `UserConstructionScript`
  (`parent.UserConstructionScript`))