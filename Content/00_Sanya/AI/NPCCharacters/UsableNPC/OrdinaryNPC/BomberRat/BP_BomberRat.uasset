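; BP_BomberRat is a rat enemy NPC that shoots, throws objects and scatters dropped grenades when it dies.
; It extends a parent NPC, gating shooting and slightly randomly delayed throws behind manager permission, and reloads when shooting stops.
; DeathOutput runs once, spawning a few grenades around BraidFlame, destroying the controller and moving the capsule far below the level.
; An older GrenadeThrow event remains, launching a physics grenade at the player along a suggested arc with debug drawing.
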(event `self.ReceiveBeginPlay`
  (`parent.ReceiveBeginPlay`))

(event `self.AfterActivation`
  ;[1 1 1] ConnectToManager
  (`parent.AfterActivation`))

(event `self.ShootingMontage`
  ;[1 1 1] ShootingMontage
  (`|PlayMontage` (`self.Mesh`) "/Game/0000_Pritch/02_Assets/3D_Assets/TempModels/NPC/Rat/Rat_ShootingMontage.Rat_ShootingMontage"))

(event `self.ReceiveTick`
  (params (DeltaSeconds :type "Float (single-precision)")))

(event `self.StartShooting`
  (bind _permissiongranted (`self.AskManagerPermission` "NewEnumerator0"))
  (if _permissiongranted
    (`parent.StartShooting`)))

(event `self.ObjectThrow`
  (`KismetSystemLibrary.Delay` (`KismetMathLibrary.RandomFloatInRange` 0.0 0.2))
  (bind _permissiongranted (`self.AskManagerPermission` "NewEnumerator1"))
  (if _permissiongranted
    (`parent.ObjectThrow`)))

(event `GrenadeThrow`
  (bind _returnvalue (`self.K2_GetActorLocation` (`GameplayStatics.GetPlayerCharacter` 0)))
  (bind _returnvalue_2 (`SceneComponent.K2_GetComponentLocation` (`self.ThrowStart`)))
  ;[1 0 0] OldGrenadeThrow
  (`KismetSystemLibrary.DrawDebugSphere` _returnvalue_2 10.0 12 (struct :`R` 1.0 :`G` 0.047946 :`A` 1.0) 1.0)
  (`KismetSystemLibrary.DrawDebugSphere` _returnvalue 100.0 12 (struct :`R` 1.0 :`G` 1.0 :`B` 1.0 :`A` 1.0) 1.0)
  (bind _outlaunchvelocity (`GameplayStatics.SuggestProjectileVelocity_CustomArc` _returnvalue_2 _returnvalue))
  (`KismetSystemLibrary.DrawDebugArrow` _returnvalue_2 (+ _returnvalue_2 _outlaunchvelocity) 100.0 (struct :`R` 1.0 :`B` 0.514808 :`A` 1.0) 1.0 20.0)
  (bind _returnvalue_3 (`|SpawnActorFromClass` "/Game/00_Sanya/AI/NPCCharacters/BaseNPC/BP_BaseGrenade.BP_BaseGrenade_C" (`KismetMathLibrary.Conv_VectorToTransform` (`SceneComponent.K2_GetComponentLocation` (`self.ThrowStart`))) "AdjustIfPossibleButAlwaysSpawn" "OverrideRootScale" null null))
  (`PrimitiveComponent.SetPhysicsLinearVelocity` (`/Game/00_Sanya/AI/NPCCharacters/BaseNPC/BP_BaseGrenade.StaticMesh` _returnvalue_3) _outlaunchvelocity false "None"))

(event `self.StopShooting`
  (`parent.StopShooting`)
  (`self.Reload`))

(event `/Game/00_Sanya/AI/Utility/Components/BPI_HitPointsInterface.DeathOutput`
  (bind _capsulecomponent (`self.CapsuleComponent`))
  (`/Engine/EditorBlueprintResources/StandardMacros.DoOnce` false
    (:`Completed`
      (for _ (range 1 (+ (`KismetMathLibrary.RandomIntegerInRange` 2 4) 1))
        (`|SpawnActorFromClass` "/Game/00_Sanya/AI/NPCCharacters/UsableNPC/OrdinaryNPC/BomberRat/BP_RatGrenade_Dropped.BP_RatGrenade_Dropped_C" (`KismetMathLibrary.MakeTransform` (+ (`SceneComponent.K2_GetComponentLocation` (`self.BraidFlame`)) (`KismetMathLibrary.MakeVector` (`KismetMathLibrary.RandomFloatInRange` -100.0 100.0) (`KismetMathLibrary.RandomFloatInRange` -100.0 100.0)))) "AlwaysSpawn" "OverrideRootScale" null null))
      (`/Game/00_Lin/Sound/AC_SoundComponent.Play Sound` (`self.AC_SoundComponent`) null false)
      (set `self.IsDead` true)
      (`SceneComponent.SetVisibility` (`self.ray_mesh1`) false false)
      (`SceneComponent.SetVisibility` (`self.ray_mesh`) false false)
      (`self.K2_DestroyActor` (`self.GetController`))
      (`CharacterMovementComponent.DisableMovement` (`self.CharacterMovement`))
      (`CapsuleComponent.SetCapsuleSize` _capsulecomponent 0.0 0.0 true)
      (`SceneComponent.K2_SetWorldLocation` _capsulecomponent (+ (`SceneComponent.K2_GetComponentLocation` _capsulecomponent) (0.0 0.0 -100000.0)) false true))))

(event `self.Death`
  (params (BoneName :type Name) (VelocityVector :type "Vector Structure"))
  (`parent.Death` BoneName VelocityVector))

(fn `UserConstructionScript`
  (`parent.UserConstructionScript`))