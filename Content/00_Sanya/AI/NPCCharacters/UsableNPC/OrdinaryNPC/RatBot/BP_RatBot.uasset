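; RatBot enemy NPC, randomly scaled at spawn, that hurts the main character with spinning blades.
; A looping timer checks player distance to toggle the blade montage and timeline-faded swish sound.
; The blade trigger deals repeated damage while overlapped.
; DeathOutput disables movement and collision, launches the mesh upward and kills its emissive glow, while a separate one-shot Explosion applies radial damage through a temporary overlap sphere, then destroys the bot.
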(event `OnComponentBeginOverlap_Event`
  (params (OverlappedComponent :type "PrimitiveComponent Object Reference") (OtherActor :type "Actor Object Reference") (OtherComp :type "PrimitiveComponent Object Reference") (OtherBodyIndex :type Integer) (bFromSweep :type Boolean) (SweepResult :type "HitResult Structure (by ref)"))
  (bind _asbp_main_character (cast `/Game/00_Lin/Character/BP_MainCharacter` OtherActor))
  (if (not (`self.IsDead`)) :!label _label
    (message `/Game/00_Sanya/AI/Utility/Components/BPI_HitPointsInterface.ReceiveDamage` _asbp_main_character 2 "None" (0.0 0.0 0.0) SweepResult null)
    (`GameplayStatics.PlaySoundAtLocation` null (`.Location` (`GameplayStatics.BreakHitResult` SweepResult)) (struct) 1.0 1.0 0.0 null null null null)
    (`KismetSystemLibrary.Delay` (`self.StabDelay`))
    (if (`PrimitiveComponent.IsOverlappingActor` (`self.BladeDamageTrigger`) _asbp_main_character)
      (goto _label))))

(event `self.ReceiveBeginPlay`
  (`parent.ReceiveBeginPlay`)
  (`SceneComponent.SetWorldScale3D` (`self.Mesh`) (`KismetMathLibrary.Conv_DoubleToVector` (`KismetMathLibrary.RandomFloatInRange` (`self.MinScale`) (`self.MaxScale`))))
  (`KismetSystemLibrary.K2_SetTimerDelegate` (delegate `BladeActivation`) 0.2 true)
  (add `PrimitiveComponent.OnComponentBeginOverlap` (`self.BladeDamageTrigger`) (delegate `OnComponentBeginOverlap_Event`)))

(event `BladeActivation`
  (if (`self.IsDead`)
    (`AudioComponent.SetVolumeMultiplier` (`self.SW_RatBot_BladesSwishing_Cue`) 0.0)
    (elif (<= (`KismetMathLibrary.VSize` (- (`self.K2_GetActorLocation` (`self.Player`)) (`self.K2_GetActorLocation`))) (`self.BladeActiveDistance`))
      (if (not (`self.IsPlayingBladesMontage`))
        (set `self.IsPlayingBladesMontage` true)
        (`|PlayMontage` (`self.Mesh`) "/Game/0000_Pritch/02_Assets/3D_Assets/Characters/RatBot/Animations/A_RatBot_attackloop_Montage.A_RatBot_attackloop_Montage"
          (:`then`
            (bind (_direction _newtrack_0) (`Timeline|BladeSoundFallof` :!via `PlayFromStart`)
              (:`Update`
                (`AudioComponent.SetVolumeMultiplier` (`self.SW_RatBot_BladesSwishing_Cue`) (`KismetMathLibrary.Lerp` 0.0 (`self.MaxBladeSoundMultiplier`) _newtrack_0)))))))
      (else
        (`self.StopAnimMontage` "/Game/0000_Pritch/02_Assets/3D_Assets/Characters/RatBot/Animations/A_RatBot_attackloop_Montage.A_RatBot_attackloop_Montage")
        (set `self.IsPlayingBladesMontage` false)
        (bind (_direction_2 _newtrack_0_2) (`Timeline|Timeline` :!via `ReverseFromEnd`)
          (:`Update`
            (`AudioComponent.SetVolumeMultiplier` (`self.SW_RatBot_BladesSwishing_Cue`) (`KismetMathLibrary.Lerp` 0.0 (`self.MaxBladeSoundMultiplier`) _newtrack_0_2))))))))

(event `self.AfterActivation`
  ;[1 1 1] ConnectToManager
  (`parent.AfterActivation`))

(event `Explosion`
  ;[1 1 1] Comment
  (`/Engine/EditorBlueprintResources/StandardMacros.DoOnce` false
    (:`Completed`
      (`NiagaraFunctionLibrary.SpawnSystemAtLocation` (`self.ExplosionEffect`) (`self.K2_GetActorLocation`))
      (bind _returnvalue (`|SpawnActorFromClass` "/Game/00_Sanya/AI/Utility/GeneralAITools/BP_SphereOverlap.BP_SphereOverlap_C" (`KismetMathLibrary.Conv_VectorToTransform` (`self.K2_GetActorLocation`)) "AlwaysSpawn" "OverrideRootScale" null null))
      (bind _actors (`/Game/00_Sanya/AI/Utility/GeneralAITools/BP_SphereOverlap.GetOverlappedActors` _returnvalue "/Script/Engine.Character" (`self.ExplosionRadius`)))
      (for _array_element _actors
        (if (`KismetSystemLibrary.DoesImplementInterface` _array_element "/Game/00_Sanya/AI/Utility/Components/BPI_HitPointsInterface.BPI_HitPointsInterface_C")
          (message `/Game/00_Sanya/AI/Utility/Components/BPI_HitPointsInterface.ReceiveDamage` _array_element (`self.ExplosionDamage`) "None" (0.0 0.0 0.0) (struct) null)))
      (`self.K2_DestroyActor` _returnvalue)
      (`self.K2_DestroyActor`))))

(event `self.ShootingMontage`
  ;[1 1 1] ShootingMontage
  (`|PlayMontage` (`self.Mesh`) "/Game/0000_Pritch/02_Assets/3D_Assets/TempModels/NPC/Rat/Rat_ShootingMontage.Rat_ShootingMontage"))

(event `self.StartShooting`
  (`parent.StartShooting`))

(event `self.ObjectThrow`
  (`parent.ObjectThrow`))

(event `self.StopShooting`
  (`parent.StopShooting`))

(event `/Game/00_Sanya/AI/Utility/Components/BPI_HitPointsInterface.DeathOutput`
  (bind _capsulecomponent (`self.CapsuleComponent`))
  (bind _mesh (`self.Mesh`))
  (set `self.IsDead` true)
  (`self.K2_DestroyActor` (`self.GetController`))
  (`CharacterMovementComponent.DisableMovement` (`self.CharacterMovement`))
  (`CapsuleComponent.SetCapsuleSize` _capsulecomponent 0.0 0.0 true)
  (`SceneComponent.K2_SetWorldLocation` _capsulecomponent (+ (`SceneComponent.K2_GetComponentLocation` _capsulecomponent) (0.0 0.0 -100000.0)) false true)
  (`PrimitiveComponent.AddImpulse` (`self.Mesh`) (* (`KismetMathLibrary.RandomUnitVectorInConeInDegrees` (0.0 0.0 1.0) 10.0) (`self.DeathImpulse`)) "body" true)
  (bind _returnvalue (`PrimitiveComponent.CreateDynamicMaterialInstance` _mesh 0 (`PrimitiveComponent.GetMaterial` _mesh 0) "None"))
  (`MaterialInstanceDynamic.SetScalarParameterValue` _returnvalue "EmissionStrength" 0.0))

(event `self.Death`
  (params (BoneName :type Name) (VelocityVector :type "Vector Structure"))
  (`parent.Death` BoneName VelocityVector))

(fn `UserConstructionScript`
  (`parent.UserConstructionScript`))