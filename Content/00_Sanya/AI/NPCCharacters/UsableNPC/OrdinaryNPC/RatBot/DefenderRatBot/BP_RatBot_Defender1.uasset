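; Defender variant of the RatBot NPC that serves an owner mechanic and can become enraged.
; After activation it writes the owner, player proximity tolerance and wander distance to its AI Blackboard.
; Enrage switches to a dedicated Behavior Tree, raises walk speed, activates sparks and smoke, and tints a dynamic material with a timeline-driven glow.
; On death it explodes and calls the parent death logic only if enraged.
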(event `/Game/00_Sanya/AI/NPCCharacters/BaseNPC/BP_BaseShooterNPC.AfterActivation`
  (bind _returnvalue (`AIBlueprintHelperLibrary.GetBlackboard` (`self.GetController`)))
  (`parent.AfterActivation`)
  (`BlackboardComponent.SetValueAsObject` _returnvalue "OwnerMechanic" (`self.OwnerMechanic`))
  (`BlackboardComponent.SetValueAsFloat` _returnvalue "PlayerToOwnerDistTolerance" (`self.PlayerProximityTolerance`))
  (`BlackboardComponent.SetValueAsFloat` _returnvalue "WanderDist" (`self.WanderDist`)))

(event `Enrage`
  (bind _mesh (`self.Mesh`))
  (`|ExecutionSequence`
    (:`then_0`
      (set `self.IsEnraged` true)
      (bind _returnvalue (`PrimitiveComponent.CreateDynamicMaterialInstance` _mesh 0 (`PrimitiveComponent.GetMaterial` _mesh 0) "None"))
      (`MaterialInstanceDynamic.SetVectorParameterValue` _returnvalue "OverlayGlowColor" (struct :`R` 0.141667 :`B` 0.00249 :`A` 1.0))
      (`MaterialInstanceDynamic.SetVectorParameterValue` _returnvalue "BaseColorTint" (struct :`R` 0.483333 :`G` 0.18125 :`B` 0.186559 :`A` 1.0))
      (set `CharacterMovementComponent.MaxWalkSpeed` 3000.0 (`self.CharacterMovement`))
      (`AIController.RunBehaviorTree` (cast `AIController` (`self.GetController`) :!pure true) "/Game/00_Sanya/AI/NPCCharacters/UsableNPC/OrdinaryNPC/RatBot/DefenderRatBot/BT_RatBot_Defender_Enraged.BT_RatBot_Defender_Enraged")
      (`ActorComponent.Activate` (`self.Sparks`) true)
      (`ActorComponent.Activate` (`self.Smoke`) true))
    (:`then_1`
      (bind (_direction _newtrack_0) (`Timeline|GlowRage` :!via `PlayFromStart`)
        (:`Update`
          (`MaterialInstanceDynamic.SetScalarParameterValue` _returnvalue "OverlayGlowStrength" _newtrack_0))))))

(event `/Game/00_Sanya/AI/Utility/Components/BPI_HitPointsInterface.DeathOutput`
  (if (`self.IsEnraged`)
    (`self.Explosion`)
    (`parent.DeathOutput`)))

(fn `UserConstructionScript`
  (`parent.UserConstructionScript`))