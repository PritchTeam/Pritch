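; Hat sniper NPC that periodically leaps between BP_SniperSpot perches and shoots when its manager grants permission.
; A looping timer, randomized once at BeginPlay, picks random JumpSpots, excluding the current one and any occupied by another sniper.
; Leaps launch the character on a suggested projectile arc at a montage notify; landing re-enables leaping and re-detects the current spot.
; Spot checks use temporary spawned BP_SphereOverlap actors.
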(event `self.ReceiveBeginPlay`
  (`parent.ReceiveBeginPlay`)
  (`self.AfterActivation`)
  (`KismetSystemLibrary.K2_SetTimerDelegate` (delegate `TestLeap`) (`KismetMathLibrary.RandomFloatInRange` 7.0 15.0) true))

(event `TestLeap`
  (bind _output_get (set `self.JumpSpots_dynamic` (`self.JumpSpots`)))
  (`KismetArrayLibrary.Array_RemoveItem` _output_get (`self.CurrentSpot`))
  (bind _output_get_2 (set `self.PotentialSpot` (`KismetArrayLibrary.Array_Random` (`self.JumpSpots_dynamic`)) :!label _label))
  (bind _occupied (`self.CheckIfSpotOccupied1` _output_get_2))
  (if _occupied
    (`KismetArrayLibrary.Array_RemoveItem` (`self.JumpSpots_dynamic`) (`self.PotentialSpot`))
    (goto _label)
    (else
      (`self.Leap` (`self.K2_GetActorLocation` (`self.PotentialSpot`))))))

(event `self.Death`
  (params (BoneName :type Name) (VelocityVector :type "Vector Structure"))
  (`parent.Death` "None" (0.0 0.0 0.0))
  (`ActorComponent.K2_DestroyComponent` (`self.PointLight`)))

(event `self.AfterActivation`
  ;[1 1 1] Setup
  (`self.DetectCurrentSpot`))

(event `Leap`
  (params (DesiredSpot :type "Vector Structure"))
  ;[1 1 1] Leap
  (if (`self.CanLeap`)
    (set `self.CanLeap` false)
    (`|PlayMontage` (`self.Mesh`) "/Game/0000_Pritch/02_Assets/3D_Assets/Characters/Sniper/Animations/A_HatSniper_JumpStart_Montage.A_HatSniper_JumpStart_Montage"
      (:`OnNotifyBegin`
        (bind _outlaunchvelocity (`GameplayStatics.SuggestProjectileVelocity_CustomArc` (`self.K2_GetActorLocation`) DesiredSpot -980.0))
        (`self.LaunchCharacter` _outlaunchvelocity true true)))))

(event `self.OnLanded`
  (params (Hit :type "HitResult Structure (by ref)"))
  ;[1 1 1] Landed
  (`parent.OnLanded` Hit)
  (`|PlayMontage` (`self.Mesh`) "/Game/0000_Pritch/02_Assets/3D_Assets/Characters/Sniper/Animations/A_HatSniper_JumpLand_Montage.A_HatSniper_JumpLand_Montage"
    (:`then`
      (set `self.CanLeap` true)
      (`self.DetectCurrentSpot`))))

(event `DetectCurrentSpot`
  ;[1 1 1] DetectCurrentSpot
  (bind _returnvalue (`|SpawnActorFromClass` "/Game/00_Sanya/AI/Utility/GeneralAITools/BP_SphereOverlap.BP_SphereOverlap_C" (`KismetMathLibrary.Conv_VectorToTransform` (`self.K2_GetActorLocation`)) "AlwaysSpawn" "OverrideRootScale" null null))
  (bind _actors (`/Game/00_Sanya/AI/Utility/GeneralAITools/BP_SphereOverlap.GetOverlappedActors` _returnvalue "/Game/00_Sanya/AI/NPCCharacters/UsableNPC/OrdinaryNPC/HatSniper/BP_SniperSpot.BP_SniperSpot_C" (`self.OtherSniperDistanceTolerance`)))
  (if (> (`KismetArrayLibrary.Array_Length` _actors) 0)
    (set `self.CurrentSpot` (cast `/Game/00_Sanya/AI/NPCCharacters/UsableNPC/OrdinaryNPC/HatSniper/BP_SniperSpot` (`|GetArrayItem` _actors) :!pure true)))
  (`self.K2_DestroyActor` _returnvalue))

(event `self.StartShooting`
  (bind _permissiongranted (`self.AskManagerPermission` "NewEnumerator1"))
  (if _permissiongranted
    (`parent.StartShooting`)
    (`|PlayMontage` (`self.Mesh`) "/Game/0000_Pritch/02_Assets/3D_Assets/Characters/Sniper/Animations/A_HatSniper_Shot_Additive_Montage.A_HatSniper_Shot_Additive_Montage")))

(fn `CheckIfSpotOccupied1`
  (params (Spot :type "/Game/00_Sanya/AI/NPCCharacters/UsableNPC/OrdinaryNPC/HatSniper/BP_SniperSpot Object Reference"))
  (returns (Occupied :type Boolean))
  (locals (OverlappedActors :type "Array of Actor Object Reference"))
  (bind _asactor (cast `Actor` Spot))
  (bind _returnvalue (`|SpawnActorFromClass` "/Game/00_Sanya/AI/Utility/GeneralAITools/BP_SphereOverlap.BP_SphereOverlap_C" (`KismetMathLibrary.Conv_VectorToTransform` (`self.K2_GetActorLocation` _asactor)) "AlwaysSpawn" "OverrideRootScale" null null))
  (bind _actors (`/Game/00_Sanya/AI/Utility/GeneralAITools/BP_SphereOverlap.GetOverlappedActors` _returnvalue "BP_HatSniper_C" (`self.OtherSniperDistanceTolerance`)))
  (set `local.OverlappedActors` _actors)
  (`self.K2_DestroyActor` _returnvalue)
  (return (> (`KismetArrayLibrary.Array_Length` (`local.OverlappedActors`)) 0)))

(fn `UserConstructionScript`
  (`parent.UserConstructionScript`))