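; BP_GromilaBullet is a bullet Blueprint for the Gromila NPC that drives a Niagara effect, apparently a trail, attached to the projectile.
; Each Tick runs the parent logic, then copies the locations of the Sphere's Trail1 and Trail2 sockets into the Niagara StartSocket and EndSocket vector parameters.
; BeginPlay, overlap and construction add no logic of their own.
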(event `self.ReceiveTick`
  (params (DeltaSeconds :type "Float (single-precision)"))
  (bind _niagara (`self.Niagara`))
  (bind _sphere (`self.Sphere`))
  (`parent.ReceiveTick` DeltaSeconds)
  (`FXSystemComponent.SetVectorParameter` _niagara "EndSocket" (`SceneComponent.GetSocketLocation` _sphere "Trail2"))
  (`FXSystemComponent.SetVectorParameter` _niagara "StartSocket" (`SceneComponent.GetSocketLocation` _sphere "Trail1")))

(fn `UserConstructionScript`
  (`parent.UserConstructionScript`))