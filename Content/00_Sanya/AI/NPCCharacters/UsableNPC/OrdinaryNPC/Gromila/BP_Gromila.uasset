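; Gromila enemy NPC, a child AI character that shoots, punches and leaps at the player with a damaging ground slam.
; Leaps and shots need manager permission; leaps launch on a suggested arc to the player, the floor below an airborne player, or a random navigable point.
; A timeline sweeps the fist, damaging and knocking back hit characters.
; Leap landings spawn Niagara, damage and shove nearby characters, and fire a radial impulse.
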(event `Leaptest`
  (bind _returnvalue (`self.K2_GetActorLocation`))
  (bind _randomlocation (`NavigationSystemV1.K2_GetRandomReachablePointInRadius` (`self.K2_GetActorLocation` (`GameplayStatics.GetPlayerCharacter` 0)) 300.0 null null))
  ;[1 0.7627 0] LeapTests
  (if (`self.CanLeap`)
    (set `self.CanLeap` false)
    (`KismetSystemLibrary.Delay` (`KismetMathLibrary.RandomFloatInRange` 0.1 1.0))
    (set `self.Desired Location` _randomlocation)
    (`KismetSystemLibrary.DrawDebugSphere` _randomlocation 100.0 12 (struct :`R` 0.197033 :`G` 1.0 :`A` 1.0) 5.0 20.0)
    (bind _outlaunchvelocity (`GameplayStatics.SuggestProjectileVelocity_CustomArc` _returnvalue _randomlocation -980.0))
    (bind _output_get (set `self.Out Launch Velocity` _outlaunchvelocity))
    (`KismetSystemLibrary.Delay` 0.0)
    (bind (_outhit _outpathpositions _outlasttracedestination) (`GameplayStatics.Blueprint_PredictProjectilePath_ByTraceChannel` _returnvalue _output_get true 40.0 "ECC_WorldStatic" false (`|MakeArray` self :!type "Actor Object Reference") "None" 5.0))
    (set `self.Result Location` (`.Location` (`GameplayStatics.BreakHitResult` _outhit)))
    (`KismetSystemLibrary.DrawDebugSphere` _outlasttracedestination 100.0 12 (struct :`R` 1.0 :`B` 0.068094 :`A` 1.0) 5.0 20.0)
    (`self.LaunchCharacter` _output_get true true)
    (`GameplayStatics.PlaySoundAtLocation` null (`self.K2_GetActorLocation`) (struct) 1.0 1.0 0.0 null null null null)
    (`KismetSystemLibrary.PrintString` (`KismetStringLibrary.Conv_DoubleToString` (`KismetMathLibrary.VSize` (- (`self.Desired Location`) (`self.Result Location`)))) true true (struct :`R` 0.063974 :`G` 1.0 :`A` 1.0))))

(event `PlayLeapSound`
  ;[0.7438 0.2276 1] Sounds
  ;;[1 1 1] LeapSound
  (`GameplayStatics.PlaySoundAtLocation` (`self.LeapSound`) (`self.K2_GetActorLocation`) (struct) 1.0 1.0 0.0 null null null null))

(event `Leap`
  (params (DesiredLocation :type "Vector Structure"))
  (bind _returnvalue (`GameplayStatics.GetPlayerCharacter` 0))
  (bind _returnvalue_2 (`GameplayStatics.GetPlayerCharacter` 0))
  (bind _returnvalue_3 (`self.K2_GetActorLocation` _returnvalue_2))
  ;[1 1 1] Leap to player
  (bind _permissiongranted (`self.AskManagerPermission` "NewEnumerator1"))
  (if _permissiongranted
    (if (`self.CanLeap`)
      (set `self.CanLeap` false)
      (`self.PlayLeapSound`)
      (if (`NavMovementComponent.IsFalling` (`Character.CharacterMovement` _returnvalue))
        (bind (_outhit _returnvalue_4) (`KismetSystemLibrary.LineTraceSingle` _returnvalue_3 (- _returnvalue_3 (0.0 0.0 600.0)) "TraceTypeQuery2" true (`|MakeArray` _returnvalue_2 :!type "Actor Object Reference")))
        (if _returnvalue_4
          (set `self.EndPos` (`.Location` (`GameplayStatics.BreakHitResult` _outhit)))
          (bind _outlaunchvelocity (`GameplayStatics.SuggestProjectileVelocity_CustomArc` (`self.K2_GetActorLocation`) (`self.EndPos`) -980.0 :!label _label))
          (bind _output_get (set `self.Out Launch Velocity` _outlaunchvelocity))
          (`self.LaunchCharacter` _output_get true true)
          (`GameplayStatics.PlaySoundAtLocation` null (`self.K2_GetActorLocation`) (struct) 1.0 1.0 0.0 null null null null)
          (set `self.CauseDamageonLanding` true)
          (else
            (bind (_randomlocation _returnvalue_5) (`NavigationSystemV1.K2_GetRandomLocationInNavigableRadius` (`self.K2_GetActorLocation` (`GameplayStatics.GetPlayerCharacter` 0)) 2000.0 null null))
            (if _returnvalue_5
              (set `self.EndPos` _randomlocation)
              (goto _label)
              (else
                (set `self.CanLeap` true)))))
        (else
          (set `self.EndPos` (`self.K2_GetActorLocation` _returnvalue))
          (goto _label))))))

(event `self.ReceiveBeginPlay`
  ;[1 1 1] Setup
  (`parent.ReceiveBeginPlay`)
  (set `self.DefaultFistLocation` (`SceneComponent.RelativeLocation` (`self.Fist`)))
  (set `self.PunchPoint` (`SceneComponent.RelativeLocation` (`self.PunchLocation`)))
  (`TimelineComponent.SetPlayRate` (`self.Punch`) 5.0))

(event `MeeleeAttack`
  ;[1 1 1] MeleeAttack
  (set `self.IsPunching` true)
  (bind (_direction _newtrack_0) (`Timeline|Punch` :!via `PlayFromStart`)
    (:`Update`
      (bind _sweephitresult (`SceneComponent.K2_SetRelativeLocation` (`self.Fist`) (`KismetMathLibrary.VLerp` (`self.DefaultFistLocation`) (`self.PunchPoint`) _newtrack_0) true false))
      (if (`self.IsPunching`)
        (bind _ascharacter (cast `Character` (`.HitActor` (`GameplayStatics.BreakHitResult` _sweephitresult))))
        (set `self.HitCharacter` _ascharacter)
        (`self.ApplyPunchEffect`)
        (`GameplayStatics.PlaySoundAtLocation` (`self.MeeleeLandedSound`) (`self.K2_GetActorLocation`) (struct) 1.0 1.0 0.0 null null null null)))
    (:`Finished`
      (set `self.IsPunching` false))))

(event `ApplyPunchEffect`
  ;[1 1 1] MeleeAttackLanded
  (`/Engine/EditorBlueprintResources/StandardMacros.DoOnce` false :!label _label_2
    (:`Completed`
      (`self.LaunchCharacter` (`self.HitCharacter`) (* (`KismetMathLibrary.GreaterGreater_VectorRotator` (`SceneComponent.GetForwardVector` (`self.CapsuleComponent`))) 3000.0) false false)
      (`/Engine/EditorBlueprintResources/StandardMacros.IsValid` (`self.HitCharacter`)
        (:`Is Valid`
          (if (`KismetSystemLibrary.DoesImplementInterface` (`self.HitCharacter`) "/Game/00_Sanya/AI/Utility/Components/BPI_HitPointsInterface.BPI_HitPointsInterface_C")
            (message `/Game/00_Sanya/AI/Utility/Components/BPI_HitPointsInterface.ReceiveDamage` (`self.HitCharacter`) (`self.BaseMeleeDamage`) "None" (0.0 0.0 0.0) (struct) null)))
        (:`Is Not Valid`
          _))
      (`KismetSystemLibrary.Delay` 1.0)
      (goto _label_2 :!via `Reset`))))

(event `StrongLanding`
  (bind (_returnvalue_x _returnvalue_y _returnvalue_z) (`KismetMathLibrary.BreakVector` (`self.K2_GetActorLocation`)))
  (`/Engine/EditorBlueprintResources/StandardMacros.DoOnce` false :!label _label_3
    (:`Completed`
      ;[1 1 1] StrongLanding
      (set `self.CauseDamageonLanding` false)
      (`NiagaraFunctionLibrary.SpawnSystemAtLocation` "/Game/00_Lin/VFX/Enemy/NS_Gromila.NS_Gromila" (`KismetMathLibrary.MakeVector` _returnvalue_x _returnvalue_y (- _returnvalue_z 100.0)))
      (bind _output_get (set `self.Overlapping Actors` (`PrimitiveComponent.GetOverlappingActors` (`self.Sphere2`) "/Script/Engine.Character")))
      (`KismetArrayLibrary.Array_RemoveItem` _output_get self)
      (for _array_element (`self.Overlapping Actors`)
        (if (`KismetSystemLibrary.DoesImplementInterface` _array_element "/Game/00_Sanya/AI/Utility/Components/BPI_HitPointsInterface.BPI_HitPointsInterface_C")
          (message `/Game/00_Sanya/AI/Utility/Components/BPI_HitPointsInterface.ReceiveDamage` _array_element (`self.LeapDamage`) "None" (0.0 0.0 0.0) (struct) null)
          (bind _ascharacter (cast `Character` _array_element))
          (if (not (`NavMovementComponent.IsFalling` (`Character.CharacterMovement` _ascharacter)))
            (`self.LaunchCharacter` _ascharacter (* (`KismetMathLibrary.Normal` (`KismetMathLibrary.MakeVector` (.x (- (`self.K2_GetActorLocation` _ascharacter) (`self.K2_GetActorLocation` self))) (.y (- (`self.K2_GetActorLocation` _ascharacter) (`self.K2_GetActorLocation` self))) (+ (.z (- (`self.K2_GetActorLocation` _ascharacter) (`self.K2_GetActorLocation` self))) 60.0))) 5000.0) false true))))
      (`RadialForceComponent.FireImpulse` (`self.RadialForce`))
      (`KismetSystemLibrary.Delay` 0.2)
      (goto _label_3 :!via `Reset`))))

(event `self.OnLanded`
  (params (Hit :type "HitResult Structure (by ref)"))
  (set `self.CanLeap` true)
  (`parent.OnLanded` Hit)
  (if (`self.CauseDamageonLanding`)
    (`self.StrongLanding`)))

(event `self.StartShooting`
  (bind _permissiongranted (`self.AskManagerPermission` "NewEnumerator0"))
  (if _permissiongranted
    (`parent.StartShooting`)
    (`self.Reload`)))

(event `self.AimAtTarget`
  (params (Target :type "Actor Object Reference"))
  (`SceneComponent.K2_SetWorldRotation` (`self.Gun`) (`KismetMathLibrary.Conv_VectorToRotator` (- (+ (`self.K2_GetActorLocation` Target) (0.0 0.0 70.0)) (`SceneComponent.K2_GetComponentLocation` (`self.Gun`)))) false true))

(fn `UserConstructionScript`
  (`parent.UserConstructionScript`))