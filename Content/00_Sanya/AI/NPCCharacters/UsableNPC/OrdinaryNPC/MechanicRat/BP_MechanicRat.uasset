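; Mechanic rat NPC that acts as a rat-bot spawner with a squad of defenders.
; On BeginPlay it scatters owned defender bots on nearby navmesh, then a looping timer spawns small waves of attack bots at its spawn spot until death.
; Shooting and object throws require manager permission, though its RatManager registration is disconnected.
; Death enrages living defenders, hides ray meshes, destroys the controller and drops the capsule far below.
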(event `self.ReceiveBeginPlay`
  (`parent.ReceiveBeginPlay`)
  (for _ (range 1 (+ (`KismetMathLibrary.RandomIntegerInRange` 12 17) 1))
    (bind _randomlocation (`NavigationSystemV1.K2_GetRandomLocationInNavigableRadius` (`self.K2_GetActorLocation`) 700.0 null null))
    (bind _returnvalue (`|SpawnActorFromClass` "/Game/00_Sanya/AI/NPCCharacters/UsableNPC/OrdinaryNPC/RatBot/DefenderRatBot/BP_RatBot_Defender1.BP_RatBot_Defender1_C" (`KismetMathLibrary.Conv_VectorToTransform` _randomlocation) "AdjustIfPossibleButAlwaysSpawn" "OverrideRootScale" null null))
    (set `/Game/00_Sanya/AI/NPCCharacters/UsableNPC/OrdinaryNPC/RatBot/DefenderRatBot/BP_RatBot_Defender1.OwnerMechanic` self _returnvalue)
    (`self.AfterActivation` _returnvalue)
    (`KismetArrayLibrary.Array_Add` (`self.DefenderRats`) _returnvalue))
  (`KismetSystemLibrary.K2_SetTimerDelegate` (delegate `SpawnAttackRat`) 10.0 true))

(event `SpawnAttackRat`
  (if (not (`self.IsDead`))
    (for _ (range 1 (+ (`KismetMathLibrary.RandomIntegerInRange` 2 3) 1))
      (`|SpawnActorFromClass` "/Game/00_Sanya/AI/NPCCharacters/UsableNPC/OrdinaryNPC/RatBot/BP_RatBot.BP_RatBot_C" (`KismetMathLibrary.Conv_VectorToTransform` (`SceneComponent.K2_GetComponentLocation` (`self.RatSpawnSpot`))) "AdjustIfPossibleButAlwaysSpawn" "OverrideRootScale" null null))))

(event `self.AfterActivation`
  ;[1 1 1] ConnectToManager
  (`parent.AfterActivation`)
  (bind _outactors (`GameplayStatics.GetAllActorsOfClass` "/Game/00_Sanya/AI/Utility/NPCDirectors/BP_RatManager.BP_RatManager_C")))

(event `self.ShootingMontage`
  ;[1 1 1] ShootingMontage
  (`|PlayMontage` (`self.Mesh`) "/Game/0000_Pritch/02_Assets/3D_Assets/TempModels/NPC/Rat/Rat_ShootingMontage.Rat_ShootingMontage"))

(event `self.ReceiveTick`
  (params (DeltaSeconds :type "Float (single-precision)")))

(event `self.StartShooting`
  (bind _permissiongranted (`self.AskManagerPermission` "NewEnumerator0"))
  (if _permissiongranted
    (`parent.StartShooting`)))

(event `self.ObjectThrow`
  (`KismetSystemLibrary.Delay` (`KismetMathLibrary.RandomFloatInRange` 0.0 0.2))
  (bind _permissiongranted (`self.AskManagerPermission` "NewEnumerator1"))
  (if _permissiongranted
    (`parent.ObjectThrow`)))

(event `self.StopShooting`
  (`parent.StopShooting`)
  (`self.Reload`))

(event `/Game/00_Sanya/AI/Utility/Components/BPI_HitPointsInterface.DeathOutput`
  (bind _capsulecomponent (`self.CapsuleComponent`))
  (for _array_element (`self.DefenderRats`)
    (if (not (`/Game/00_Sanya/AI/NPCCharacters/BaseNPC/BP_BaseShooterNPC.IsDead` _array_element))
      (`/Game/00_Sanya/AI/NPCCharacters/UsableNPC/OrdinaryNPC/RatBot/DefenderRatBot/BP_RatBot_Defender1.Enrage` _array_element)))
  (`/Game/00_Lin/Sound/AC_SoundComponent.Play Sound` (`self.AC_SoundComponent`) null false)
  (set `self.IsDead` true)
  (`SceneComponent.SetVisibility` (`self.ray_mesh1`) false false)
  (`SceneComponent.SetVisibility` (`self.ray_mesh`) false false)
  (`self.K2_DestroyActor` (`self.GetController`))
  (`CharacterMovementComponent.DisableMovement` (`self.CharacterMovement`))
  (`CapsuleComponent.SetCapsuleSize` _capsulecomponent 0.0 0.0 true)
  (`SceneComponent.K2_SetWorldLocation` _capsulecomponent (+ (`SceneComponent.K2_GetComponentLocation` _capsulecomponent) (0.0 0.0 -100000.0)) false true))

(event `self.Death`
  (params (BoneName :type Name) (VelocityVector :type "Vector Structure"))
  (`parent.Death` BoneName VelocityVector))

(fn `UserConstructionScript`
  (`parent.UserConstructionScript`))