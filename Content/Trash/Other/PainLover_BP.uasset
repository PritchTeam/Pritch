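; PainLover is a damageable actor, apparently a test dummy, that shows its hit points and flashes when hurt.
; ReceiveDamage forwards to HealthComponent, and the HealthComponentOutput event updates the TextRender and plays the RedFlash timeline.
; The timeline lerps the Color of a dynamic material created in the construction script.
; Dialogue participant functions return only names, gender or empty defaults; StartDialogue is empty, with its launch logic disconnected.
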(event `DamagedFX`
  (bind (_direction _flash) (`Timeline|RedFlash` :!via `PlayFromStart`)
    (:`Update`
      (`MaterialInstanceDynamic.SetVectorParameterValue` (`self.BodyMATinstance`) "Color" (`KismetMathLibrary.LinearColorLerp` (`self.BodyColor`) (`self.DamagedColor`) _flash)))))

(event `StartDialogue`)

(event `/Game/00_Sanya/AI/Utility/Components/BPI_HitPointsInterface.HealthComponentOutput`
  (params (DamageTaken :type Integer) (CurrentHitPoints :type Integer))
  (`TextRenderComponent.K2_SetText` (`self.TextRender`) (`KismetTextLibrary.Conv_IntToText` CurrentHitPoints))
  (`self.DamagedFX`))

(fn `CheckCondition`
  (params (Context :type "DlgContext Object Reference") (ConditionName :type Name))
  (returns (ReturnValue :type Boolean))
  (return false))

(fn `GetBoolValue`
  (params (ValueName :type Name))
  (returns (ReturnValue :type Boolean))
  (return false))

(fn `GetFloatValue`
  (params (ValueName :type Name))
  (returns (ReturnValue :type "Float (double-precision)"))
  (return 0.0))

(fn `GetIntValue`
  (params (ValueName :type Name))
  (returns (ReturnValue :type Integer))
  (return 0))

(fn `GetNameValue`
  (params (ValueName :type Name))
  (returns (ReturnValue :type Name))
  (return "None"))

(fn `GetParticipantDisplayName`
  (params (ActiveSpeaker :type Name))
  (returns (ReturnValue :type Text))
  (return (`self.DisplayName`)))

(fn `GetParticipantGender`
  (returns (ReturnValue :type "ETextGender Enum"))
  (return "Masculine"))

(fn `GetParticipantIcon`
  (params (ActiveSpeaker :type Name) (ActiveSpeakerState :type Name))
  (returns (ReturnValue :type "Texture2D Object Reference"))
  (return null))

(fn `GetParticipantName`
  (returns (ReturnValue :type Name))
  (return (`self.ParticipantName`)))

(fn `ModifyBoolValue`
  (params (ValueName :type Name) (bNewValue :type Boolean))
  (returns (ReturnValue :type Boolean))
  (return false))

(fn `ModifyFloatValue`
  (params (ValueName :type Name) (bDelta :type Boolean) (Value :type "Float (double-precision)"))
  (returns (ReturnValue :type Boolean))
  (return false))

(fn `ModifyIntValue`
  (params (ValueName :type Name) (bDelta :type Boolean) (Value :type Integer))
  (returns (ReturnValue :type Boolean))
  (return false))

(fn `ModifyNameValue`
  (params (ValueName :type Name) (NameValue :type Name))
  (returns (ReturnValue :type Boolean))
  (return false))

(fn `OnDialogueEvent`
  (params (Context :type "DlgContext Object Reference") (EventName :type Name))
  (returns (ReturnValue :type Boolean))
  (return false))

(fn `ReceiveDamage`
  (params (IncomingDamage :type Integer))
  (returns (DidInteract :type Boolean))
  (`/Game/00_Sanya/AI/Utility/Components/BP_HealthComponent.TakeDamage` (`self.HealthComponent`) IncomingDamage)
  (return false))

(fn `UserConstructionScript`
  (bind _returnvalue (`PrimitiveComponent.CreateDynamicMaterialInstance` (`self.StaticMesh`) 0 "/Game/0000_Pritch/04_Materials/01_Parent_Materials/DebugMaterials/DebugMAT.DebugMAT" "None"))
  (`MaterialInstanceDynamic.SetVectorParameterValue` _returnvalue "Color" (`self.BodyColor`))
  (set `self.BodyMATinstance` _returnvalue))