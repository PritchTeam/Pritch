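; Static modular arrow actor whose tip, wood and feather meshes are each tinted with their own color.
; The construction script creates a dynamic instance of a debug material on each mesh and sets its Color parameter from the color variables.
; On BeginPlay, ArrowSetup reads the first crafted arrow's colors from the player's BP_MainCharacter and re-applies them the same way, ignoring the black values passed in.
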(event `self.ReceiveBeginPlay`
  (`parent.ReceiveBeginPlay`)
  (`self.ArrowSetup` (struct)))

(event `ArrowSetup`
  (params (EndColor :type "LinearColor Structure") (WoodColor :type "LinearColor Structure") (FeatherColor :type "LinearColor Structure"))
  (bind _asbp_main_character (cast `/Game/00_Lin/Character/BP_MainCharacter` (`GameplayStatics.GetPlayerCharacter` 0)))
  (bind (_craftedarrow1_parameters_name _craftedarrow1_parameters_image _craftedarrow1_parameters_description _craftedarrow1_parameters_baseprojectileparameters _craftedarrow1_parameters_explosionparameters _craftedarrow1_parameters_tipcolor _craftedarrow1_parameters_woodcolor _craftedarrow1_parameters_feathercolor) (break `/Game/Trash/MightBeInportant/AmmunitionStats` (`/Game/00_Lin/Character/BP_MainCharacter.CraftedArrow1_parameters` _asbp_main_character)))
  (set `self.EndColor` _craftedarrow1_parameters_tipcolor)
  (set `self.WoodColor` _craftedarrow1_parameters_woodcolor)
  (set `self.FeatherColor` _craftedarrow1_parameters_feathercolor)
  (bind _returnvalue (`PrimitiveComponent.CreateDynamicMaterialInstance` (`self.End`) 0 "/Game/0000_Pritch/04_Materials/01_Parent_Materials/DebugMaterials/DebugMAT_Red.DebugMAT_Red" "None"))
  (`MaterialInstanceDynamic.SetVectorParameterValue` _returnvalue "Color" (`self.EndColor`))
  (bind _returnvalue_2 (`PrimitiveComponent.CreateDynamicMaterialInstance` (`self.StaticMesh`) 0 "/Game/0000_Pritch/04_Materials/01_Parent_Materials/DebugMaterials/DebugMAT_Red.DebugMAT_Red" "None"))
  (`MaterialInstanceDynamic.SetVectorParameterValue` _returnvalue_2 "Color" (`self.WoodColor`))
  (bind _returnvalue_3 (`PrimitiveComponent.CreateDynamicMaterialInstance` (`self.Plane`) 0 "/Game/0000_Pritch/04_Materials/01_Parent_Materials/DebugMaterials/DebugMAT_Red.DebugMAT_Red" "None"))
  (`MaterialInstanceDynamic.SetVectorParameterValue` _returnvalue_3 "Color" (`self.FeatherColor`)))

(fn `UserConstructionScript`
  (`parent.UserConstructionScript`)
  (`|ExecutionSequence`
    (:`then_0`
      (bind _returnvalue (`PrimitiveComponent.CreateDynamicMaterialInstance` (`self.End`) 0 "/Game/0000_Pritch/04_Materials/01_Parent_Materials/DebugMaterials/DebugMAT_Red.DebugMAT_Red" "None"))
      (`MaterialInstanceDynamic.SetVectorParameterValue` _returnvalue "Color" (`self.EndColor`)))
    (:`then_1`
      (bind _returnvalue_2 (`PrimitiveComponent.CreateDynamicMaterialInstance` (`self.StaticMesh`) 0 "/Game/0000_Pritch/04_Materials/01_Parent_Materials/DebugMaterials/DebugMAT_Red.DebugMAT_Red" "None"))
      (`MaterialInstanceDynamic.SetVectorParameterValue` _returnvalue_2 "Color" (`self.WoodColor`)))
    (:`then_2`
      (bind _returnvalue_3 (`PrimitiveComponent.CreateDynamicMaterialInstance` (`self.Plane`) 0 "/Game/0000_Pritch/04_Materials/01_Parent_Materials/DebugMaterials/DebugMAT_Red.DebugMAT_Red" "None"))
      (`MaterialInstanceDynamic.SetVectorParameterValue` _returnvalue_3 "Color" (`self.FeatherColor`)))))