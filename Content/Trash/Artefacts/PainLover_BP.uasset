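; PainLover is a damageable actor, apparently a test target, that shows its hit points and flashes when hurt.
; ReceiveDamage forwards damage to HealthComponent and returns false; the component's output event updates the TextRender and triggers DamagedFX.
; The construction script creates a dynamic material instance, whose Color the RedFlash timeline blends between body and damaged colors.
; An unconnected copy of the feedback logic remains in ReceiveDamage.
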(event `DamagedFX`
  (bind (_direction _flash) (`Timeline|RedFlash` :!via `PlayFromStart`)
    (:`Update`
      (`MaterialInstanceDynamic.SetVectorParameterValue` (`self.BodyMATinstance`) "Color" (`KismetMathLibrary.LinearColorLerp` (`self.BodyColor`) (`self.DamagedColor`) _flash)))))

(event `/Game/00_Sanya/AI/Utility/Components/BPI_HitPointsInterface.HealthComponentOutput`
  (params (DamageTaken :type Integer) (CurrentHitPoints :type Integer))
  (`TextRenderComponent.K2_SetText` (`self.TextRender`) (`KismetTextLibrary.Conv_IntToText` CurrentHitPoints))
  (`self.DamagedFX`))

(fn `ReceiveDamage`
  (params (IncomingDamage :type Integer))
  (returns (DidInteract :type Boolean))
  (`/Game/00_Sanya/AI/Utility/Components/BP_HealthComponent.TakeDamage` (`self.HealthComponent`) IncomingDamage)
  (return false))

(fn `UserConstructionScript`
  (bind _returnvalue (`PrimitiveComponent.CreateDynamicMaterialInstance` (`self.StaticMesh`) 0 "/Game/0000_Pritch/04_Materials/01_Parent_Materials/DebugMaterials/DebugMAT.DebugMAT" "None"))
  (`MaterialInstanceDynamic.SetVectorParameterValue` _returnvalue "Color" (`self.BodyColor`))
  (set `self.BodyMATinstance` _returnvalue))