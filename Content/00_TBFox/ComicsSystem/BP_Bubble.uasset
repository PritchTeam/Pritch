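; Speech bubble actor for the comics system, showing text in a W_Bubble widget, colored by speaker and optionally depth-offset from its Frame.
; Construct sizes widget and collision box and fetches localized Subtitle text; BeginPlay then reapplies the Text variable and stores dynamic materials for recoloring.
; Hover tints and enlarges the bubble through a timeline.
; Click broadcasts OnClicked, recolors, plays a sound through BP_ComicsCharacter and disables further hover effects.
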(event `self.ReceiveBeginPlay`
  (bind (_returnvalue_x _returnvalue_y _returnvalue_z) (`KismetMathLibrary.BreakVector` (`self.K2_GetActorLocation`)))
  (bind (_returnvalue_x_2 _returnvalue_y_2) (`KismetMathLibrary.BreakVector` (`SceneComponent.K2_GetComponentLocation` (`/Game/00_TBFox/ComicsSystem/BP_ComicsFrame.Plane` (`self.Frame`)))))
  (`|ExecutionSequence`
    (:`then_0`
      (`/Engine/EditorBlueprintResources/StandardMacros.IsValid` (`self.Frame`)
        (:`Is Valid`
          ;[1 1 1] Все баблы близко к фрейму
          (if (`self.UseZLayer`)
            (`self.K2_SetActorLocation` (`KismetMathLibrary.MakeVector` _returnvalue_x (+ _returnvalue_y_2 (`KismetMathLibrary.Conv_IntToDouble` (/ (`self.ZLayer`) 10))) _returnvalue_z))))))
    (:`then_1`
      (`self.Construct`))
    (:`then_2`
      (`self.ShowBubble` (not (`self.StartHidden`))))
    (:`then_3`
      ;[1 1 1] Видимо из-за конструирования нужна повторная инициализация текста
      (bind _asw_bubble (cast `/Game/00_TBFox/ComicsSystem/W_Bubble` (`WidgetComponent.GetWidget` (`self.Widget`))))
      (`/Game/00_TBFox/ComicsSystem/W_Bubble.SetText` _asw_bubble (`self.Text`))
      ;[1 1 1] Цвет рамки бабблов
      (bind _returnvalue (`KismetMaterialLibrary.CreateDynamicMaterialInstance` "/Game/00_TBFox/ComicsSystem/M_BubbleBackgroundColor.M_BubbleBackgroundColor"))
      (set `self.BorderMat` _returnvalue)
      (`MaterialInstanceDynamic.SetVectorParameterValue` _returnvalue "Color" (`self.SpeakerToBorderColor`))
      (`Image.SetBrushFromMaterial` (`/Game/00_TBFox/ComicsSystem/W_Bubble.Image_BorderColor` _asw_bubble) _returnvalue)
      ;[1 1 1] Цвет фона бабблов
      (bind _returnvalue_2 (`KismetMaterialLibrary.CreateDynamicMaterialInstance` "/Game/00_TBFox/ComicsSystem/M_BubbleMainColor.M_BubbleMainColor"))
      (set `self.BGMat` _returnvalue_2)
      (`MaterialInstanceDynamic.SetVectorParameterValue` _returnvalue_2 "Color" (`self.SpeakerToMainColor`))
      (`Image.SetBrushFromMaterial` (`/Game/00_TBFox/ComicsSystem/W_Bubble.Image_MainColor` _asw_bubble) _returnvalue_2)
      (bind _textblock_842 (`/Game/00_TBFox/ComicsSystem/W_Bubble.TextBlock_842` _asw_bubble))
      (set `self.TextColor` _textblock_842)
      (`TextBlock.SetColorAndOpacity` _textblock_842 (`self.SpeakerToTextColor`)))))

(event `HoverBubble`
  ;[0.2165 0.2923 1] Overlap Events
  (if (not (`self.WasClicked`))
    (`self.OverlapColor`)
    (`TimelineComponent.SetPlayRate` (`self.SetSize`) 4.0)
    (bind (_direction _float) (`Timeline|SetSize` :!label _label)
      (:`Update`
        (`WidgetComponent.SetDrawSize` (`self.Widget`) (* (`self.BubbleSize`) (`KismetMathLibrary.Lerp` 1.0 1.1 _float)))))))

(event `UnhoverBubble`
  ;[0.2165 0.2923 1] Overlap Events
  (if (not (`self.WasClicked`))
    (`self.NormalColor`)
    (goto _label :!via `Reverse`)))

(event `ShowBubble`
  (params (_Show :type Boolean))
  (bind _returnvalue (select `bool` _Show :`false` "NoCollision" :`true` "QueryAndPhysics" :!type "ECollisionEnabled Enum"))
  (`self.SetActorHiddenInGame` (not _Show))
  (`PrimitiveComponent.SetCollisionEnabled` (`self.Box`) _returnvalue)
  (`PrimitiveComponent.SetCollisionEnabled` (`self.Widget`) _returnvalue))

(event `Click`
  ;[1 1 1] Comment
  (if (`self.bHidden`)
    (`KismetSystemLibrary.PrintString` "BUBBLE HIDDEN")
    (else
      (`self.On_Clicked` self)
      (set `self.WasClicked` true)
      (`self.ClickColor`)
      (bind _asbp_comics_character (cast `/Game/00_TBFox/ComicsSystem/BP_ComicsCharacter` (`GameplayStatics.GetPlayerPawn` 0)))
      (`/Game/00_TBFox/ComicsSystem/BP_ComicsCharacter.PlaySoundCue` _asbp_comics_character "/Game/00_Anton/Sounds/SoundDesign/UI_Sounds/A_UI_ClickBubble_Cue.A_UI_ClickBubble_Cue" 1.0 1.0 0.0))))

(event `Construct`
  (bind (_returnvalue_x _returnvalue_y _returnvalue_z) (`KismetMathLibrary.BreakVector` (`self.K2_GetActorLocation`)))
  (bind (_bubblesize_x _bubblesize_y) (`KismetMathLibrary.BreakVector2D` (`self.BubbleSize`)))
  (bind _subtitle (`self.Subtitle`))
  (bind _widget (`self.Widget`))
  (bind (_returnvalue_x_2 _returnvalue_y_2) (`KismetMathLibrary.BreakVector` (`SceneComponent.K2_GetComponentLocation` (`/Game/00_TBFox/ComicsSystem/BP_ComicsFrame.Plane` (`self.Frame`)))))
  (`|ExecutionSequence`
    (:`then_0`
      (`/Engine/EditorBlueprintResources/StandardMacros.IsValid` (`self.Frame`)
        (:`Is Valid`
          (if (`self.UseZLayer`)
            (`self.K2_SetActorLocation` (`KismetMathLibrary.MakeVector` _returnvalue_x (+ _returnvalue_y_2 (* (`KismetMathLibrary.Conv_IntToDouble` (`self.ZLayer`)) 100.0)) _returnvalue_z))))))
    (:`then_1`
      (`WidgetComponent.SetDrawSize` _widget (`self.BubbleSize`))
      (bind _asw_bubble (cast `/Game/00_TBFox/ComicsSystem/W_Bubble` (`WidgetComponent.GetWidget` _widget)))
      (`/Engine/EditorBlueprintResources/StandardMacros.IsValid` _subtitle
        (:`Is Valid`
          (bind (_speaker _text) (`/Game/00_TBFox/LocalizaationSystem/Subtitle_BP/Subtitles_DataAsset.GetText` _subtitle (`self.Id`) (`/Game/00_TBFox/ComicsSystem/GameMode_Comics.Language` (cast `/Game/00_TBFox/ComicsSystem/GameMode_Comics` (`GameplayStatics.GetGameMode`) :!pure true))))
          (`/Game/00_TBFox/ComicsSystem/W_Bubble.SetText` _asw_bubble (`KismetTextLibrary.Conv_StringToText` _text)))
        (:`Is Not Valid`
          (`/Game/00_TBFox/ComicsSystem/W_Bubble.SetText` _asw_bubble (`self.Text`))))
      (bind _returnvalue (`KismetMaterialLibrary.CreateDynamicMaterialInstance` "/Game/00_TBFox/ComicsSystem/M_BubbleBackgroundColor.M_BubbleBackgroundColor"))
      (`MaterialInstanceDynamic.SetVectorParameterValue` _returnvalue "Color" (`self.SpeakerToBorderColor`))
      (`Image.SetBrushFromMaterial` (`/Game/00_TBFox/ComicsSystem/W_Bubble.Image_BorderColor` _asw_bubble) _returnvalue)
      (bind _returnvalue_2 (`KismetMaterialLibrary.CreateDynamicMaterialInstance` "/Game/00_TBFox/ComicsSystem/M_BubbleMainColor.M_BubbleMainColor"))
      (`MaterialInstanceDynamic.SetVectorParameterValue` _returnvalue_2 "Color" (`self.SpeakerToMainColor`))
      (`Image.SetBrushFromMaterial` (`/Game/00_TBFox/ComicsSystem/W_Bubble.Image_MainColor` _asw_bubble) _returnvalue_2)
      (`TextBlock.SetColorAndOpacity` (`/Game/00_TBFox/ComicsSystem/W_Bubble.TextBlock_842` _asw_bubble) (`self.SpeakerToTextColor`)))
    (:`then_2`
      (`BoxComponent.SetBoxExtent` (`self.Box`) (`KismetMathLibrary.MakeVector` (/ _bubblesize_x 2.0) 5.0 (/ _bubblesize_y 2.0)) true))))

(event `SetNewText`
  (params (Text :type String))
  (bind _output_get (set `self.Text` (`KismetTextLibrary.Conv_StringToText` Text)))
  (bind _asw_bubble (cast `/Game/00_TBFox/ComicsSystem/W_Bubble` (`WidgetComponent.GetWidget` (`self.Widget`))))
  (`/Game/00_TBFox/ComicsSystem/W_Bubble.SetText` _asw_bubble _output_get))

(fn `ClickColor`
  (switch `/Game/00_TBFox/ComicsSystem/LinStuff/E_Speaker` (`self.SpeakerEnum`)
    (:`NewEnumerator0`
      (`MaterialInstanceDynamic.SetVectorParameterValue` (`self.BorderMat`) "Color" (struct :`R` 0.039216 :`B` 1.0 :`A` 1.0)))
    (:`NewEnumerator1`
      (`MaterialInstanceDynamic.SetVectorParameterValue` (`self.BGMat`) "Color" (struct :`R` 0.039216 :`B` 1.0 :`A` 1.0))
      (`TextBlock.SetColorAndOpacity` (`self.TextColor`) (`self.White Text Color`)))
    (:`NewEnumerator2`
      (`MaterialInstanceDynamic.SetVectorParameterValue` (`self.BorderMat`) "Color" (struct :`R` 0.4 :`G` 0.4 :`B` 0.4 :`A` 1.0)))
    (:`NewEnumerator3`
      (`MaterialInstanceDynamic.SetVectorParameterValue` (`self.BorderMat`) "Color" (struct :`R` 0.4 :`G` 0.4 :`B` 0.4 :`A` 1.0)))))

(fn `NormalColor`
  (`MaterialInstanceDynamic.SetVectorParameterValue` (`self.BGMat`) "Color" (`self.SpeakerToMainColor`))
  (`MaterialInstanceDynamic.SetVectorParameterValue` (`self.BorderMat`) "Color" (`self.SpeakerToBorderColor`))
  (`TextBlock.SetColorAndOpacity` (`self.TextColor`) (`self.SpeakerToTextColor`)))

(fn `OverlapColor`
  (switch `/Game/00_TBFox/ComicsSystem/LinStuff/E_Speaker` (`self.SpeakerEnum`)
    (:`NewEnumerator0`
      (`TextBlock.SetColorAndOpacity` (`self.TextColor`) (`self.Blue Color`)))
    (:`NewEnumerator3`
      (`TextBlock.SetColorAndOpacity` (`self.TextColor`) (`self.DefTextCol`)))))

(fn `SpeakerToBorderColor`
  (returns (BoardColor :type "LinearColor Structure"))
  (switch `/Game/00_TBFox/ComicsSystem/LinStuff/E_Speaker` (`self.SpeakerEnum`)
    (:`NewEnumerator0`
      (return (struct :`R` 1.0 :`G` 1.0 :`B` 1.0 :`A` 1.0)))
    (:`NewEnumerator3`
      (return (struct :`A` 1.0)))
    (:`NewEnumerator4`
      (return (struct :`G` 0.143019 :`B` 1.0 :`A` 1.0)))
    (:`NewEnumerator5`
      (return (`self.Boarderless Color`)))))

(fn `SpeakerToMainColor`
  (returns (BoardColor :type "LinearColor Structure"))
  (switch `/Game/00_TBFox/ComicsSystem/LinStuff/E_Speaker` (`self.SpeakerEnum`)
    (:`NewEnumerator0`
      (return (struct :`A` 1.0)))
    (:`NewEnumerator2`
      (return (struct :`R` 0.129167 :`G` 0.129167 :`B` 0.129167 :`A` 1.0)))
    (:`NewEnumerator3`
      (return (struct :`R` 1.0 :`G` 1.0 :`B` 1.0 :`A` 1.0)))
    (:`NewEnumerator4`
      (return (struct :`R` 0.299988 :`G` 0.573822 :`B` 1.0 :`A` 1.0)))
    (:`NewEnumerator5`
      (return (`self.Boarderless Color`)))))

(fn `SpeakerToTextColor`
  (returns (TextColor :type "SlateColor Structure"))
  (switch `/Game/00_TBFox/ComicsSystem/LinStuff/E_Speaker` (`self.SpeakerEnum`)
    (:`NewEnumerator0`
      (return (`self.White Text Color`)))
    (:`NewEnumerator1`
      (return (`self.Black TextColor`)))
    (:`NewEnumerator2`
      (return (`self.White Text Color`)))
    (:`NewEnumerator3`
      (return (`self.Black TextColor`)))
    (:`NewEnumerator4`
      (return (`self.DefTextCol`)))))

(fn `UserConstructionScript`)