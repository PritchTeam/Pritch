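; Player-controlled camera actor for the comics system, which views the comic one frame at a time.
; On BeginPlay it points the camera at FirstFrame and marks that frame as current; Space Bar fires the OnClick dispatcher.
; Helper functions get and set the view, using actor location for position and the camera's relative Y offset as zoom.
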(event `self.ReceiveBeginPlay`
  (bind _firstframe (`self.FirstFrame`))
  (`/Game/00_TBFox/ComicsSystem/BP_ComicsFrame.SetCameraToCurrentFrame` _firstframe)
  (`/Game/00_TBFox/ComicsSystem/BP_ComicsFrame.SetAsCurrentFrame` _firstframe))

(event `self.ReceiveTick`
  (params (DeltaSeconds :type "Float (single-precision)")))

(event `Key|SpaceBar`
  (params (Key :type "Key Structure"))
  (:`Pressed`
    (`self.On_Click`)))

(fn `GetCameraPosition`
  (returns (CameraPosition :type "Vector Structure"))
  (return (`self.K2_GetActorLocation`)))

(fn `GetCameraZoom`
  (returns (CurrentZoom :type "Float (double-precision)"))
  (bind (_relativelocation_x _relativelocation_y) (`KismetMathLibrary.BreakVector` (`SceneComponent.RelativeLocation` (`self.Camera`))))
  (return _relativelocation_y))

(fn `SetCameraPosition`
  (params (Location :type "Vector Structure") (Zoom :type "Float (double-precision)"))
  (`self.K2_SetActorLocation` Location)
  (`SceneComponent.K2_SetRelativeLocation` (`self.Camera`) (`KismetMathLibrary.MakeVector` 0.0 Zoom) false false))

(fn `UserConstructionScript`)