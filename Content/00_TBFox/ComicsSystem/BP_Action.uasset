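; BP_Action is a chainable action step actor for the comics system that forwards player clicks while it is active.
; Start retries until it finds a BP_ComicsCharacter, then binds to its OnClick and fires OnStart.
; Finish unbinds, fires OnFinished and starts NextAction, while Abort fires OnAbort and then calls Finish, so the chain continues.
; The construction script draws a link arrow to NextAction to visualize the sequence.
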(event `self.ReceiveBeginPlay`)

(event `self.ReceiveTick`
  (params (DeltaSeconds :type "Float (single-precision)")))

(event `Start`
  (bind _returnvalue (`GameplayStatics.GetActorOfClass` "/Game/00_TBFox/ComicsSystem/BP_ComicsCharacter.BP_ComicsCharacter_C" :!label _label))
  (`/Engine/EditorBlueprintResources/StandardMacros.IsValid` _returnvalue
    (:`Is Valid`
      (set `self._playerCamera` _returnvalue)
      (add `/Game/00_TBFox/ComicsSystem/BP_ComicsCharacter.On_Click` (`self._playerCamera`) (`|CreateDelegate` :!event `Click`))
      (`self.On_Start` self)
      (set `self._isActive` true))
    (:`Is Not Valid`
      (`KismetSystemLibrary.Delay` 0.0)
      (goto _label))))

(event `Click`
  (`self.On_Click` self))

(event `Finish`
  (remove `/Game/00_TBFox/ComicsSystem/BP_ComicsCharacter.On_Click` (`self._playerCamera`) (`|CreateDelegate` :!event `Click`))
  (`self.On_Finished ` self)
  (set `self._isActive` false)
  (`/Engine/EditorBlueprintResources/StandardMacros.IsValid` (`self.NextAction`)
    (:`Is Valid`
      (`self.Start` (`self.NextAction`)))))

(event `Abort`
  (`self.On_Abort` self)
  (`self.Finish`))

(fn `UserConstructionScript`
  (`/Engine/EditorBlueprintResources/StandardMacros.IsValid` (`self.NextAction`)
    (:`Is Valid`
      (bind _returnvalue (`AddComponent|NODE_AddLinkArrow_Component-0`))
      (`/Game/00_TBFox/ComicsSystem/LinkArrow_Component.Update_Actor` _returnvalue self (`self.NextAction`)))))