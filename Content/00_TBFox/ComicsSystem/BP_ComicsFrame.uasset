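; Clickable comic panel actor for the comics system, built as a textured plane sized from its dimensions and scale at construction.
; Hover plays a timeline that slightly enlarges the plane, and a click either fires the clicked callback or saves itself to the comic slot and opens another level.
; It can position the comics character's camera on itself and start its linked first action, shown by an arrow component.
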(event `Hover Frame`
  (bind _rememberedscale (`self.RememberedScale`))
  (if (and (`self.CanHover`) (not (`self.WasClicked`)))
    (`TimelineComponent.SetPlayRate` (`self.SetSize`) 4.0)
    (bind (_direction _float) (`Timeline|SetSize` :!label _label)
      (:`Update`
        (`SceneComponent.SetWorldScale3D` (`self.Plane`) (`KismetMathLibrary.VLerp` _rememberedscale (* _rememberedscale (1.05 1.05 1.0)) _float))))))

(event `Unhover Frame`
  (if (and (`self.CanHover`) (not (`self.WasClicked`)))
    (goto _label :!via `Reverse`)))

(event `ClickedFrameUnhover`
  (goto _label :!via `Reverse`))

(event `self.ReceiveBeginPlay`
  (bind _returnvalue (`GameplayStatics.GetActorOfClass` "/Game/00_TBFox/ComicsSystem/BP_ComicsCharacter.BP_ComicsCharacter_C"))
  (set `self._playerCamera` _returnvalue)
  (`self.EnableInput` (`GameplayStatics.GetPlayerController` 0)))

(event `SetCameraToCurrentFrame`
  (bind _returnvalue (`GameplayStatics.GetActorOfClass` "/Game/00_TBFox/ComicsSystem/BP_ComicsCharacter.BP_ComicsCharacter_C"))
  (bind (_location _zoom) (`self.GetCameraPosition`))
  (`/Game/00_TBFox/ComicsSystem/BP_ComicsCharacter.SetCameraPosition` _returnvalue _location _zoom)
  (set `/Game/00_TBFox/ComicsSystem/BP_ComicsCharacter.FirstFrame` self _returnvalue))

(event `Key|SpaceBar`
  (params (Key :type "Key Structure")))

(event `SetAsCurrentFrame`
  (`/Engine/EditorBlueprintResources/StandardMacros.IsValid` (`self.FirstAction`)
    (:`Is Valid`
      (`/Game/00_TBFox/ComicsSystem/BP_Action.Start` (`self.FirstAction`)))))

(event `Click`
  (`/Game/00_TBFox/ComicsSystem/BP_ComicsCharacter.PlaySoundCue` (`self._playerCamera`) "/Game/00_Anton/Sounds/SoundDesign/UI_Sounds/A_UI_Click_Cue.A_UI_Click_Cue" 1.0 1.0 0.0)
  (if (not (`self.Teleport To Level?`))
    (`self.ClickedFrameUnhover`)
    (`self.On_Clicked` self)
    (set `self.WasClicked` true)
    (if (`self.CanHover`)
      (`PrimitiveComponent.SetRenderCustomDepth` (`self.Plane`) false))
    (else
      (bind _asgi_main (cast `/Game/00_Lin/GI_Main` (`GameplayStatics.GetGameInstance`)))
      (bind _savedata (`/Game/00_Lin/GI_Main.SaveData` _asgi_main))
      (set `/Game/00_Lin/SaveGame/SG_Main.Slot` self _savedata)
      (`GameplayStatics.SaveGameToSlot` _savedata "comic")
      (`GameplayStatics.OpenLevel` (`self.LevelTeleport`)))))

(fn `GetCameraPosition`
  (returns (Location :type "Vector Structure") (Zoom :type "Float (double-precision)"))
  (bind (_offset_x _offset_y) (`KismetMathLibrary.BreakVector2D` (`self.Offset`)))
  (bind (_returnvalue_x _returnvalue_y _returnvalue_z) (`KismetMathLibrary.BreakVector` (+ (`self.K2_GetActorLocation`) (`KismetMathLibrary.MakeVector` _offset_x 0.0 _offset_y))))
  (return (`KismetMathLibrary.MakeVector` _returnvalue_x 0.0 _returnvalue_z) (- (- (`self.Zoom`) 1080.0) 120.0)))

(fn `Remember`
  (params (vector :type "Vector Structure"))
  (returns (_vector :type "Vector Structure"))
  (return vector))

(fn `UserConstructionScript`
  (bind (_dimensions_x _dimensions_y) (`KismetMathLibrary.BreakVector2D` (`self.Dimensions`)))
  (`|ExecutionSequence`
    (:`then_0`
      ;[1 1 1] Назначение материала
      (bind _returnvalue (`KismetMaterialLibrary.CreateDynamicMaterialInstance` "/Game/00_TBFox/ComicsSystem/M_ComicsFrame.M_ComicsFrame"))
      (`MaterialInstanceDynamic.SetTextureParameterValue` _returnvalue "Texture" (`self.Texture`))
      (`PrimitiveComponent.SetMaterial` (`self.Plane`) 0 _returnvalue)
      ;[1 1 1] Размер фрейма
      (`SceneComponent.SetWorldScale3D` (`self.Plane`) (`KismetMathLibrary.MakeVector` (* _dimensions_x 0.01 (`self.Scale`)) (* _dimensions_y 0.01 (`self.Scale`)) 1.0))
      (`/Engine/EditorBlueprintResources/StandardMacros.IsValid` (`self.FirstAction`)
        (:`Is Valid`
          (bind _returnvalue_2 (`AddComponent|NODE_AddLinkArrow_Component-0`))
          (`/Game/00_TBFox/ComicsSystem/LinkArrow_Component.Update_Actor` _returnvalue_2 self (`self.FirstAction`)))))
    (:`then_1`
      (if (`self.CanHover`)
        _))
    (:`then_2`
      (set `self.RememberedScale` (`SceneComponent.K2_GetComponentScale` (`self.Plane`))))))