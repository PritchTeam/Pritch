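; BP_JumpBaseComponent is a base jump component for BP_MainCharacter.
; On BeginPlay it casts its owner to that character and caches it as OwnChar, which GetOwningChar returns.
; Jump forwards to the character's Jump, and OnLand sets its CurrentMovement to a fixed enum value.
; StopJumping and GetJumpCount are empty stubs.
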(event `self.ReceiveBeginPlay`
  (bind _asbp_main_character (cast `/Game/00_Lin/Character/BP_MainCharacter` (`self.GetOwner`)))
  (set `self.OwnChar` _asbp_main_character))

(fn `GetJumpCount`)

(fn `GetOwningChar`
  (returns (OwnChar :type "/Game/00_Lin/Character/BP_MainCharacter Object Reference"))
  (return (`self.OwnChar`)))

(fn `Jump`
  (`Character.Jump` (`self.OwnChar`)))

(fn `OnLand`
  (set `/Game/00_Lin/Character/BP_MainCharacter.Current Movement` "NewEnumerator17" (`self.OwnChar`)))

(fn `StopJumping`)