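; BP_GlideComponent is a character jump component that adds a glide whenever Jump is called.
; Jump runs the parent jump, then enables tick and restarts a timer; the CanJump check is disconnected.
; Each tick, a float curve sets a floor on vertical velocity, while MaxWalkSpeed grows cumulatively without being restored here.
; StopJumping or passing the curve's end disables tick, ending the glide.
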(event `self.ReceiveTick`
  (params (DeltaSeconds :type "Float (single-precision)"))
  (`self.TickGlide` DeltaSeconds))

(fn `BeginGlide`
  (`self.SetComponentTickEnabled` true)
  (set `self.GlideTimer` (`CurveBase.GetTimeRange` (`self.GlideCurve`)))
  (`KismetSystemLibrary.PrintString` "GLIDE" true true (struct :`R` 1.0 :`G` 0.698709 :`A` 1.0)))

(fn `EndGlide`
  (`self.SetComponentTickEnabled` false))

(fn `Jump`
  (`parent.Jump`)
  (`self.BeginGlide`))

(fn `StopJumping`
  (`self.EndGlide`)
  (`parent.StopJumping`))

(fn `TickGlide`
  (params (DeltaSeconds :type "Float (double-precision)"))
  (bind (_mintime _maxtime) (`CurveBase.GetTimeRange` (`self.GlideCurve`)))
  (bind _charactermovement (`Character.CharacterMovement` (`self.GetOwningChar`)))
  (bind (_velocity_x _velocity_y _velocity_z) (`KismetMathLibrary.BreakVector` (`MovementComponent.Velocity` _charactermovement)))
  (bind _output_get (set `self.GlideTimer` (+ (`self.GlideTimer`) DeltaSeconds)))
  (if (`KismetMathLibrary.InRange_FloatFloat` _output_get _mintime _maxtime)
    (set `MovementComponent.Velocity` (`KismetMathLibrary.MakeVector` _velocity_x _velocity_y (`KismetMathLibrary.FMax` _velocity_z (`CurveFloat.GetFloatValue` (`self.GlideCurve`) (`self.GlideTimer`)))) _charactermovement)
    (set `CharacterMovementComponent.MaxWalkSpeed` (+ (`CharacterMovementComponent.MaxWalkSpeed` _charactermovement) 1000.0) _charactermovement)
    (else
      (`self.EndGlide`))))