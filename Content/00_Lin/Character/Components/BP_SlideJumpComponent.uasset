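; Character jump component that adds a slide jump, a curve-driven horizontal boost, to the inherited jump.
; Jump calls the parent, then enables component tick and resets a timer to the start of SlideJumpCurve.
; Each tick overwrites horizontal velocity with first-person camera forward minus WishDir, scaled by the curve, preserving vertical velocity.
; Tick is disabled when the timer leaves the curve's range or jumping stops.
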(event `self.ReceiveTick`
  (params (DeltaSeconds :type "Float (single-precision)"))
  (`self.TickSlideJump` DeltaSeconds))

(fn `BeginSlideJump`
  (`self.SetComponentTickEnabled` true)
  (set `self.SlideJumpTimer` (`CurveBase.GetTimeRange` (`self.SlideJumpCurve`))))

(fn `EndSlideJump`
  (`self.SetComponentTickEnabled` false))

(fn `Jump`
  (`parent.Jump`)
  (`self.BeginSlideJump`))

(fn `StopJumping`
  (`self.EndSlideJump`)
  (`parent.StopJumping`))

(fn `TickSlideJump`
  (params (DeltaSeconds :type "Float (double-precision)"))
  (bind _ownchar (`self.GetOwningChar`))
  (bind (_mintime _maxtime) (`CurveBase.GetTimeRange` (`self.SlideJumpCurve`)))
  (bind _charactermovement (`Character.CharacterMovement` _ownchar))
  (bind (_velocity_x _velocity_y _velocity_z) (`KismetMathLibrary.BreakVector` (`MovementComponent.Velocity` _charactermovement)))
  (bind (_returnvalue_x _returnvalue_y) (`KismetMathLibrary.BreakVector` (* (- (`SceneComponent.GetForwardVector` (`/Game/00_Lin/Character/BP_MainCharacter.FirstPersonCamera` _ownchar)) (`/Game/00_Lin/Character/BP_MainCharacter.Wish Dir` _ownchar)) (`CurveFloat.GetFloatValue` (`self.SlideJumpCurve`) (`self.SlideJumpTimer`)))))
  (bind _output_get (set `self.SlideJumpTimer` (+ (`self.SlideJumpTimer`) DeltaSeconds)))
  (if (`KismetMathLibrary.InRange_FloatFloat` _output_get _mintime _maxtime)
    (bind _output_get_2 (set `MovementComponent.Velocity` (`KismetMathLibrary.MakeVector` _returnvalue_x _returnvalue_y _velocity_z) _charactermovement))
    (set `self.NewVar` _output_get_2)
    (else
      (`self.EndSlideJump`))))