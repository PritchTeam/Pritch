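; Character movement component that turns the jump action into a sideways dash, left or right based on the owner's RightMovement.
; Jump enables component tick, which drives horizontal velocity from a float curve over time while preserving vertical velocity.
; When the curve ends, tick switches off, CanDash resets and BP_MainCharacter's StopDash is called.
; Air-strafe limit, cooldown timer and forward-direction fallback are present but unwired.
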(event `self.ReceiveTick`
  (params (DeltaSeconds :type "Float (single-precision)"))
  (`self.TickStrafe` DeltaSeconds))

(fn `BeginStrafe`
  (bind _ownchar (`self.GetOwningChar`))
  (bind _returnvalue (`Actor.GetActorRightVector` _ownchar))
  (`self.SetComponentTickEnabled` true)
  (set `self.StrafeTimer` (`CurveBase.GetTimeRange` (`self.StraveCurve`)))
  (set `self.CanDash` false)
  (set `self.StrafeDir` (`KismetMathLibrary.Normal2D` (`KismetMathLibrary.Conv_VectorToVector2D` (`KismetMathLibrary.SelectVector` _returnvalue (* _returnvalue -1.0) (`/Game/00_Lin/Character/BP_MainCharacter.RightMovement` _ownchar)))))
  (set `self.Finished` false))

(fn `EndStrafe`
  (`self.SetComponentTickEnabled` false)
  (set `self.CanDash` true))

(fn `Jump`
  (if (not (`self.IsComponentTickEnabled`))
    (`self.BeginStrafe`)))

(fn `OnLand`
  (`parent.OnLand`))

(fn `ResetStrafe`
  (set `self.CanDash` true))

(fn `StopJumping`
  (`parent.StopJumping`))

(fn `TickStrafe`
  (params (`Delta Seconds` :type "Float (double-precision)"))
  (bind (_mintime _maxtime) (`CurveBase.GetTimeRange` (`self.StraveCurve`)))
  (bind _charactermovement (`Character.CharacterMovement` (`self.GetOwningChar`)))
  (bind (_returnvalue_x _returnvalue_y) (`KismetMathLibrary.BreakVector2D` (* (`self.StrafeDir`) (`CurveFloat.GetFloatValue` (`self.StraveCurve`) (`self.StrafeTimer`)))))
  (bind (_velocity_x _velocity_y _velocity_z) (`KismetMathLibrary.BreakVector` (`MovementComponent.Velocity` _charactermovement)))
  (bind _output_get (set `self.StrafeTimer` (+ (`self.StrafeTimer`) `Delta Seconds`)))
  (if (`KismetMathLibrary.InRange_FloatFloat` _output_get _mintime _maxtime)
    (set `MovementComponent.Velocity` (`KismetMathLibrary.MakeVector` _returnvalue_x _returnvalue_y _velocity_z) _charactermovement)
    (set `self.Finished` false)
    (else
      (`self.EndStrafe`)
      (set `self.Finished` true)
      (bind _asbp_main_character (cast `/Game/00_Lin/Character/BP_MainCharacter` (`self.GetOwner`)))
      (`/Game/00_Lin/Character/BP_MainCharacter.Stop Dash` _asbp_main_character))))