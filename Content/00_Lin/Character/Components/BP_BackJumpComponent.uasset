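; Jump component that makes the character leap backward, then triggers slow motion on BP_MainCharacter when the leap ends.
; Jump calls the parent jump and enables tick, which drives velocity opposite the actor's facing from BJumpCurve, with a curve-scaled minimum upward speed.
; Running past the curve's time range or stopping the jump disables tick and starts the slow motion.
; Strafe-direction logic is present but never runs.
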(event `self.ReceiveTick`
  (params (DeltaSeconds :type "Float (single-precision)"))
  (`self.TickBJump` DeltaSeconds))

(fn `BeginBJump`
  (`self.SetComponentTickEnabled` true)
  (set `self.BJumpTimer` (`CurveBase.GetTimeRange` (`self.BJumpCurve`)))
  (`KismetSystemLibrary.PrintString` "back jumping"))

(fn `EndBJump`
  (`self.SetComponentTickEnabled` false)
  (bind _asbp_main_character (cast `/Game/00_Lin/Character/BP_MainCharacter` (`self.GetOwner`)))
  (set `/Game/00_Lin/Character/BP_MainCharacter.slow mo timer (changed)` 8.0 _asbp_main_character)
  (`/Game/00_Lin/Character/BP_MainCharacter.Start Slow-mo` _asbp_main_character))

(fn `Jump`
  (if (not (`self.IsComponentTickEnabled`))
    (`parent.Jump`)
    (`self.BeginBJump`)))

(fn `OnLand`
  (`parent.OnLand`))

(fn `StopJumping`
  (`self.EndBJump`)
  (`parent.StopJumping`))

(fn `TickBJump`
  (params (DeltaSeconds :type "Float (double-precision)"))
  (bind _ownchar (`self.GetOwningChar`))
  (bind (_mintime _maxtime) (`CurveBase.GetTimeRange` (`self.BJumpCurve`)))
  (bind (_returnvalue_x _returnvalue_y _returnvalue_z) (`KismetMathLibrary.BreakVector` (`Actor.GetVelocity` _ownchar)))
  (bind _returnvalue (`CurveFloat.GetFloatValue` (`self.BJumpCurve`) (`self.BJumpTimer`)))
  (bind (_returnvalue_x_2 _returnvalue_y_2) (`KismetMathLibrary.BreakVector` (* (* (`Actor.GetActorForwardVector` (`self.GetOwningChar`)) (-1.0 -1.0 0.0)) _returnvalue)))
  (bind _output_get (set `self.BJumpTimer` (+ (`self.BJumpTimer`) DeltaSeconds)))
  (if (`KismetMathLibrary.InRange_FloatFloat` _output_get _mintime _maxtime)
    (set `MovementComponent.Velocity` (`KismetMathLibrary.MakeVector` _returnvalue_x_2 _returnvalue_y_2 (`KismetMathLibrary.FMax` (/ _returnvalue 10.0) _returnvalue_z)) (`Character.CharacterMovement` _ownchar))
    (else
      (`self.EndBJump`))))