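; Player bow weapon that handles aiming, charged shots, reloading and arrow-type switching for BP_MainCharacter.
; Aim timelines tighten the crosshair and build arrow velocity, and release spawns BP_ProjectileArrow, with random spread on weaker draws, then animates a reload.
; Aiming while falling, sliding or gliding with enough stamina triggers delayed global slow motion, with key timelines ignoring dilation.
; Strong mode fires homing arrows at targeted enemies on a looping timer.
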(event `self.ReceiveBeginPlay`
  (bind _bowmesh (`self.BowMesh`))
  (bind _returnvalue (`GameplayStatics.GetActorOfClass` "/Game/00_Lin/Character/BP_MainCharacter.BP_MainCharacter_C"))
  ;[1 1 1] Set Up
  (set `self.CharRef` _returnvalue)
  (set `self.ArrowDefaultLocation` (`SceneComponent.RelativeLocation` (`self.ArrowMesh`)))
  (set `self.Bow Relative Location` (`SceneComponent.RelativeLocation` _bowmesh))
  (set `self.Bow Relative Rotation` (`SceneComponent.RelativeRotation` _bowmesh)))

(event `Move Bow`
  (bind _charref (`self.CharRef`))
  ;[1 0.2982 0.005113] Tilt Bow Anim
  (`TimelineComponent.SetPlayRate` (`self.Bow Aim`) 2.0)
  (bind (_direction _move) (`Timeline|Bow Aim` :!via `PlayFromStart` :!label _label)
    (:`Update`
      (if (>= _move 1.0)
        (`/Game/00_Lin/CharacterUI/Crosshair/WBP_RoundCrosshair.ChangeRadius` (`/Game/00_Lin/Character/BP_MainCharacter.RoundCrosshair` _charref) 0.7)
        (`TimelineComponent.SetPlayRate` (`self.Finishing Radius`) 1.5)
        (bind (_direction_2 _move_2) (`Timeline|Finishing Radius` :!via `PlayFromStart` :!label _label_2)
          (:`Update`
            (`/Game/00_Lin/CharacterUI/Crosshair/WBP_RoundCrosshair.ChangeRadius` (`/Game/00_Lin/Character/BP_MainCharacter.RoundCrosshair` _charref) (`KismetMathLibrary.Lerp` 0.7 0.2 _move_2))))
        (else
          (bind _returnvalue (`KismetMathLibrary.Lerp` 1.0 0.7 _move))
          (set `self.CrosshairRadius` _returnvalue)
          (`/Game/00_Lin/CharacterUI/Crosshair/WBP_RoundCrosshair.ChangeRadius` (`/Game/00_Lin/Character/BP_MainCharacter.RoundCrosshair` (`self.CharRef`)) _returnvalue))))))

(event `Stop Bow Move`
  ;[1 0.2982 0.005113] Tilt Bow Anim
  (`|ExecutionSequence`
    (:`then_0`
      (goto _label :!via `Stop`))
    (:`then_1`
      (goto _label_2 :!via `Stop`))
    (:`then_2`
      (`TimelineComponent.SetPlayRate` (`self.BowReturn`) 3.0)
      (bind (_direction _move) (`Timeline|BowReturn`)
        (:`Update`
          (`SceneComponent.K2_SetRelativeLocationAndRotation` (`self.BowMesh`) (`self.Bow Relative Location`) (`KismetMathLibrary.RLerp` (struct :`Pitch` 90.0) (struct :`Pitch` 90.0) _move) false false))))))

(event `Aim`
  (params (`Trigger Down` :type Boolean))
  ;[1 1 1] Aim
  (if `Trigger Down`
    (set `self.Aiming` true)
    (`self.Move Bow`)
    (`self.Move Arrow`)
    (`self.Can Slow-mo?`)
    (set `self.Current Bow Stage` "NewEnumerator0")
    (else
      (set `self.Aiming` false)
      (`self.Stop Aim` false)
      (`self.Shoot Arrow` false)
      (`self.Arrow Animation`)
      (`NiagaraFunctionLibrary.SpawnSystemAtLocation` "/Game/00_Lin/VFX/Character/StaminaVFX/NS_CoinBurst.NS_CoinBurst" (`SceneComponent.K2_GetComponentLocation` (`self.NiagaraSpark`))))))

(event `Move Arrow`
  (bind _arrowdefaultlocation (`self.ArrowDefaultLocation`))
  ;[1 0.3634 0] Aim Arrow Anim
  (`TimelineComponent.SetPlayRate` (`self.Arrow Aim`) 2.0)
  (bind (_direction _move) (`Timeline|Arrow Aim` :!via `PlayFromStart`)
    (:`Update`
      (`SceneComponent.K2_SetRelativeLocation` (`self.ArrowMesh`) (`KismetMathLibrary.VLerp` _arrowdefaultlocation _arrowdefaultlocation _move) false false)
      (set `self.Arrow Velocity` (`KismetMathLibrary.Lerp` 500.0 (`self.Arrow Velocity Max`) _move)))))

(event `Stop Aim`
  (params (`Stop Stage?` :type Boolean))
  ;[1 1 1] Reset Settings
  (`self.Stop Bow Move`)
  (`/Game/00_Lin/CharacterUI/Crosshair/WBP_RoundCrosshair.ReturnRadius` (`/Game/00_Lin/Character/BP_MainCharacter.RoundCrosshair` (`self.CharRef`)))
  (`self.Stop Slow Mo`)
  (if (not `Stop Stage?`)
    (set `self.Current Bow Stage` "NewEnumerator10")))

(event `Stop Slow Mo`
  (bind _slowmowbp (`self.SlowMoWBP`))
  (bind _charref (`self.CharRef`))
  (bind _slowmo_pp (`self.SlowMo_PP`))
  ;[1 1 1] Reset Settings
  (`|ExecutionSequence`
    (:`then_0`
      (`KismetSystemLibrary.K2_ClearAndInvalidateTimerHandle` (`self.Slow Mo Timer`))
      (`/Engine/EditorBlueprintResources/StandardMacros.IsValid` _slowmo_pp
        (:`Is Valid`
          (`ActorComponent.K2_DestroyComponent` _slowmo_pp))
        (:`Is Not Valid`
          _))
      (`GameplayStatics.SetGlobalTimeDilation` 1.0)
      (set `SpringArmComponent.bEnableCameraRotationLag` true (`/Game/00_Lin/Character/BP_MainCharacter.BowSpringArm` _charref))
      (set `/Game/00_Lin/Character/BP_MainCharacter.slow mo timer (changed)` (`/Game/00_Lin/Character/BP_MainCharacter.slow mo timer (default)` _charref) _charref))
    (:`then_1`
      (`/Engine/EditorBlueprintResources/StandardMacros.IsValid` _slowmowbp
        (:`Is Valid`
          (`Widget.RemoveFromParent` _slowmowbp))))))

(event `Arrow Animation`
  (bind _arrowmesh (`self.ArrowMesh`))
  ;[1 0.3905 0] Load Arrow Anim
  (set `self.Arrow In?` false)
  (`SceneComponent.SetVisibility` _arrowmesh false false)
  (`SceneComponent.K2_SetRelativeLocation` (`self.ArrowMesh`) (`SceneComponent.RelativeLocation` (`self.LoadArrowLoc`)) false false)
  (`KismetSystemLibrary.Delay` 0.2)
  (`SceneComponent.SetVisibility` _arrowmesh true false)
  (`TimelineComponent.SetPlayRate` (`self.Load Arrow`) 3.0)
  (bind (_direction _move) (`Timeline|Load Arrow` :!via `PlayFromStart`)
    (:`Update`
      (`SceneComponent.K2_SetRelativeLocation` (`self.ArrowMesh`) (`KismetMathLibrary.VLerp` (`SceneComponent.RelativeLocation` (`self.ArrowMesh`)) (`self.ArrowDefaultLocation`) _move) false false)
      (set `self.Arrow In?` true))))

(event `Shoot Arrow`
  (params (`Is homing?` :type Boolean))
  (bind _arrow_spread (`self.Arrow Spread`))
  (bind _arrow_velocity (`self.Arrow Velocity`))
  (bind _returnvalue (* _arrow_spread -1.0))
  (bind _aim1 (`/Game/00_Lin/Character/BP_MainCharacter.Aim1` (`self.CharRef`)))
  (bind _returnvalue_2 (`SceneComponent.K2_GetComponentLocation` _aim1))
  ;[1 1 1] Spawn Arrow
  (if `Is homing?`
    (`self.Homing Set Up` null)
    (else
      (`|SpawnActorFromClass` "/Game/00_Lin/Weapon/BP_ProjectileArrow.BP_ProjectileArrow_C" (`KismetMathLibrary.MakeTransform` (`KismetMathLibrary.SelectVector` (+ _returnvalue_2 (`KismetMathLibrary.MakeVector` (`KismetMathLibrary.RandomFloatInRange` _returnvalue _arrow_spread) (`KismetMathLibrary.RandomFloatInRange` _returnvalue _arrow_spread) (`KismetMathLibrary.RandomFloatInRange` _returnvalue _arrow_spread))) _returnvalue_2 (< _arrow_velocity 5000.0)) (`SceneComponent.K2_GetComponentRotation` _aim1)) "Undefined" "OverrideRootScale" null (`KismetMathLibrary.SelectFloat` (* _arrow_velocity 2.0) (* _arrow_velocity 5.0) (< _arrow_velocity 4000.0)) (`self.Arrow Type`) null))))

(event `Start Slow-mo`
  (bind _charref (`self.CharRef`))
  ;[0.429 1 0.01729] Slow Mo
  (`GameplayStatics.SetGlobalTimeDilation` (`self.Slow Mo`))
  (set `Actor.CustomTimeDilation` 1.0 (`self.CharRef`))
  (`TimelineComponent.SetIgnoreTimeDilation` (`self.Bow Aim`) true)
  (`TimelineComponent.SetIgnoreTimeDilation` (`self.Arrow Aim`) true)
  (`TimelineComponent.SetIgnoreTimeDilation` (`self.Load Arrow`) true)
  (`TimelineComponent.SetIgnoreTimeDilation` (`/Game/00_Lin/Character/BP_MainCharacter.Zoom` (`self.CharRef`)) true)
  (set `SpringArmComponent.bEnableCameraRotationLag` false (`/Game/00_Lin/Character/BP_MainCharacter.BowSpringArm` (`self.CharRef`)))
  (`TimelineComponent.SetIgnoreTimeDilation` (`/Game/00_Lin/Character/BP_MainCharacter.Slow Mo Timer` _charref) true)
  (`TimelineComponent.SetIgnoreTimeDilation` (`self.Finishing Radius`) true)
  (if (not (== (`/Game/00_Lin/Character/BP_MainCharacter.slow mo timer (changed)` _charref) 0.0))
    (`/Game/00_Lin/Character/BP_MainCharacter.Open Tick Slow Mo` _charref))
  (`/Engine/EditorBlueprintResources/StandardMacros.DoOnce` false :!label _label_3
    (:`Completed`
      (bind _returnvalue (`|CreateWidget` "/Game/00_Lin/VFX/Character/WBP_SlowMo.WBP_SlowMo_C"))
      (`UserWidget.AddToViewport` _returnvalue 0)
      (set `self.SlowMoWBP` _returnvalue))))

(event `Can Slow-mo?`
  (bind _charref (`self.CharRef`))
  ;[0.429 1 0.01729] Slow Mo
  (if (>= (`/Game/00_Lin/Character/BP_MainCharacter.Stamina` _charref) (`/Game/00_Lin/Character/BP_MainCharacter.Slide Stamina` _charref))
    (if (or (`NavMovementComponent.IsFalling` (`Character.CharacterMovement` (`self.CharRef`))) (`self.Is Sliding`) (`self.Is Gliding`))
      (bind _returnvalue (`KismetSystemLibrary.K2_SetTimerDelegate` (delegate `Start Slow-mo`) 0.4))
      (set `self.Slow Mo Timer` _returnvalue)
      (goto _label_3 :!via `Reset`))))

(event `Strong Bow`
  ;[1 1 1] Strong Arrow Throw
  (bind _returnvalue (`KismetSystemLibrary.K2_SetTimer` null "StrongThrowArrows" (`self.Time Between Shots`) true))
  (set `self.Strong Arrows Timer` _returnvalue))

(event `Change Arrow`
  (params (RowName :type Name) (`Arrow Type` :type "/Game/00_Lin/Craft/Recipes/E_ArrowID Enum" :default "NewEnumerator0"))
  ;[1 1 1] Arrow Change
  (bind _returnvalue (`DataTableFunctionLibrary.DoesDataTableRowExist` "/Game/00_Lin/Craft/DT_Recipes.DT_Recipes" RowName))
  (if _returnvalue
    (bind _returnvalue_2 (`|GetDataTableRow` "/Game/00_Lin/Craft/DT_Recipes.DT_Recipes" RowName)
      (:`then`
        (`NiagaraComponent.SetAsset` (`self.Niagara`) (`.Niagara_33_32B7A04A450CD9D2D90602BC5263EF94` (break `/Game/00_Lin/Craft/Recipes/S_Recipes` _returnvalue_2)) true)
        (set `self.Arrow Type` `Arrow Type`)))))

(fn `Homing Set Up`
  (params (Arrow :type "/Game/00_Lin/Weapon/BP_ProjectileArrow Object Reference"))
  (bind _completed_enemies (`self.Completed Enemies`))
  (bind _targeted_enemies (`/Game/00_Lin/Character/BP_MainCharacter.Targeted Enemies` (`self.CharRef`)))
  (bind _aim1 (`/Game/00_Lin/Character/BP_MainCharacter.Aim1` (`self.CharRef`)))
  (bind _output (`|GetArrayItem` _targeted_enemies))
  (bind _returnvalue (/ (`KismetMathLibrary.Round` (`self.Strong Arrow Amount`)) 2))
  (bind _output_2 (`|GetArrayItem` _targeted_enemies _returnvalue))
  (bind _returnvalue_2 (`|SpawnActorFromClass` "/Game/00_Lin/Weapon/BP_ProjectileArrow.BP_ProjectileArrow_C" (`KismetMathLibrary.MakeTransform` (`SceneComponent.K2_GetComponentLocation` _aim1) (`SceneComponent.K2_GetComponentRotation` _aim1)) "Undefined" "OverrideRootScale" null 100.0 "NewEnumerator0" null))
  (if (== (`KismetArrayLibrary.Array_Length` _targeted_enemies) 1)
    (bind _projectilemovement (`/Game/00_Lin/Weapon/BP_ProjectileArrow.ProjectileMovement` _returnvalue_2))
    (set `ProjectileMovementComponent.HomingTargetComponent` (`/Game/00_Sanya/AI/NPCCharacters/BaseNPC/BP_BaseShooterNPC.Sphere1` _output) _projectilemovement)
    (set `ProjectileMovementComponent.HomingAccelerationMagnitude` 100000.0 _projectilemovement)
    (`KismetArrayLibrary.Array_Add` (`self.Completed Enemies`) _output)
    (else
      (`KismetSystemLibrary.PrintString` (`KismetStringLibrary.Conv_IntToString` _returnvalue) true true (struct :`R` 0.751891 :`G` 1.0 :`A` 1.0))
      (bind _projectilemovement_2 (`/Game/00_Lin/Weapon/BP_ProjectileArrow.ProjectileMovement` _returnvalue_2))
      (set `ProjectileMovementComponent.HomingTargetComponent` (`/Game/00_Sanya/AI/NPCCharacters/BaseNPC/BP_BaseShooterNPC.Sphere1` _output_2) _projectilemovement_2)
      (set `ProjectileMovementComponent.HomingAccelerationMagnitude` 100000.0 _projectilemovement_2)
      (if (== (`KismetArrayLibrary.Array_Find` _completed_enemies _output_2) -1)
        (`KismetArrayLibrary.Array_Add` _completed_enemies _output_2)))))

(fn `StrongThrowArrows`
  (bind _charref (`self.CharRef`))
  (set `self.Arrow Velocity` (`self.Arrow Velocity Max`))
  (`self.Shoot Arrow` true)
  (`self.Arrow Animation`)
  (set `self.Strong Arrow Amount` (+ (`self.Strong Arrow Amount`) 1.0))
  (if (>= (- (`KismetArrayLibrary.Array_Length` (`self.Completed Enemies`)) 1) (`KismetArrayLibrary.Array_Length` (`/Game/00_Lin/Character/BP_MainCharacter.Targeted Enemies` (`self.CharRef`))))
    (`/Game/00_Lin/Character/BP_MainCharacter.Return StrongBow to Normal` _charref)
    (`/Game/00_Lin/Character/BP_MainCharacter.Throw Bow` _charref false)))

(fn `UserConstructionScript`)