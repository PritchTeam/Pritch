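; Arrow projectile fired from the player character's bow, with initial speed set in construction and a trail whose start socket follows bow velocity.
; Hits on hit-point interface actors deal velocity-scaled damage, then after a delay update the bow's strong-hit streak by stage and destroy the arrow.
; Other valid hits spawn a flash, while bullets are destroyed and grenades detonated with punch effects.
; The trail deactivates on impact.
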(event `self.ReceiveTick`
  (params (DeltaSeconds :type "Float (single-precision)"))
  (bind _trail (`self.Trail`))
  (if (< (`/Game/00_Lin/Weapon/BP_BowNew.Arrow Velocity` (`self.Bow Ref`)) 4000.0)
    (`FXSystemComponent.SetVectorParameter` _trail "StartSocket" (`SceneComponent.GetSocketLocation` (`self.StaticMesh`) "Trail2"))
    (else
      (`FXSystemComponent.SetVectorParameter` _trail "StartSocket" (`SceneComponent.GetSocketLocation` (`self.StaticMesh`) "Trail3")))))

(event `self.ReceiveBeginPlay`
  (bind _asbp_main_character (cast `/Game/00_Lin/Character/BP_MainCharacter` (`GameplayStatics.GetPlayerCharacter` 0)))
  (set `self.Bow Ref` (`/Game/00_Lin/Character/BP_MainCharacter.Bow Ref New` _asbp_main_character)))

(event `self.ReceiveHit`
  (params (MyComp :type "PrimitiveComponent Object Reference") (Other :type "Actor Object Reference") (OtherComp :type "PrimitiveComponent Object Reference") (bSelfMoved :type Boolean) (HitLocation :type "Vector Structure") (HitNormal :type "Vector Structure") (NormalImpulse :type "Vector Structure") (Hit :type "HitResult Structure (by ref)"))
  (bind (_bblockinghit _binitialoverlap _time _distance _location _impactpoint _normal _impactnormal _physmat _hitactor) (`GameplayStatics.BreakHitResult` Hit))
  (bind _bow_ref (`self.Bow Ref`))
  (bind _bow_ref_2 (`self.Bow Ref`))
  (`|ExecutionSequence`
    (:`then_0`
      (`/Engine/EditorBlueprintResources/StandardMacros.IsValid` _hitactor
        (:`Is Valid`
          (if (`KismetSystemLibrary.DoesImplementInterface` _hitactor "/Game/00_Sanya/AI/Utility/Components/BPI_HitPointsInterface.BPI_HitPointsInterface_C")
            (message `/Game/00_Sanya/AI/Utility/Components/BPI_HitPointsInterface.ReceiveDamage` _hitactor (`KismetMathLibrary.FTrunc` (* (/ (`/Game/00_Lin/Weapon/BP_BowNew.Arrow Velocity` _bow_ref) (`/Game/00_Lin/Weapon/BP_BowNew.Arrow Velocity Max` _bow_ref)) (`KismetMathLibrary.Conv_IntToDouble` (`self.Damage`)))))
            (`KismetSystemLibrary.Delay` 2.0)
            (if (`|EnumEquality` (`/Game/00_Lin/Weapon/BP_BowNew.Current Bow Stage` _bow_ref_2) "NewEnumerator5")
              (set `/Game/00_Lin/Weapon/BP_BowNew.Strong Arrow Hit` (+ (`/Game/00_Lin/Weapon/BP_BowNew.Strong Arrow Hit` _bow_ref_2) 1) _bow_ref_2)
              (else
                (set `/Game/00_Lin/Weapon/BP_BowNew.Strong Arrow Hit` 0 _bow_ref_2)))
            (`self.K2_DestroyActor`)
            (else
              (`NiagaraFunctionLibrary.SpawnSystemAtLocation` "/Game/00_Lin/VFX/Bow/Flash/NS_Flash.NS_Flash" HitLocation (struct) (0.2 0.2 0.2)))))))
    (:`then_1`
      (bind _asebbullet (cast `EBBullet` _hitactor)
        (:`then`
          (`NiagaraFunctionLibrary.SpawnSystemAtLocation` "/Game/00_Lin/VFX/Enemy/NS_Punch.NS_Punch" (`KismetMathLibrary.MakeVector` (+ (.x (`self.K2_GetActorLocation` _asebbullet)) 150.0) (+ (.y (`self.K2_GetActorLocation` _asebbullet)) 150.0) (.z (`self.K2_GetActorLocation` _asebbullet))) (struct) (0.2 0.2 0.2))
          (`self.K2_DestroyActor` _asebbullet))
        (:`CastFailed`
          (bind _asbp_base_grenade (cast `/Game/00_Sanya/AI/NPCCharacters/BaseNPC/BP_BaseGrenade` _hitactor))
          (`NiagaraFunctionLibrary.SpawnSystemAtLocation` "/Game/00_Lin/VFX/Enemy/NS_Punch.NS_Punch" (`KismetMathLibrary.MakeVector` (.x (`self.K2_GetActorLocation` _asbp_base_grenade)) (- (.y (`self.K2_GetActorLocation` _asbp_base_grenade)) 150.0) (.z (`self.K2_GetActorLocation` _asbp_base_grenade))) (struct) (5.0 5.0 5.0))
          (`/Game/00_Sanya/AI/NPCCharacters/BaseNPC/BP_BaseGrenade.Explosion` _asbp_base_grenade))))
    (:`then_2`
      (`ActorComponent.Deactivate` (`self.Trail`)))))

(fn `UserConstructionScript`
  (set `ProjectileMovementComponent.InitialSpeed` (`self.initialspeed`) (`self.ProjectileMovement`)))