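; Player bow weapon (apparently a backup) that handles aiming, drawing and firing arrows.
; Shoot raises the bow and runs a draw timeline driving arrow velocity, crosshair spread and nock position; release spawns BP_ProjectileArrow, scattered at low velocity.
; Drawing while falling, sliding or gliding with enough stamina triggers timed global slow motion, with bow timelines ignoring dilation.
; A strong-throw mode fires a timed arrow volley, then has the character throw the bow.
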(event `self.ReceiveBeginPlay`
  ;[1 0.195 0] SetUp
  (`parent.ReceiveBeginPlay`)
  (set `self.ArrowDefaultLocation` (`SceneComponent.RelativeLocation` (`self.ArrowMesh`)))
  (bind _asbp_main_character (cast `/Game/00_Lin/Character/BP_MainCharacter` (`GameplayStatics.GetPlayerCharacter` 0)))
  (set `self.Char_Ref` _asbp_main_character)
  (`self.Move Bow` (`self.BowMesh_down`)))

(event `self.Shoot`
  (params (TriggerDown :type Boolean) (Spread :type "Float (single-precision)"))
  ;[0 0.4836 1] Draw Arrow
  ;[0.1017 0.4719 1] Shoot
  (`KismetSystemLibrary.K2_ClearAndInvalidateTimerHandle` (`self.SlowMoTimer`))
  (if TriggerDown
    (`self.Aim`)
    (else
      (`self.Stop Aim`)
      (`self.NoBarrelShoot`)
      (`self.ArrowAnimation`)
      (`NiagaraFunctionLibrary.SpawnSystemAtLocation` "/Game/00_Lin/VFX/Character/StaminaVFX/NS_CoinBurst.NS_CoinBurst" (`SceneComponent.K2_GetComponentLocation` (`self.NiagaraSpark`))))))

(event `ArrowAnimation`
  (bind (_arrowdefaultlocation_x _arrowdefaultlocation_y _arrowdefaultlocation_z) (`KismetMathLibrary.BreakVector` (`self.ArrowDefaultLocation`)))
  ;[0.1017 0.4719 1] Shoot
  (set `self.ArrowIn` false)
  (`SceneComponent.SetVisibility` (`self.ChangingArrow`) false false)
  (`KismetSystemLibrary.Delay` 0.1)
  (`TimelineComponent.SetPlayRate` (`self.ArrowAnim`) 4.0)
  (bind (_direction _newtrack_0) (`Timeline|ArrowAnim` :!via `PlayFromStart`)
    (:`Update`
      (`SceneComponent.K2_SetRelativeLocation` (`self.ArrowMesh`) (`KismetMathLibrary.VLerp` (`KismetMathLibrary.MakeVector` (+ _arrowdefaultlocation_x 50.0) _arrowdefaultlocation_y _arrowdefaultlocation_z) (`self.ArrowDefaultLocation`) _newtrack_0) false false)
      (`SceneComponent.SetVisibility` (`self.ChangingArrow`) true false))
    (:`Finished`
      (set `self.ArrowIn` true))))

(event `PlayFromStartTimeline`
  (bind (_arrowdefaultlocation_x _arrowdefaultlocation_y _arrowdefaultlocation_z) (`KismetMathLibrary.BreakVector` (`self.ArrowDefaultLocation`)))
  ;[0 0.4836 1] Draw Arrow
  (set `self.IsShooting` true)
  (bind (_direction _draw) (`Timeline|DrawArrow` :!via `PlayFromStart` :!label _label)
    (:`Update`
      (set `/Game/00_Lin/CharacterUI/WBP_Crosshair.crosshair_spread` (`KismetMathLibrary.Lerp` 27.0 5.0 _draw) (`/Game/00_Lin/Character/BP_MainCharacter.Crosshair` (`self.Char_Ref`)))
      (if (not (`self.is bow thrown`))
        (`SceneComponent.K2_SetRelativeLocation` (`self.ArrowMesh`) (`KismetMathLibrary.MakeVector` (+ (`KismetMathLibrary.Lerp` 0.0 -22.0 _draw) _arrowdefaultlocation_x) _arrowdefaultlocation_y _arrowdefaultlocation_z) false false))
      (set `self.UsedBlowbackMultiplier` (`KismetMathLibrary.Lerp` 0.0 (`self.BlowbackMultiplier`) _draw))
      (set `self.ArrowVelocity` (`KismetMathLibrary.Lerp` 500.0 (`.MuzzleVelocityMax` (defaults `Object` (`|GetArrayItem` (`EBBarrel.GetAmmo` (`self.EBBarrel`) false) (`self.EquippedArrow`)))) _draw))
      (set `self.ArrowInAlpha` _draw))
    (:`Finished`
      (`/Game/00_Lin/Character/BP_MainCharacter.Close Tick Strong Throw` (`self.Char_Ref`))
      (if (not (> (`GameplayStatics.GetGlobalTimeDilation`) (`self.SlowMo`)))
        (`Timeline|TimerSlowMo` :!via `PlayFromStart`
          (:`Finished`
            (`self.ResetSlowMoWithAim`)))))))

(event `StopTimeline`
  ;[0 0.4836 1] Draw Arrow
  (goto _label :!via `Stop`))

(event `NoBarrelShoot`
  (bind _arrowspread (`self.ArrowSpread`))
  (bind _arrowvelocity (`self.ArrowVelocity`))
  (bind _returnvalue (* _arrowspread -1.0))
  (bind _aim1 (`/Game/00_Lin/Character/BP_MainCharacter.Aim1` (`self.Char_Ref`)))
  (bind _returnvalue_2 (`SceneComponent.K2_GetComponentLocation` _aim1))
  ;[0 0.4601 1] Shoot Direction
  (`|SpawnActorFromClass` "/Game/00_Lin/Weapon/BP_ProjectileArrow.BP_ProjectileArrow_C" (`KismetMathLibrary.MakeTransform` (`KismetMathLibrary.SelectVector` (+ _returnvalue_2 (`KismetMathLibrary.MakeVector` (`KismetMathLibrary.RandomFloatInRange` _returnvalue _arrowspread) (`KismetMathLibrary.RandomFloatInRange` _returnvalue _arrowspread) (`KismetMathLibrary.RandomFloatInRange` _returnvalue _arrowspread))) _returnvalue_2 (< _arrowvelocity 5000.0)) (`SceneComponent.K2_GetComponentRotation` _aim1)) "Undefined" "OverrideRootScale" null (`KismetMathLibrary.SelectFloat` (* _arrowvelocity 2.0) (* _arrowvelocity 5.0) (< _arrowvelocity 4000.0)) null)
  (set `self.IsShooting` false)
  (if (< (`self.ArrowInAlpha`) 0.9)
    ;[1 0 0.02876] SHOOT
    (`GameplayStatics.PlaySound2D` "/Game/00_Anton/Sounds/PLR/CMBT/Bow/BowLightShot/PLR_CMBT_Bow_BowLightShot_Cue.PLR_CMBT_Bow_BowLightShot_Cue" 1.0 1.0 0.0 null null)
    (else
      ;[1 0 0.02876] STRONG SHOOT
      (`GameplayStatics.PlaySound2D` null 1.0 1.0 0.0 null null))))

(event `Aim`
  (bind _char_ref (`self.Char_Ref`))
  ;[0 0.6503 1] Aiming
  (set `self.aiming` true)
  (`self.Move Bow` (`self.BowMesh_up`))
  (if (>= (`/Game/00_Lin/Character/BP_MainCharacter.Stamina` _char_ref) (`/Game/00_Lin/Character/BP_MainCharacter.Slide Stamina` _char_ref))
    (if (`NavMovementComponent.IsFalling` (`Character.CharacterMovement` (`self.Char_Ref`)))
      (`/Engine/EditorBlueprintResources/StandardMacros.DoOnce` false :!label _label_2
        (:`Completed`
          (bind _returnvalue (`KismetSystemLibrary.K2_SetTimerDelegate` (delegate `Set SlowMo`) 0.2))
          (set `self.SlowMoTimer` _returnvalue)))
      (elif (or (`self.is sliding`) (`self.is gliding`))
        (goto _label_2)
        (else
          (`self.PlayFromStartTimeline` :!label _label_3)
          (set `self.TimeBetweenShots` 0.8))))
    (else
      (goto _label_3))))

(event `Reset Cooldown`
  ;[0 0.6503 1] Aiming
  (goto _label_2 :!via `Reset`))

(event `Set SlowMo`
  ;[0 0.6503 1] Aiming
  (`self.Slow Mo Sound`)
  (`GameplayStatics.SetGlobalTimeDilation` (`self.SlowMo`))
  (set `Actor.CustomTimeDilation` 1.0 (`self.Char_Ref`))
  (`TimelineComponent.SetIgnoreTimeDilation` (`self.DrawArrow`) true)
  (`TimelineComponent.SetIgnoreTimeDilation` (`self.Bow_Move`) true)
  (`TimelineComponent.SetIgnoreTimeDilation` (`/Game/00_Lin/Character/BP_MainCharacter.Zoom` (`self.Char_Ref`)) true)
  (`TimelineComponent.SetIgnoreTimeDilation` (`self.TimerSlowMo`) true)
  (`self.PlayFromStartTimeline`)
  (set `self.TimeBetweenShots` (- (`self.TimeBetweenShots`) 0.75))
  (`/Game/00_Lin/Character/BP_MainCharacter.DecreseStamina(SlowMo)` (`self.Char_Ref`)))

(event `Move Bow`
  (params (Target :type "SceneComponent Object Reference"))
  (bind _bowmesh (`self.BowMesh`))
  ;[0.1275 1 0.2907] Bow Rotation
  (`TimelineComponent.SetPlayRate` (`self.Bow_Move`) 3.0)
  (bind (_direction _move) (`Timeline|Bow_Move` :!via `PlayFromStart` :!label _label_4)
    (:`Update`
      (`SceneComponent.K2_SetRelativeLocationAndRotation` (`self.BowMesh`) (`KismetMathLibrary.VLerp` (`SceneComponent.RelativeLocation` _bowmesh) (`SceneComponent.RelativeLocation` Target) _move) (`KismetMathLibrary.RLerp` (`SceneComponent.RelativeRotation` _bowmesh) (`SceneComponent.RelativeRotation` Target) _move true) false false))))

(event `Stop Bow Move`
  ;[0.1275 1 0.2907] Bow Rotation
  (goto _label_4 :!via `Stop`))

(event `Stop Aim`
  (bind _char_ref (`self.Char_Ref`))
  ;[0 0.6503 1] Aiming
  (`KismetSystemLibrary.K2_ClearAndInvalidateTimerHandle` (`self.SlowMoTimer`))
  (set `self.aiming` false)
  (if (`|EnumEquality` (`self.CurrentBowStage`) "NewEnumerator5")
    (if (not (> (`GameplayStatics.GetGlobalTimeDilation`) (`self.SlowMo`)))
      (`self.Move Bow` (`self.BowMesh_down`) :!label _label_5)
      (`/Game/00_Lin/Character/BP_MainCharacter.Destroy Slow-Mo PP` (`self.Char_Ref`))
      (`self.StopTimeline`)
      (`GameplayStatics.SetGlobalTimeDilation` 1.0)
      (`self.Reset Cooldown`)
      (set `/Game/00_Lin/CharacterUI/WBP_Crosshair.crosshair_spread` 27.0 (`/Game/00_Lin/Character/BP_MainCharacter.Crosshair` (`self.Char_Ref`)))
      (`/Game/00_Lin/Character/BP_MainCharacter.Reverse Zoom` _char_ref)
      (set `/Game/00_Lin/Character/BP_MainCharacter.TriggerDown` false _char_ref)
      (`KismetSystemLibrary.K2_ClearAndInvalidateTimerHandle` (`self.StrongArrowsTimer`))
      (set `self.StrongArrowAmount` 0.0)
      (set `self.CurrentBowStage` "NewEnumerator0"))
    (else
      (goto _label_5))))

(event `self.ReceiveTick`
  (params (DeltaSeconds :type "Float (single-precision)")))

(event `Strong Bow Throw`
  ;[0 0.7046 1] STRONG BOW THROW
  (`self.Stop Bow Move`)
  (bind _returnvalue (`KismetSystemLibrary.K2_SetTimer` null "StrongThrowArrows" (`self.TimeBetweenShots`) true))
  (set `self.StrongArrowsTimer` _returnvalue))

(event `Close Shift-After`
  (`/Engine/EditorBlueprintResources/StandardMacros.Gate` false :!via `Close`
    (:`Exit`
      (`self.SlowTime`)
      (`self.Close Shift-After`))))

(event `SlowTime`)

(fn `ResetSlowMoWithAim`
  (`self.StopTimeline`)
  (`GameplayStatics.SetGlobalTimeDilation` 1.0)
  (`self.Reset Cooldown`)
  (`KismetSystemLibrary.K2_ClearAndInvalidateTimerHandle` (`self.StrongArrowsTimer`))
  (set `self.StrongArrowAmount` 0.0)
  (set `self.CurrentBowStage` "NewEnumerator0"))

(fn `SetUpArrowColors`
  (bind _asmodular_arrow_static (cast `/Game/00_Lin/Weapon/ModularArrow_static` (`ChildActorComponent.ChildActor` (`self.ChangingArrow`))))
  (bind _asbp_main_character (cast `/Game/00_Lin/Character/BP_MainCharacter` (`GameplayStatics.GetPlayerCharacter` 0)))
  (bind (_craftedarrow1_parameters_name _craftedarrow1_parameters_image _craftedarrow1_parameters_description _craftedarrow1_parameters_baseprojectileparameters _craftedarrow1_parameters_explosionparameters _craftedarrow1_parameters_tipcolor _craftedarrow1_parameters_woodcolor _craftedarrow1_parameters_feathercolor) (break `/Game/00_Lin/Weapon/AmmunitionStats` (`/Game/00_Lin/Character/BP_MainCharacter.CraftedArrow1_parameters` _asbp_main_character)))
  (`/Game/00_Lin/Weapon/ModularArrow_static.ArrowSetup` _asmodular_arrow_static _craftedarrow1_parameters_tipcolor _craftedarrow1_parameters_woodcolor _craftedarrow1_parameters_feathercolor))

(fn `Slow Mo Sound`
  (`/Game/00_Lin/Character/BP_MainCharacter.Create Slow-Mo PP` (`self.Char_Ref`))
  ;[1 0 0.02876] SLOW MO
  (`GameplayStatics.PlaySound2D` null 1.0 1.0 0.0 null null))

(fn `StrongThrowArrows`
  (`self.NoBarrelShoot`)
  (`KismetSystemLibrary.PrintString` "SHOT")
  (`self.ArrowAnimation`)
  (bind _output_get (set `self.StrongArrowAmount` (+ (`self.StrongArrowAmount`) 1.0)))
  (if (> _output_get (`self.StrongArrowAmountMAX`))
    (`KismetSystemLibrary.K2_ClearAndInvalidateTimerHandle` (`self.StrongArrowsTimer`))
    (`/Game/00_Lin/Character/BP_MainCharacter.Throw Bow` (`self.Char_Ref`))
    (set `self.StrongArrowAmount` 0.0)
    (set `/Game/00_Lin/CharacterUI/WBP_Crosshair.crosshair_spread` 27.0 (`/Game/00_Lin/Character/BP_MainCharacter.Crosshair` (`self.Char_Ref`)))))

(fn `UserConstructionScript`
  (`parent.UserConstructionScript`))