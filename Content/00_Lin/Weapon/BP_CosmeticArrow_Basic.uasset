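; Cosmetic arrow actor that shows the look of a given arrow type, with data from DT_Recipes.
; BeginPlay applies mesh and material for the arrow type selected on the player's bow.
; SetUpArrowVariables rebuilds the Niagara effect, sets its colors, then per type toggles visibility, Lightning and Blood parameters, and the extra impulse effect.
; The construction script finds BP_BowNew and styles the existing effect from ArrowType, sharing parts of that branch logic.
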(event `self.ReceiveBeginPlay`
  (bind _staticmesh (`self.StaticMesh`))
  (`parent.ReceiveBeginPlay`)
  (set `self.NiagaraTransform` (`SceneComponent.GetRelativeTransform` (`self.ArrowEffect`)))
  (bind _asbp_main_character (cast `/Game/00_Lin/Character/BP_MainCharacter` (`GameplayStatics.GetPlayerCharacter` 0)))
  (bind _bow_ref_new (`/Game/00_Lin/Character/BP_MainCharacter.Bow Ref New` _asbp_main_character))
  (set `self.Bow Ref New` _bow_ref_new)
  (bind _name (`/Game/00_Lin/Craft/Resorses/BPF_Enums.ArrowID to Name` (`/Game/00_Lin/Weapon/BP_BowNew.Arrow Type` _bow_ref_new)))
  (bind _returnvalue (`|GetDataTableRow` "/Game/00_Lin/Craft/DT_Recipes.DT_Recipes" _name)
    (:`then`
      (bind (_name_2 _damage _effect _image _arrowcrafted _desc _niagara _arrowmesh _arrowmaterial) (break `/Game/00_Lin/Craft/Recipes/S_Recipes` _returnvalue))
      (`StaticMeshComponent.SetStaticMesh` _staticmesh _arrowmesh)
      (`PrimitiveComponent.SetMaterial` _staticmesh 0 _arrowmaterial))))

(event `SetUpArrowVariables`
  (params (Selection :type "/Game/00_Lin/Craft/Recipes/E_ArrowID Enum" :default "NewEnumerator0") (BowRef :type "/Game/00_Lin/Weapon/BP_BowNew Object Reference"))
  (bind _arroweffect (`self.ArrowEffect`))
  (bind _arroweffect_2 (`self.ArrowEffect`))
  (set `self.Bow Ref` BowRef)
  (`ActorComponent.K2_DestroyComponent` (`self.ArrowEffect`))
  (bind _returnvalue (`AddComponent|NODE_AddNiagaraComponent-2` :`RelativeTransform` (`self.NiagaraTransform`)))
  (set `self.ArrowEffect` _returnvalue)
  (bind _name (`/Game/00_Lin/Craft/Resorses/BPF_Enums.ArrowID to Name` Selection))
  (bind _returnvalue_2 (`|GetDataTableRow` "/Game/00_Lin/Craft/DT_Recipes.DT_Recipes" _name)
    (:`then`
      (bind (_name_2 _damage _effect _image _arrowcrafted _desc _niagara _arrowmesh _arrowmaterial _colorbig _colorsmall) (break `/Game/00_Lin/Craft/Recipes/S_Recipes` _returnvalue_2))
      (`NiagaraComponent.SetVariableLinearColor` (`self.ArrowEffect`) "BigColor" _colorbig)
      (`NiagaraComponent.SetVariableLinearColor` (`self.ArrowEffect`) "SmallColor" _colorsmall)
      (switch `/Game/00_Lin/Craft/Recipes/E_ArrowID` Selection
        (:`NewEnumerator0`
          (`SceneComponent.SetVisibility` (`self.ArrowEffect`) false false)
          (`ActorComponent.K2_DestroyComponent` (`self.ImpulseEffect`) :!label _label))
        (:`NewEnumerator3`
          (`SceneComponent.SetVisibility` (`self.ArrowEffect`) true false)
          (`NiagaraComponent.SetVariableFloat` (`self.ArrowEffect`) "Lightning" 1.0 :!label _label_2)
          (goto _label))
        (:`NewEnumerator5`
          (`SceneComponent.SetVisibility` _arroweffect true false :!label _label_3)
          (`NiagaraComponent.SetVariableFloat` _arroweffect "Blood" 0.0 :!label _label_4)
          (`NiagaraComponent.SetVariableFloat` (`self.ArrowEffect`) "Lightning" 0.0)
          (bind _returnvalue_3 (`AddComponent|NODE_AddNiagaraComponent-1` :`RelativeTransform` (`SceneComponent.GetRelativeTransform` (`self.ArrowEffect`))))
          (set `self.ImpulseEffect` _returnvalue_3))
        (:`NewEnumerator6`
          (goto _label_3))
        (:`NewEnumerator7`
          (`SceneComponent.SetVisibility` (`self.ArrowEffect`) true false :!label _label_5)
          (`NiagaraComponent.SetVariableFloat` _arroweffect_2 "Lightning" 0.0 :!label _label_6)
          (`NiagaraComponent.SetVariableFloat` _arroweffect_2 "Blood" 1.0)
          (goto _label))
        (:`NewEnumerator8`
          (goto _label_5))))))

(event `SetUpConstrustion`
  (params (Selection :type "/Game/00_Lin/Craft/Recipes/E_ArrowID Enum" :default "NewEnumerator0"))
  (set `self.ArrowEffect` (`self.ArrowEffect`))
  (bind _name (`/Game/00_Lin/Craft/Resorses/BPF_Enums.ArrowID to Name` Selection))
  (bind _returnvalue (`|GetDataTableRow` "/Game/00_Lin/Craft/DT_Recipes.DT_Recipes" _name)
    (:`then`
      (bind (_name_2 _damage _effect _image _arrowcrafted _desc _niagara _arrowmesh _arrowmaterial _colorbig _colorsmall) (break `/Game/00_Lin/Craft/Recipes/S_Recipes` _returnvalue))
      (`NiagaraComponent.SetVariableLinearColor` (`self.ArrowEffect`) "BigColor" _colorbig)
      (`NiagaraComponent.SetVariableLinearColor` (`self.ArrowEffect`) "SmallColor" _colorsmall)
      (switch `/Game/00_Lin/Craft/Recipes/E_ArrowID` Selection
        (:`NewEnumerator3`
          (goto _label_2))
        (:`NewEnumerator5`
          (goto _label_4))
        (:`NewEnumerator7`
          (goto _label_6))
        (:`NewEnumerator8`
          (goto _label_6))))))

(fn `UserConstructionScript`
  (`parent.UserConstructionScript`)
  (bind _returnvalue (`GameplayStatics.GetActorOfClass` "/Game/00_Lin/Weapon/BP_BowNew.BP_BowNew_C"))
  (set `self.Bow Ref` _returnvalue)
  (`self.SetUpConstrustion` (`self.ArrowType`)))