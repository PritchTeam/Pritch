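; Thrown-bow projectile that spins like a boomerang, homes between enemies and returns to the player, hiding the held bow during flight.
; A bounce sphere gathers living shooter NPCs, and damage overlaps hit each through the hit-points interface, retargeting projectile homing to the next.
; Afterwards it homes back to the player, or self-destructs if a box trace is blocked.
; Catching, stalling or a between-enemy timeout also destroys it, calling the owner's stamina increase.
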(event `self.ReceiveTick`
  (params (DeltaSeconds :type "Float (single-precision)"))
  (bind _bowref (`self.BowRef`))
  (bind _staticmesh (`self.StaticMesh`))
  (bind _owningplayer (`self.OwningPlayer`))
  (bind (_returnvalue_roll _returnvalue_pitch) (`KismetMathLibrary.BreakRotator` (`SceneComponent.K2_GetComponentRotation` _staticmesh)))
  ;[0 1 0.359] Rotate Bow
  (`SceneComponent.K2_AddLocalRotation` _staticmesh (`KismetMathLibrary.MakeRotator` 0.0 (+ _returnvalue_pitch 20.0)) false false)
  (if (<= (`KismetMathLibrary.VSize` (`self.GetVelocity`)) 0.0)
    (set `/Game/00_Lin/Character/BP_MainCharacter.BowProjectile` null _owningplayer)
    (`/Game/00_Lin/Character/BP_MainCharacter.CloseTrace` _owningplayer)
    (set `/Game/00_Lin/Weapon/Old/BP_BowOld.CurrentBowStage` "NewEnumerator8" _bowref)
    (`self.SetActorHiddenInGame` _bowref false)
    (`self.BowDestroy`)))

(event `self.ReceiveBeginPlay`
  ;[1 0.1291 0] Set Bow Reference
  (bind _asbp_main_character (cast `/Game/00_Lin/Character/BP_MainCharacter` (`GameplayStatics.GetPlayerCharacter` 0)))
  (bind _output_get (set `self.BowRef` (`/Game/00_Lin/Character/BP_MainCharacter.BowRef` _asbp_main_character)))
  (`self.SetActorHiddenInGame` _output_get true)
  ;;[1 0 0.02876] BOOMERANG SHOOT
  (`GameplayStatics.PlaySound2D` null 1.0 1.0 0.0 null null)
  (`KismetSystemLibrary.Delay` 0.1)
  (`PrimitiveComponent.SetCollisionResponseToChannel` (`self.DamageCollision`) "ECC_WorldStatic" "ECR_Block"))

(event `Set Hoaming`
  (params (Target :type "Actor Object Reference"))
  ;[1 0.1557 0] Set Hoaming Target
  (`/Engine/EditorBlueprintResources/StandardMacros.DoOnce` false
    (:`Completed`
      (set `ProjectileMovementComponent.HomingTargetComponent` (`Actor.RootComponent` Target) (`self.ProjectileMovement`)))))

(event `Return Hoaming`
  (bind _owningplayer (`self.OwningPlayer`))
  ;[1 0.1682 0] Return Hoaming Player
  (`KismetSystemLibrary.Delay` (`self.ThownBowTimeReturn`))
  (set `ProjectileMovementComponent.HomingTargetComponent` (`Character.CapsuleComponent` _owningplayer) (`self.ProjectileMovement`))
  (set `self.Return` true)
  (set `/Game/00_Lin/Character/BP_MainCharacter.BowProjectile` null _owningplayer)
  (`/Game/00_Lin/Character/BP_MainCharacter.CloseTrace` _owningplayer)
  (`KismetArrayLibrary.Array_Clear` (`self.AlreadyDamagedEnemies`))
  (`KismetArrayLibrary.Array_Clear` (`self.EnemiesToHit`)))

(event `Remove Collision`
  (`KismetSystemLibrary.Delay` 1.0)
  (`PrimitiveComponent.SetCollisionEnabled` (`self.DamageCollision`) "QueryAndPhysics"))

(event `self.BounceCollision.OnComponentBeginOverlap`
  (params (OverlappedComponent :type "PrimitiveComponent Object Reference") (OtherActor :type "Actor Object Reference") (OtherComp :type "PrimitiveComponent Object Reference") (OtherBodyIndex :type Integer) (bFromSweep :type Boolean) (SweepResult :type "HitResult Structure (by ref)"))
  (bind _bouncecollision (`self.BounceCollision`))
  (bind _enemiestohit (`self.EnemiesToHit`))
  (bind _output (`|GetArrayItem` (`self.EnemiesToHit`)))
  (if (<= (`KismetArrayLibrary.Array_Length` (`self.EnemiesToHit`)) 0)
    (`KismetArrayLibrary.Array_Clear` (`self.AlreadyDamagedEnemies`))
    (bind _outactors (`KismetSystemLibrary.ComponentOverlapActors` _bouncecollision (`SceneComponent.K2_GetComponentToWorld` _bouncecollision) (`|MakeArray` "ObjectTypeQuery3" :!type "EObjectTypeQuery Enum") null (`|MakeArray` (`GameplayStatics.GetPlayerCharacter` 0) :!type "Actor Object Reference")))
    (for _array_element _outactors
      (bind _asbp_base_shooter_npc (cast `/Game/00_Sanya/AI/NPCCharacters/BaseNPC/BP_BaseShooterNPC` _array_element))
      (if (not (`/Game/00_Sanya/AI/NPCCharacters/BaseNPC/BP_BaseShooterNPC.IsDead` _asbp_base_shooter_npc))
        (`KismetArrayLibrary.Array_Add` _enemiestohit _array_element)))
    (`/Engine/EditorBlueprintResources/StandardMacros.IsValid` _output
      (:`Is Valid`
        (set `ProjectileMovementComponent.HomingTargetComponent` (`Actor.RootComponent` _output) (`self.ProjectileMovement`))
        (`KismetSystemLibrary.PrintString` (`KismetStringLibrary.Concat_StrStr` "LENGTH OF ENEMIES  " (`KismetStringLibrary.Conv_IntToString` (`KismetArrayLibrary.Array_Length` _enemiestohit))) true true (struct :`R` 0.906802 :`G` 1.0 :`A` 1.0))
        (`SphereComponent.SetSphereRadius` (`self.BounceCollision`) 2000.0 true)))))

(event `ResetSpeed`)

(event `self.ReceiveHit`
  (params (MyComp :type "PrimitiveComponent Object Reference") (Other :type "Actor Object Reference") (OtherComp :type "PrimitiveComponent Object Reference") (bSelfMoved :type Boolean) (HitLocation :type "Vector Structure") (HitNormal :type "Vector Structure") (NormalImpulse :type "Vector Structure") (Hit :type "HitResult Structure (by ref)"))
  (bind _owningplayer (`self.OwningPlayer`))
  (bind (_enemy _failed) (`self.Cast to Target` Other))
  (if _failed
    (if (not (> (`KismetArrayLibrary.Array_Length` (`self.EnemiesToHit`)) 0))
      (`KismetSystemLibrary.Delay` 0.2)
      (set `ProjectileMovementComponent.HomingTargetComponent` (`Character.CapsuleComponent` _owningplayer) (`self.ProjectileMovement`))
      (set `self.Return` true)
      (set `/Game/00_Lin/Character/BP_MainCharacter.BowProjectile` null _owningplayer)
      (`/Game/00_Lin/Character/BP_MainCharacter.CloseTrace` _owningplayer))))

(event `self.DamageCollision.OnComponentBeginOverlap`
  (params (OverlappedComponent :type "PrimitiveComponent Object Reference") (OtherActor :type "Actor Object Reference") (OtherComp :type "PrimitiveComponent Object Reference") (OtherBodyIndex :type Integer) (bFromSweep :type Boolean) (SweepResult :type "HitResult Structure (by ref)"))
  (bind _owningplayer (`self.OwningPlayer`))
  (bind _enemiestohit (`self.EnemiesToHit`))
  (bind _output (`|GetArrayItem` _enemiestohit (`KismetArrayLibrary.Array_LastIndex` _enemiestohit)))
  (if (`self.Return`)
    (`self.Return To Player and Destroy` OtherActor)
    (else
      (cast `/Game/00_Lin/Character/BP_MainCharacter` OtherActor
        (:`CastFailed`
          (`PrimitiveComponent.SetCollisionResponseToChannel` (`self.DamageCollision`) "ECC_WorldStatic" "ECR_Block")
          (bind (_enemy _failed) (`self.Cast to Target` null))
          (if _failed
            (if (`KismetArrayLibrary.Array_Contains` (`self.EnemiesToHit`) OtherActor)
              (`KismetArrayLibrary.Array_Add` (`self.AlreadyDamagedEnemies`) OtherActor)
              (`self.ReciveDamage` OtherActor)
              (`KismetSystemLibrary.K2_ClearAndInvalidateTimerHandle` (`self.BetweenEnemiesTimer`))
              (bind _returnvalue (`KismetSystemLibrary.K2_SetTimer` null "Start Timer" (`self.Timer`)))
              (set `self.BetweenEnemiesTimer` _returnvalue)
              (`KismetArrayLibrary.Array_RemoveItem` (`self.EnemiesToHit`) OtherActor)
              (`/Engine/EditorBlueprintResources/StandardMacros.IsValid` _output
                (:`Is Valid`
                  (set `ProjectileMovementComponent.HomingTargetComponent` (`Actor.RootComponent` _output) (`self.ProjectileMovement`))
                  (`KismetSystemLibrary.PrintString` "POST DELAY")
                  (`PrimitiveComponent.SetCollisionResponseToChannel` (`self.DamageCollision`) "ECC_WorldStatic" "ECR_Overlap"))
                (:`Is Not Valid`
                  (set `self.Return` true)
                  (`SphereComponent.SetSphereRadius` (`self.BounceCollision`) 1200.0 true)
                  (set `/Game/00_Lin/Character/BP_MainCharacter.BowProjectile` null _owningplayer)
                  (`/Game/00_Lin/Character/BP_MainCharacter.CloseTrace` _owningplayer)
                  (set `/Game/00_Lin/Weapon/Old/BP_BowOld.CurrentBowStage` "NewEnumerator8" (`self.BowRef`))
                  (bind _returnvalue_2 (`self.Line Trace For Character`))
                  (if _returnvalue_2
                    (`KismetArrayLibrary.Array_Clear` (`self.AlreadyDamagedEnemies`))
                    (`KismetArrayLibrary.Array_Clear` (`self.EnemiesToHit`))
                    (`self.BowDestroy`)
                    (else
                      (set `ProjectileMovementComponent.HomingTargetComponent` (`Character.CapsuleComponent` (`self.OwningPlayer`)) (`self.ProjectileMovement`)))))))))))))

(event `self.CharacterCol.OnComponentBeginOverlap`
  (params (OverlappedComponent :type "PrimitiveComponent Object Reference") (OtherActor :type "Actor Object Reference") (OtherComp :type "PrimitiveComponent Object Reference") (OtherBodyIndex :type Integer) (bFromSweep :type Boolean) (SweepResult :type "HitResult Structure (by ref)"))
  (bind _owningplayer (`self.OwningPlayer`))
  (bind _bowref (`self.BowRef`))
  (if (`self.Return`)
    (`KismetArrayLibrary.Array_Clear` (`self.AlreadyDamagedEnemies`))
    (`KismetArrayLibrary.Array_Clear` (`self.EnemiesToHit`))
    (cast `/Game/00_Lin/Character/BP_MainCharacter` OtherActor)
    (set `/Game/00_Lin/Character/BP_MainCharacter.BowProjectile` null _owningplayer)
    (`/Game/00_Lin/Character/BP_MainCharacter.CloseTrace` _owningplayer)
    (set `/Game/00_Lin/Weapon/Old/BP_BowOld.CurrentBowStage` "NewEnumerator8" _bowref)
    (`self.SetActorHiddenInGame` _bowref false)
    (`self.BowDestroy`)))

(fn `BowDestroy`
  (`/Game/00_Lin/Character/BP_MainCharacter.Increase Stamina` (`self.OwningPlayer`))
  (`self.K2_DestroyActor`))

(fn `Cast to Target`
  (params (Object :type "Actor Object Reference"))
  (returns (Enemy :type "Actor Object Reference") (failed :type Boolean))
  (bind _aspain_lover_bp (cast `/Game/Trash/Artefacts/PainLover_BP` Object)
    (:`then`
      (return _aspain_lover_bp false))
    (:`CastFailed`
      (bind _asbp_base_shooter_npc (cast `/Game/00_Sanya/AI/NPCCharacters/BaseNPC/BP_BaseShooterNPC` Object)
        (:`then`
          (if (`/Game/00_Sanya/AI/NPCCharacters/BaseNPC/BP_BaseShooterNPC.IsDead` _asbp_base_shooter_npc)
            _
            (else
              (return _asbp_base_shooter_npc false))))
        (:`CastFailed`
          _))
      (return null true))))

(fn `Enemies To Hit Hoam`
  (bind _output (`|GetArrayItem` (`self.EnemiesToHit`)))
  (`/Engine/EditorBlueprintResources/StandardMacros.IsValid` _output
    (:`Is Valid`
      (set `ProjectileMovementComponent.HomingTargetComponent` (`Actor.RootComponent` _output) (`self.ProjectileMovement`)))))

(fn `Line Trace For Character`
  (returns (ReturnValue :type Boolean))
  (bind _returnvalue (`GameplayStatics.GetPlayerCharacter` 0))
  (bind _alreadydamagedenemies (`self.AlreadyDamagedEnemies`))
  (bind (_outhit _returnvalue_2) (`KismetSystemLibrary.BoxTraceSingleForObjects` (`self.K2_GetActorLocation` (`|GetArrayItem` _alreadydamagedenemies (`KismetArrayLibrary.Array_LastIndex` _alreadydamagedenemies))) (`self.K2_GetActorLocation` _returnvalue) (5.0 5.0 5.0) (struct) (`|MakeArray` "ObjectTypeQuery1" :!type "EObjectTypeQuery Enum") false (`|MakeArray` self _returnvalue :!type "Actor Object Reference") "None" true (struct :`R` 1.0 :`A` 1.0) (struct :`G` 1.0 :`A` 1.0) 2.0))
  (return _returnvalue_2))

(fn `ReciveDamage`
  (params (InputObject :type "Object Object Reference"))
  (bind _bowref (`self.BowRef`))
  (`/Engine/EditorBlueprintResources/StandardMacros.IsValid` InputObject
    (:`Is Valid`
      (if (`KismetSystemLibrary.DoesImplementInterface` InputObject "/Game/00_Sanya/AI/Utility/Components/BPI_HitPointsInterface.BPI_HitPointsInterface_C")
        (message `/Game/00_Sanya/AI/Utility/Components/BPI_HitPointsInterface.ReceiveDamage` InputObject (select `bool` (`|EnumEquality` (`/Game/00_Lin/Weapon/Old/BP_BowOld.CurrentBowStage` _bowref) "NewEnumerator5") :`false` (`self.Damage`) :`true` (* (`self.Damage_Strong`) (`/Game/00_Lin/Weapon/Old/BP_BowOld.StrongArrowAmount_HIT` _bowref))))))))

(fn `Return To Player and Destroy`
  (params (Object :type "Object Object Reference"))
  (bind _bowref (`self.BowRef`))
  (bind _asbp_main_character (cast `/Game/00_Lin/Character/BP_MainCharacter` Object)
    (:`then`
      (set `/Game/00_Lin/Weapon/Old/BP_BowOld.CurrentBowStage` "NewEnumerator8" _bowref)
      (set `/Game/00_Lin/Character/BP_MainCharacter.BowProjectile` null _asbp_main_character)
      (`self.SetActorHiddenInGame` _bowref false)
      (`self.BowDestroy`))
    (:`CastFailed`
      (return))))

(fn `Start Timer`
  (`KismetSystemLibrary.PrintString` "TIMER OFF" true true (struct :`R` 1.0 :`G` 0.011522 :`A` 1.0) 10.0)
  (set `/Game/00_Lin/Weapon/Old/BP_BowOld.CurrentBowStage` "NewEnumerator8" (`self.BowRef`))
  (set `/Game/00_Lin/Character/BP_MainCharacter.BowProjectile` null (`self.OwningPlayer`))
  (`self.SetActorHiddenInGame` (`self.BowRef`) false)
  (`self.BowDestroy`))

(fn `UserConstructionScript`)