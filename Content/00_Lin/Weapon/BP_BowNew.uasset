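; Player bow weapon that draws, fires and reloads arrows, with a slow-motion aim and a homing volley.
; Timelines animate bow and arrow while aiming, shrinking the crosshair and building arrow velocity, which sets shot speed and random spread.
; Aiming while falling, sliding or gliding with enough stamina triggers delayed global time dilation, with timelines ignoring it.
; StrongBow loops a timer firing homing arrows at targeted enemies, then calls ThrowBow.
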(event `self.ReceiveBeginPlay`
  (bind _bowmesh (`self.BowMesh`))
  ;[1 1 1] Set Up
  (bind _asbp_main_character (cast `/Game/00_Lin/Character/BP_MainCharacter` (`GameplayStatics.GetPlayerCharacter` 0)))
  (set `self.CharRef` _asbp_main_character)
  (set `self.ArrowDefaultLocation` (`SceneComponent.RelativeLocation` (`self.ArrowMesh`)))
  (set `self.Bow Relative Location` (`SceneComponent.RelativeLocation` _bowmesh))
  (set `self.Bow Relative Rotation` (`SceneComponent.RelativeRotation` _bowmesh)))

(event `Move Bow`
  (bind _strongbowloc (`self.StrongBowLoc`))
  ;[1 0.2982 0.005113] Tilt Bow Anim
  (`TimelineComponent.SetPlayRate` (`self.Bow Aim`) 2.0)
  (bind (_direction _move) (`Timeline|Bow Aim` :!via `PlayFromStart` :!label _label)
    (:`Update`
      (`SceneComponent.K2_SetRelativeLocationAndRotation` (`self.BowMesh`) (`KismetMathLibrary.VLerp` (`self.Bow Relative Location`) (`SceneComponent.RelativeLocation` _strongbowloc) _move) (`KismetMathLibrary.RLerp` (`self.Bow Relative Rotation`) (`SceneComponent.RelativeRotation` _strongbowloc) _move true) false false)
      (`/Game/00_Lin/CharacterUI/Crosshair/WBP_RoundCrosshair.ChangeRadius` (`/Game/00_Lin/Character/BP_MainCharacter.RoundCrosshair` (`self.CharRef`)) (`KismetMathLibrary.Lerp` 1.0 0.2 _move)))))

(event `Stop Bow Move`
  ;[1 0.2982 0.005113] Tilt Bow Anim
  (goto _label :!via `Reverse`))

(event `Aim`
  (params (`Trigger Down` :type Boolean))
  ;[1 1 1] Aim
  (if `Trigger Down`
    (set `self.Aiming` true)
    (`self.Move Bow`)
    (`self.Move Arrow`)
    (`self.Can Slow-mo?`)
    (set `self.Current Bow Stage` "NewEnumerator0")
    (else
      (set `self.Aiming` false)
      (`self.Stop Aim`)
      (`self.Shoot Arrow` false)
      (`self.Arrow Animation`)
      (`NiagaraFunctionLibrary.SpawnSystemAtLocation` "/Game/00_Lin/VFX/Character/StaminaVFX/NS_CoinBurst.NS_CoinBurst" (`SceneComponent.K2_GetComponentLocation` (`self.NiagaraSpark`))))))

(event `Move Arrow`
  ;[1 0.3634 0] Aim Arrow Anim
  (`TimelineComponent.SetPlayRate` (`self.Arrow Aim`) 2.0)
  (bind (_direction _move) (`Timeline|Arrow Aim` :!via `PlayFromStart`)
    (:`Update`
      (`SceneComponent.K2_SetRelativeLocation` (`self.ArrowMesh`) (`KismetMathLibrary.VLerp` (`self.ArrowDefaultLocation`) (`SceneComponent.RelativeLocation` (`self.StrongArrowLoc`)) _move) false false)
      (set `self.Arrow Velocity` (`KismetMathLibrary.Lerp` 500.0 (`self.Arrow Velocity Max`) _move)))))

(event `Stop Aim`
  ;[1 1 1] Reset Settings
  (`self.Stop Bow Move`)
  (`/Game/00_Lin/CharacterUI/Crosshair/WBP_RoundCrosshair.ReturnRadius` (`/Game/00_Lin/Character/BP_MainCharacter.RoundCrosshair` (`self.CharRef`)))
  (`self.Stop Slow Mo`)
  (set `self.Current Bow Stage` "NewEnumerator10"))

(event `Stop Slow Mo`
  ;[1 1 1] Reset Settings
  (`KismetSystemLibrary.K2_ClearAndInvalidateTimerHandle` (`self.Slow Mo Timer`))
  (`GameplayStatics.SetGlobalTimeDilation` 1.0)
  (set `SpringArmComponent.bEnableCameraRotationLag` true (`/Game/00_Lin/Character/BP_MainCharacter.BowSpringArm` (`self.CharRef`))))

(event `Arrow Animation`
  (bind _arrowmesh (`self.ArrowMesh`))
  ;[1 0.3905 0] Load Arrow Anim
  (set `self.Arrow In?` false)
  (`SceneComponent.SetVisibility` _arrowmesh false false)
  (`SceneComponent.K2_SetRelativeLocation` (`self.ArrowMesh`) (`SceneComponent.RelativeLocation` (`self.LoadArrowLoc`)) false false)
  (`KismetSystemLibrary.Delay` 0.2)
  (`SceneComponent.SetVisibility` _arrowmesh true false)
  (`TimelineComponent.SetPlayRate` (`self.Load Arrow`) 3.0)
  (bind (_direction _move) (`Timeline|Load Arrow` :!via `PlayFromStart`)
    (:`Update`
      (`SceneComponent.K2_SetRelativeLocation` (`self.ArrowMesh`) (`KismetMathLibrary.VLerp` (`SceneComponent.RelativeLocation` (`self.ArrowMesh`)) (`self.ArrowDefaultLocation`) _move) false false)
      (set `self.Arrow In?` true))))

(event `Shoot Arrow`
  (params (`Is homing?` :type Boolean))
  (bind _arrow_spread (`self.Arrow Spread`))
  (bind _arrow_velocity (`self.Arrow Velocity`))
  (bind _returnvalue (* _arrow_spread -1.0))
  (bind _aim1 (`/Game/00_Lin/Character/BP_MainCharacter.Aim1` (`self.CharRef`)))
  (bind _returnvalue_2 (`SceneComponent.K2_GetComponentLocation` _aim1))
  ;[1 1 1] Spawn Arrow
  (if `Is homing?`
    (`self.Homing Set Up` null)
    (else
      (`|SpawnActorFromClass` "/Game/00_Lin/Weapon/BP_ProjectileArrow.BP_ProjectileArrow_C" (`KismetMathLibrary.MakeTransform` (`KismetMathLibrary.SelectVector` (+ _returnvalue_2 (`KismetMathLibrary.MakeVector` (`KismetMathLibrary.RandomFloatInRange` _returnvalue _arrow_spread) (`KismetMathLibrary.RandomFloatInRange` _returnvalue _arrow_spread) (`KismetMathLibrary.RandomFloatInRange` _returnvalue _arrow_spread))) _returnvalue_2 (< _arrow_velocity 5000.0)) (`SceneComponent.K2_GetComponentRotation` _aim1)) "Undefined" "OverrideRootScale" null (`KismetMathLibrary.SelectFloat` (* _arrow_velocity 2.0) (* _arrow_velocity 5.0) (< _arrow_velocity 4000.0)) null))))

(event `Start Slow-mo`
  (bind _charref (`self.CharRef`))
  ;[0.429 1 0.01729] Slow Mo
  (`GameplayStatics.SetGlobalTimeDilation` (`self.Slow Mo`))
  (set `Actor.CustomTimeDilation` 1.0 (`self.CharRef`))
  (`TimelineComponent.SetIgnoreTimeDilation` (`self.Bow Aim`) true)
  (`TimelineComponent.SetIgnoreTimeDilation` (`self.Arrow Aim`) true)
  (`TimelineComponent.SetIgnoreTimeDilation` (`self.Load Arrow`) true)
  (`TimelineComponent.SetIgnoreTimeDilation` (`/Game/00_Lin/Character/BP_MainCharacter.Zoom` (`self.CharRef`)) true)
  (set `SpringArmComponent.bEnableCameraRotationLag` false (`/Game/00_Lin/Character/BP_MainCharacter.BowSpringArm` (`self.CharRef`)))
  (`TimelineComponent.SetIgnoreTimeDilation` (`/Game/00_Lin/Character/BP_MainCharacter.Slow Mo Timer` _charref) true)
  (`/Game/00_Lin/Character/BP_MainCharacter.Open Tick Slow Mo` _charref))

(event `Can Slow-mo?`
  (bind _charref (`self.CharRef`))
  ;[0.429 1 0.01729] Slow Mo
  (if (>= (`/Game/00_Lin/Character/BP_MainCharacter.Stamina` _charref) (`/Game/00_Lin/Character/BP_MainCharacter.Slide Stamina` _charref))
    (if (or (`NavMovementComponent.IsFalling` (`Character.CharacterMovement` (`self.CharRef`))) (`self.Is Sliding`) (`self.Is Gliding`))
      (bind _returnvalue (`KismetSystemLibrary.K2_SetTimerDelegate` (delegate `Start Slow-mo`) 0.2))
      (set `self.Slow Mo Timer` _returnvalue))))

(event `Strong Bow`
  ;[1 1 1] Strong Arrow Throw
  (bind _returnvalue (`KismetSystemLibrary.K2_SetTimer` null "StrongThrowArrows" (`self.Time Between Shots`) true))
  (set `self.Strong Arrows Timer` _returnvalue))

(fn `Homing Set Up`
  (params (Arrow :type "/Game/00_Lin/Weapon/BP_ProjectileArrow Object Reference"))
  (bind _targeted_enemies (`/Game/00_Lin/Character/BP_MainCharacter.Targeted Enemies` (`self.CharRef`)))
  (bind _aim1 (`/Game/00_Lin/Character/BP_MainCharacter.Aim1` (`self.CharRef`)))
  (bind _returnvalue (/ (`KismetMathLibrary.Round` (`self.Strong Arrow Amount`)) 2))
  (bind _returnvalue_2 (`|SpawnActorFromClass` "/Game/00_Lin/Weapon/BP_ProjectileArrow.BP_ProjectileArrow_C" (`KismetMathLibrary.MakeTransform` (`SceneComponent.K2_GetComponentLocation` _aim1) (`SceneComponent.K2_GetComponentRotation` _aim1)) "Undefined" "OverrideRootScale" null 100.0 null))
  (if (== (`KismetArrayLibrary.Array_Length` _targeted_enemies) 1)
    (bind _projectilemovement (`/Game/00_Lin/Weapon/BP_ProjectileArrow.ProjectileMovement` _returnvalue_2))
    (set `ProjectileMovementComponent.HomingTargetComponent` (`/Game/00_Sanya/AI/NPCCharacters/BaseNPC/BP_BaseShooterNPC.Sphere1` (`|GetArrayItem` _targeted_enemies)) _projectilemovement)
    (set `ProjectileMovementComponent.HomingAccelerationMagnitude` 100000.0 _projectilemovement)
    (else
      (`KismetSystemLibrary.PrintString` (`KismetStringLibrary.Conv_IntToString` _returnvalue) true true (struct :`R` 0.751891 :`G` 1.0 :`A` 1.0))
      (bind _projectilemovement_2 (`/Game/00_Lin/Weapon/BP_ProjectileArrow.ProjectileMovement` _returnvalue_2))
      (set `ProjectileMovementComponent.HomingTargetComponent` (`/Game/00_Sanya/AI/NPCCharacters/BaseNPC/BP_BaseShooterNPC.Sphere1` (`|GetArrayItem` _targeted_enemies _returnvalue)) _projectilemovement_2)
      (set `ProjectileMovementComponent.HomingAccelerationMagnitude` 100000.0 _projectilemovement_2))))

(fn `StrongThrowArrows`
  (set `self.Arrow Velocity` (`self.Arrow Velocity Max`))
  (`self.Shoot Arrow` true)
  (`self.Arrow Animation`)
  (bind _output_get (set `self.Strong Arrow Amount` (+ (`self.Strong Arrow Amount`) 1.0)))
  (if (> _output_get (`self.Strong Arrow Amount MAX`))
    (`KismetSystemLibrary.K2_ClearAndInvalidateTimerHandle` (`self.Strong Arrows Timer`))
    (`/Game/00_Lin/Character/BP_MainCharacter.Throw Bow` (`self.CharRef`))
    (set `self.Strong Arrow Amount` 0.0)))

(fn `UserConstructionScript`)