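; Stamina bar actor that displays the player character's stamina through a dynamic material on its Bar component.
; Tick feeds the clamped stamina ratio to UpdateBar, which accumulates drops into a BottomProgress segment that shrinks over time.
; StaminaAnim plays a timeline pulsing the background red at low stamina.
; The low-stamina top-color bounce lerps identical colors, and the Niagara decrease effect is unwired.
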(event `DecreaseNiagara`)

(event `self.ReceiveBeginPlay`
  (set `self.CustomTimeDilation` 1.0)
  (bind _returnvalue (`KismetMaterialLibrary.CreateDynamicMaterialInstance` (`self.MatInst`)))
  (bind _output_get (set `self.DynamicInst` _returnvalue))
  (`PrimitiveComponent.SetMaterial` (`self.Bar`) 0 _output_get))

(event `self.ReceiveTick`
  (params (DeltaSeconds :type "Float (single-precision)"))
  (set `self.CustomTimeDilation` 2.0)
  (bind _asbp_main_character (cast `/Game/00_Lin/Character/BP_MainCharacter` (`GameplayStatics.GetPlayerCharacter` 0)))
  (bind _stamina (`/Game/00_Lin/Character/BP_MainCharacter.Stamina` _asbp_main_character))
  (`self.UpdateBar` (`KismetMathLibrary.FClamp` (/ (`KismetMathLibrary.Conv_IntToDouble` _stamina) (`KismetMathLibrary.Conv_IntToDouble` (`/Game/00_Lin/Character/BP_MainCharacter.MAX Stamina` _asbp_main_character)))) DeltaSeconds)
  (if (< _stamina 500)
    (`/Engine/EditorBlueprintResources/StandardMacros.DoOnce` false :!label _label
      (:`Completed`
        (bind (_direction _value) (`Timeline|BounceColor` :!via `PlayFromStart` :!label _label_2)
          (:`Update`
            (`MaterialInstanceDynamic.SetVectorParameterValue` (`self.DynamicInst`) "TopColor" (`KismetMathLibrary.LinearColorLerp` (struct :`G` 0.226966 :`B` 0.327778 :`A` 1.0) (struct :`G` 0.226966 :`B` 0.327778 :`A` 1.0) _value)))
          (:`Finished`
            (goto _label :!via `Reset`)))))
    (else
      (`|ExecutionSequence`
        (:`then_0`
          (goto _label_2 :!via `Stop`))
        (:`then_1`
          (`MaterialInstanceDynamic.SetVectorParameterValue` (`self.DynamicInst`) "TopColor" (struct :`G` 0.226966 :`B` 0.327778 :`A` 1.0)))))))

(event `StaminaAnim`
  (bind (_direction _value) (`Timeline|RedPulsation` :!via `PlayFromStart`)
    (:`Update`
      (if (> (`/Game/00_Lin/Character/BP_MainCharacter.Stamina` (stale `self.ReceiveTick` _asbp_main_character)) 300)
        (`MaterialInstanceDynamic.SetVectorParameterValue` :`self` (`self.DynamicInst`) :`ParameterName` "BackgroundColor" :!label _label_3)
        (else
          (`MaterialInstanceDynamic.SetVectorParameterValue` (`self.DynamicInst`) "BackgroundColor" (`KismetMathLibrary.LinearColorLerp` (struct :`R` 1.0 :`G` 0.019814 :`A` 1.0) (struct) _value)))))
    (:`Finished`
      (goto _label_3))))

(fn `UpdateBar`
  (params (TopProgress :type "Float (double-precision)") (DeltaSeconds :type "Float (double-precision)"))
  (set `self.BottomProgress` (+ (`self.BottomProgress`) (* (- (`local.TopProgress`) (`self.PrevTopProgress`)) -1.0)))
  (set `self.PrevTopProgress` (`local.TopProgress`))
  (`MaterialInstanceDynamic.SetScalarParameterValue` (`self.DynamicInst`) "TopProgress" (`local.TopProgress`))
  (`MaterialInstanceDynamic.SetScalarParameterValue` (`self.DynamicInst`) "BottomProgress" (`self.BottomProgress`))
  (set `self.BottomProgress` (`KismetMathLibrary.FClamp` (- (`self.BottomProgress`) (* (`local.DeltaSeconds`) (`self.AnimSpeed`))) 0.0 (`self.BottomProgress`))))

(fn `UserConstructionScript`)