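; BP_HealthBarActor is an actor that displays the player character's health on a bar with a trailing change effect.
; BeginPlay puts a dynamic material instance on the Bar component.
; Each Tick clamps the ratio of BP_MainCharacter's MAXHP to MAXHPProgress and passes it to UpdateBar as TopProgress.
; UpdateBar adds any drop to BottomProgress, sends both values to the material, then shrinks BottomProgress toward zero at AnimSpeed.
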(event `self.ReceiveBeginPlay`
  (set `self.CustomTimeDilation` 1.0)
  (bind _returnvalue (`KismetMaterialLibrary.CreateDynamicMaterialInstance` (`self.MatInst`)))
  (bind _output_get (set `self.DynamicInst` _returnvalue))
  (`PrimitiveComponent.SetMaterial` (`self.Bar`) 0 _output_get))

(event `self.ReceiveTick`
  (params (DeltaSeconds :type "Float (single-precision)"))
  (bind _asfirst_person_character (cast `/Game/00_Lin/Character/BP_MainCharacter` (`GameplayStatics.GetPlayerCharacter` 0)))
  (`self.UpdateBar` (`KismetMathLibrary.FClamp` (/ (`KismetMathLibrary.Conv_IntToDouble` (`/Game/00_Lin/Character/BP_MainCharacter.MAX HP` _asfirst_person_character)) (`KismetMathLibrary.Conv_IntToDouble` (`/Game/00_Lin/Character/BP_MainCharacter.MAX HP(progress)` _asfirst_person_character)))) DeltaSeconds))

(fn `UpdateBar`
  (params (TopProgress :type "Float (double-precision)") (DeltaSeconds :type "Float (double-precision)"))
  (set `self.BottomProgress` (+ (`self.BottomProgress`) (* (- (`local.TopProgress`) (`self.PrevTopProgress`)) -1.0)))
  (set `self.PrevTopProgress` (`local.TopProgress`))
  (`MaterialInstanceDynamic.SetScalarParameterValue` (`self.DynamicInst`) "TopProgress" (`local.TopProgress`))
  (`MaterialInstanceDynamic.SetScalarParameterValue` (`self.DynamicInst`) "BottomProgress" (`self.BottomProgress`))
  (set `self.BottomProgress` (`KismetMathLibrary.FClamp` (- (`self.BottomProgress`) (* (`local.DeltaSeconds`) (`self.AnimSpeed`))) 0.0 (`self.BottomProgress`))))

(fn `UserConstructionScript`)