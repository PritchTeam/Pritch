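; BP_VectorCamera is a racing camera actor that flies a camera along a spline path.
; MoveGhostCamera plays a timeline that moves the camera from the spline's start to its end in world space, caching each position as GhostLocation.
; When the timeline finishes, it passes that last position to the player's BP_RacingKlin through LerpCameraPos, non-reversed, to hand off the camera move.
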(event `MoveGhostCamera`
  (bind _spline (`self.Spline`))
  (bind (_direction _lerp) (`Timeline|Timeline`)
    (:`Update`
      (bind _returnvalue (`SplineComponent.GetLocationAtDistanceAlongSpline` _spline (`KismetMathLibrary.Lerp` 0.0 (`SplineComponent.GetSplineLength` _spline) _lerp) "World"))
      (`SceneComponent.K2_SetWorldLocation` (`self.Camera`) _returnvalue false false)
      (set `self.GhostLocation` _returnvalue))
    (:`Finished`
      (bind _asbp_racing_klin (cast `/Game/00_Lin/Racing/BP_RacingKlin` (`GameplayStatics.GetPlayerCharacter` 0)))
      (`/Game/00_Lin/Racing/BP_RacingKlin.LerpCameraPos` _asbp_racing_klin (`self.GhostLocation`) false))))

(fn `UserConstructionScript`)