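; One-shot trigger volume for the racing mode that switches BP_RacingKlin to a new spline and camera.
; On box overlap it hands its Spline to the racer and, if a Camera is set, makes it current, calls MoveGhostCamera and lerps the racer's camera to the ghost location.
; It then destroys itself and calls AutomaticallyMove on the racer.
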(event `self.Box.OnComponentBeginOverlap`
  (params (OverlappedComponent :type "PrimitiveComponent Object Reference") (OtherActor :type "Actor Object Reference") (OtherComp :type "PrimitiveComponent Object Reference") (OtherBodyIndex :type Integer) (bFromSweep :type Boolean) (SweepResult :type "HitResult Structure (by ref)"))
  (bind _camera (`self.Camera`))
  (bind _asbp_racing_klin (cast `/Game/00_Lin/Racing/BP_RacingKlin` OtherActor))
  (set `/Game/00_Lin/Racing/BP_RacingKlin.Spline` (`self.Spline`) _asbp_racing_klin)
  (`/Engine/EditorBlueprintResources/StandardMacros.IsValid` (`self.Camera`)
    (:`Is Valid`
      (set `/Game/00_Lin/Racing/BP_RacingKlin.CurrentCamera` _camera _asbp_racing_klin)
      (`/Game/00_Lin/Racing/BP_VectorCamera.MoveGhostCamera` _camera)
      (`/Game/00_Lin/Racing/BP_RacingKlin.LerpCameraPos` _asbp_racing_klin (`/Game/00_Lin/Racing/BP_VectorCamera.GhostLocation` _camera) false))
    (:`Is Not Valid`
      _))
  (`self.K2_DestroyActor`)
  (`/Game/00_Lin/Racing/BP_RacingKlin.AutomaticallyMove` _asbp_racing_klin))

(fn `UserConstructionScript`)