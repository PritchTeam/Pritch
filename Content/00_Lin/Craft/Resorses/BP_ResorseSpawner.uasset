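; Resource spawner actor that scatters BP_Resorse pickups around itself on BeginPlay.
; For each ID and count in ResorsesToSpawn, it looks up the DT_Resorses row and sets up each spawned actor, re-rolling its position once if overlapping.
; Positions come from Visibility line traces starting at random points in a flat box sized by SpawnerRadius.
; A radius-scaled DebugSphere marks the center and is destroyed after spawning.
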(event `self.ReceiveBeginPlay`
  (`self.Activate Spawn`)
  (`ActorComponent.K2_DestroyComponent` (`self.DebugSphere`)))

(event `Activate Spawn`
  (bind _resorsestospawn (`self.ResorsesToSpawn`))
  (bind _keys (`BlueprintMapLibrary.Map_Keys` _resorsestospawn))
  (for _array_element _keys
    (bind _namerow (`/Game/00_Lin/Craft/Resorses/BPF_Enums.Resorse IDto Name` _array_element))
    (bind _returnvalue (`|GetDataTableRow` "/Game/00_Lin/Craft/Resorses/DT_Resorses.DT_Resorses" _namerow)
      (:`then`
        (for _ (range 1 (+ (`BlueprintMapLibrary.Map_Find` _resorsestospawn _array_element) 1))
          (bind _impactpoint (`self.Find Random Point`))
          (bind _returnvalue_2 (`|SpawnActorFromClass` "/Game/00_Lin/Craft/Resorses/BP_Resorse.BP_Resorse_C" (`KismetMathLibrary.MakeTransform` _impactpoint) "Undefined" "OverrideRootScale" null null))
          ;[1 1 1] fix this ltr
          (`/Game/00_Lin/Craft/Resorses/BP_Resorse.SetUpResorse` _returnvalue_2 _returnvalue _array_element (2.0 2.0 2.0))
          (if (`PrimitiveComponent.IsOverlappingActor` (`/Game/00_Lin/Craft/Resorses/BP_Resorse.Collision` _returnvalue_2) null)
            (bind _impactpoint_2 (`self.Find Random Point`))
            (`self.K2_SetActorLocation` _returnvalue_2 _impactpoint_2 false false)))))))

(fn `Find Random Point`
  (returns (ImpactPoint :type "Vector Structure"))
  (bind _returnvalue (* (`self.SpawnerRadius`) 50.0))
  (bind _returnvalue_2 (`KismetMathLibrary.RandomPointInBoundingBox` (`SceneComponent.K2_GetComponentLocation` (`self.DebugSphere`)) (`KismetMathLibrary.MakeVector` _returnvalue _returnvalue 0.5)))
  (bind _outhit (`KismetSystemLibrary.LineTraceSingle` _returnvalue_2 (+ _returnvalue_2 (* _returnvalue_2 (0.0 0.0 5.0))) "TraceTypeQuery1"))
  (return (`.ImpactPoint` (`GameplayStatics.BreakHitResult` _outhit))))

(fn `UserConstructionScript`
  (bind _debugsphere (`self.DebugSphere`))
  (`SceneComponent.SetWorldScale3D` _debugsphere (* (`SceneComponent.K2_GetComponentScale` _debugsphere) (`self.SpawnerRadius`))))