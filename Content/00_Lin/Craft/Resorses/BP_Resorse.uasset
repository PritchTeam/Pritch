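; BP_Resorse is a crafting resource pickup with a mesh and a widget that turns toward the player every tick.
; SetUpResorse applies the mesh from the resource struct, a scale and a fixed crystal material, and stores the struct and enum ID.
; Logic for magnet pull and collection into BP_MainCharacter's inventory is disconnected, so both begin-overlap events do nothing.
; Leaving the magnet collision only clears the Magnet flag.
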(event `self.ReceiveTick`
  (params (DeltaSeconds :type "Float (single-precision)"))
  (`SceneComponent.K2_SetWorldRotation` (`self.Widget`) (`KismetMathLibrary.FindLookAtRotation` (`self.K2_GetActorLocation`) (`self.K2_GetActorLocation` (`GameplayStatics.GetPlayerCharacter` 0))) false false))

(event `self.MagnetCollision.OnComponentEndOverlap`
  (params (OverlappedComponent :type "PrimitiveComponent Object Reference") (OtherActor :type "Actor Object Reference") (OtherComp :type "PrimitiveComponent Object Reference") (OtherBodyIndex :type Integer))
  (set `self.Magnet` false))

(event `self.MagnetCollision.OnComponentBeginOverlap`
  (params (OverlappedComponent :type "PrimitiveComponent Object Reference") (OtherActor :type "Actor Object Reference") (OtherComp :type "PrimitiveComponent Object Reference") (OtherBodyIndex :type Integer) (bFromSweep :type Boolean) (SweepResult :type "HitResult Structure (by ref)")))

(event `self.Collision.OnComponentBeginOverlap`
  (params (OverlappedComponent :type "PrimitiveComponent Object Reference") (OtherActor :type "Actor Object Reference") (OtherComp :type "PrimitiveComponent Object Reference") (OtherBodyIndex :type Integer) (bFromSweep :type Boolean) (SweepResult :type "HitResult Structure (by ref)")))

(event `ReturnToNormal`)

(fn `SetUpResorse`
  (params (ResorseStruct :type "/Game/00_Lin/Craft/Resorses/S_Resourses Structure") (EnumID :type "/Game/00_Lin/Craft/Resorses/E_ResourseID Enum" :default "NewEnumerator2") (NewScale :type "Vector Structure"))
  (bind _resorsemesh (`self.ResorseMesh`))
  (`StaticMeshComponent.SetStaticMesh` _resorsemesh (`.Mesh_22_795E82DC408E6FE5BC79188B6F4A11B5` (break `/Game/00_Lin/Craft/Resorses/S_Resourses` ResorseStruct)))
  (`SceneComponent.SetWorldScale3D` _resorsemesh NewScale)
  (set `self.ResorseStructure` ResorseStruct)
  (set `self.Enum ID` EnumID)
  (`PrimitiveComponent.SetMaterial` (`self.ResorseMesh`) 0 "/Game/0000_Pritch/02_Assets/3D_Assets/Crystals/CrystalMat_Inst1.CrystalMat_Inst1"))

(fn `UserConstructionScript`)