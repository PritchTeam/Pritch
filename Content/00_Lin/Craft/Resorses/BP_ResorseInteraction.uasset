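; BP_ResorseInteraction is a one-time resource pickup that grants resources to the main character's inventory.
; Entering its box caches the character and enables a per-tick check for the interact key.
; On a press, it loops through its ResorsesToGive map, validates each ID against DT_Resorses, calls the inventory component's CollectResorse once per unit, then marks itself depleted.
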(event `self.ReceiveTick`
  (params (DeltaSeconds :type "Float (single-precision)"))
  (if (`self.OpenTick?`)
    (if (`PlayerController.WasInputKeyJustPressed` (`GameplayStatics.GetPlayerController` 0) (`self.InteractKey`))
      (if (not (`self.Depleted?`))
        (set `self.OpenTick?` false)
        (`self.AddResorses`)))))

(event `self.Box.OnComponentBeginOverlap`
  (params (OverlappedComponent :type "PrimitiveComponent Object Reference") (OtherActor :type "Actor Object Reference") (OtherComp :type "PrimitiveComponent Object Reference") (OtherBodyIndex :type Integer) (bFromSweep :type Boolean) (SweepResult :type "HitResult Structure (by ref)"))
  (bind _asbp_main_character (cast `/Game/00_Lin/Character/BP_MainCharacter` OtherActor))
  (set `self.As BP Main Character` _asbp_main_character)
  (set `self.OpenTick?` true))

(event `AddResorses`
  (bind _resorsestogive (`self.ResorsesToGive`))
  (bind _keys (`BlueprintMapLibrary.Map_Keys` _resorsestogive))
  (for _array_element _keys
    (bind _namerow (`/Game/00_Lin/Craft/Resorses/BPF_Enums.Resorse IDto Name` _array_element))
    (`|GetDataTableRow` "/Game/00_Lin/Craft/Resorses/DT_Resorses.DT_Resorses" _namerow
      (:`then`
        (for _ (range 1 (+ (`BlueprintMapLibrary.Map_Find` _resorsestogive _array_element) 1))
          (`/Game/00_Lin/Craft/Resorses/AC_Inventory.CollectResorse` (`/Game/00_Lin/Character/BP_MainCharacter.AC_Inventory` (`self.As BP Main Character`)) _array_element)))))
  (set `self.Depleted?` true))

(fn `UserConstructionScript`)