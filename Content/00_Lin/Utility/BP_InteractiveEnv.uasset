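; BP_InteractiveEnv is an interactive environment actor whose death effect sends an electrical shock to nearby shooter NPCs.
; DeathEffect adds a BP_SphereOverlap child actor to find BP_BaseShooterNPCs within a large radius.
; Each target gets a Niagara ribbon stretched from this actor and random damage through its HealthComponent.
; ReceiveDamage only returns false and DeathOutput is empty; nothing in this graph calls DeathEffect.
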(event `self.ReceiveBeginPlay`)

(event `DeathEffect`
  (bind _returnvalue (`AddComponent|NODE_AddChildActorComponent-0`))
  (bind _asbp_sphere_overlap (cast `/Game/00_Sanya/AI/Utility/GeneralAITools/BP_SphereOverlap` (`ChildActorComponent.ChildActor` _returnvalue)))
  (bind _actors (`/Game/00_Sanya/AI/Utility/GeneralAITools/BP_SphereOverlap.GetOverlappedActors` _asbp_sphere_overlap "/Game/00_Sanya/AI/NPCCharacters/BaseNPC/BP_BaseShooterNPC.BP_BaseShooterNPC_C" 2000.0))
  (for _array_element _actors
    (bind _asbp_base_shooter_npc (cast `/Game/00_Sanya/AI/NPCCharacters/BaseNPC/BP_BaseShooterNPC` _array_element))
    (bind _returnvalue_2 (`NiagaraFunctionLibrary.SpawnSystemAtLocation` "/Game/00_Lin/VFX/Explosion/NS_ElectricalRibbon.NS_ElectricalRibbon" (`self.K2_GetActorLocation`) (struct) (1.0 1.0 1.0) false))
    (`FXSystemComponent.SetVectorParameter` _returnvalue_2 "UserEnd" (`self.K2_GetActorLocation` _asbp_base_shooter_npc))
    (`/Game/00_Sanya/AI/Utility/Components/BP_HealthComponent.DamageCalculation` :`self` (`/Game/00_Sanya/AI/NPCCharacters/BaseNPC/BP_BaseShooterNPC.HealthComponent` _asbp_base_shooter_npc) :`IncomingDamage` (`KismetMathLibrary.RandomIntegerInRange` 20 100))))

(event `/Game/00_Sanya/AI/Utility/Components/BPI_HitPointsInterface.DeathOutput`)

(fn `ReceiveDamage`
  (params (IncomingDamage :type Integer) (BoneName :type Name) (HitLoc :type "Vector Structure") (Hit :type "HitResult Structure") (ArrowActor :type "Actor Object Reference"))
  (returns (DidInteract :type Boolean))
  (return false))

(fn `UserConstructionScript`)