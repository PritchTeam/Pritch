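; Electrical interactive box that starts an electrical fog effect when damaged and sets off an electric explosion with sound on death.
; On death it also runs a lightning strike, using a temporary BP_SphereOverlap child actor to find shooter NPCs within a large radius.
; Each NPC found gets a ribbon effect drawn from the box to its location and takes random damage through its HealthComponent.
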(event `LightningStrike`
  (bind _returnvalue (`AddComponent|NODE_AddChildActorComponent-0`))
  (set `self.NewVar` _returnvalue)
  (bind _asbp_sphere_overlap (cast `/Game/00_Sanya/AI/Utility/GeneralAITools/BP_SphereOverlap` (`ChildActorComponent.ChildActor` _returnvalue)))
  (bind _actors (`/Game/00_Sanya/AI/Utility/GeneralAITools/BP_SphereOverlap.GetOverlappedActors` _asbp_sphere_overlap "/Game/00_Sanya/AI/NPCCharacters/BaseNPC/BP_BaseShooterNPC.BP_BaseShooterNPC_C" 2000.0))
  (for _array_element _actors
    (bind _asbp_base_shooter_npc (cast `/Game/00_Sanya/AI/NPCCharacters/BaseNPC/BP_BaseShooterNPC` _array_element))
    (bind _returnvalue_2 (`NiagaraFunctionLibrary.SpawnSystemAtLocation` "/Game/00_Lin/VFX/Explosion/NS_ElectricalRibbon.NS_ElectricalRibbon" (`self.K2_GetActorLocation`)))
    (`FXSystemComponent.SetVectorParameter` _returnvalue_2 "UserEnd" (`self.K2_GetActorLocation` _asbp_base_shooter_npc))
    (`/Game/00_Sanya/AI/Utility/Components/BP_HealthComponent.DamageCalculation` :`self` (`/Game/00_Sanya/AI/NPCCharacters/BaseNPC/BP_BaseShooterNPC.HealthComponent` _asbp_base_shooter_npc) :`IncomingDamage` (`KismetMathLibrary.RandomIntegerInRange` 20 100) :`ArrowType` "NewEnumerator3")
    (`KismetSystemLibrary.PrintString` (`KismetSystemLibrary.GetDisplayName` _asbp_base_shooter_npc) true true (struct :`R` 0.033676 :`B` 1.0 :`A` 1.0)))
  (`ActorComponent.K2_DestroyComponent` (`self.NewVar`)))

(event `/Game/00_Sanya/AI/Utility/Components/BPI_HitPointsInterface.DeathOutput`
  (`self.DeathEffect`)
  (`NiagaraFunctionLibrary.SpawnSystemAtLocation` "/Game/00_Lin/VFX/Explosion/NS_ExplosionElectrisity.NS_ExplosionElectrisity" (`self.K2_GetActorLocation`))
  (`ActorComponent.K2_DestroyComponent` (`self.Fog`))
  (`self.LightningStrike`)
  (`GameplayStatics.SpawnSoundAtLocation` "/Game/00_Anton/Sounds/SoundDesign/Shooter_Sounds/Environment_Sounds/Arrows/A_Sh_PLR_CMBT_Arrows_ElectricExplosion_Cue.A_Sh_PLR_CMBT_Arrows_ElectricExplosion_Cue" (`self.K2_GetActorLocation`) (struct) 1.0 1.0 0.0 null null))

(event `/Game/00_Sanya/AI/Utility/Components/BPI_HitPointsInterface.DamageOutput`
  (params (DamageTaken :type Integer) (CurrentHitPoints :type Integer) (BoneName :type Name) (VelocityVector :type "Vector Structure"))
  (`/Engine/EditorBlueprintResources/StandardMacros.IsValid` (`self.Fog`)
    (:`Is Not Valid`
      (bind _returnvalue (`NiagaraFunctionLibrary.SpawnSystemAtLocation` "/Game/00_Lin/VFX/Explosion/NS_ElectricalFog.NS_ElectricalFog" (`self.K2_GetActorLocation`)))
      (set `self.Fog` _returnvalue))))

(fn `UserConstructionScript`
  (`parent.UserConstructionScript`))