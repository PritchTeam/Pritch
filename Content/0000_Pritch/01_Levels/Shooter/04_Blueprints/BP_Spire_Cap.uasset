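; BP_Spire_Cap is a one-shot closing piece in the Shooter level that moves into place and blocks passage once the player triggers it.
; When the player character first overlaps the Collision component, it records the mesh's location and waits briefly.
; The Close timeline then lerps the mesh by AddVector without sweeping.
; The Blocker component, non-colliding from BeginPlay, gains full collision when the movement finishes.
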(event `self.ReceiveBeginPlay`
  (`PrimitiveComponent.SetCollisionEnabled` (`self.Blocker`) "NoCollision"))

(event `self.Collision.OnComponentBeginOverlap`
  (params (OverlappedComponent :type "PrimitiveComponent Object Reference") (OtherActor :type "Actor Object Reference") (OtherComp :type "PrimitiveComponent Object Reference") (OtherBodyIndex :type Integer) (bFromSweep :type Boolean) (SweepResult :type "HitResult Structure (by ref)"))
  (if (== OtherActor (`GameplayStatics.GetPlayerCharacter` 0))
    (`/Engine/EditorBlueprintResources/StandardMacros.DoOnce` false
      (:`Completed`
        (set `self.Location` (`SceneComponent.K2_GetComponentLocation` (`self.StaticMeshComponent`)))
        (`KismetSystemLibrary.Delay` 0.5)
        (bind (_direction _newtrack_0) (`Timeline|Close` :!via `PlayFromStart`)
          (:`Update`
            (`SceneComponent.K2_SetWorldLocation` (`self.StaticMeshComponent`) (`KismetMathLibrary.VLerp` (`self.Location`) (+ (`self.Location`) (`self.AddVector`)) _newtrack_0) false false))
          (:`Finished`
            (`PrimitiveComponent.SetCollisionEnabled` (`self.Blocker`) "QueryAndPhysics")))))))

(fn `UserConstructionScript`)