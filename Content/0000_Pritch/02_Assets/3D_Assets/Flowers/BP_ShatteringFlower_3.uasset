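; Flower actor that shatters and disappears when the player overlaps its Sphere or DeathOutput fires.
; Construction applies a shared dynamic material to its static meshes; at BeginPlay, those under the Sphere become physics-only.
; Shattering enables physics on these pieces and applies a radial impulse, while a timeline fades material opacity before destroying the actor.
; ReceiveDamage only returns false.
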(event `Spawn`
  (bind _output_get (set `self.Components` (`SceneComponent.GetChildrenComponents` (`self.Sphere`) true)))
  (for _array_element _output_get
    (bind _asstatic_mesh_component (cast `StaticMeshComponent` _array_element))
    (`PrimitiveComponent.SetCollisionEnabled` _asstatic_mesh_component "PhysicsOnly")))

(event `self.ReceiveBeginPlay`
  (`self.Spawn`))

(event `/Game/00_Sanya/AI/Utility/Components/BPI_HitPointsInterface.DeathOutput`
  (`|ExecutionSequence` :!label _label
    (:`then_0`
      (for _array_element (`self.Components`)
        (bind _asstatic_mesh_component (cast `StaticMeshComponent` _array_element))
        (`PrimitiveComponent.SetSimulatePhysics` _asstatic_mesh_component true)
        (`PrimitiveComponent.SetMassScale` _asstatic_mesh_component "None" 3.0)
        (`PrimitiveComponent.AddRadialImpulse` _asstatic_mesh_component (`SceneComponent.K2_GetComponentLocation` (`self.DefaultSceneRoot`)) 1000.0 1000000.0 "RIF_Linear" false)))
    (:`then_1`
      (`KismetSystemLibrary.Delay` 0.1)
      (bind (_direction _newtrack_0) (`Timeline|Fade`)
        (:`Update`
          (`MaterialInstanceDynamic.SetScalarParameterValue` (`self.Material`) "Opacity" _newtrack_0))
        (:`Finished`
          (`KismetSystemLibrary.Delay` 0.1)
          (`self.K2_DestroyActor`))))))

(event `self.Sphere.OnComponentBeginOverlap`
  (params (OverlappedComponent :type "PrimitiveComponent Object Reference") (OtherActor :type "Actor Object Reference") (OtherComp :type "PrimitiveComponent Object Reference") (OtherBodyIndex :type Integer) (bFromSweep :type Boolean) (SweepResult :type "HitResult Structure (by ref)"))
  (if (== OtherActor (`GameplayStatics.GetPlayerCharacter` 0))
    (goto _label)))

(fn `ReceiveDamage`
  (params (IncomingDamage :type Integer) (BoneName :type Name) (HitLoc :type "Vector Structure") (Hit :type "HitResult Structure") (ArrowActor :type "Actor Object Reference"))
  (returns (DidInteract :type Boolean))
  (return false))

(fn `UserConstructionScript`
  (`/Engine/EditorBlueprintResources/StandardMacros.DoOnce` false
    (:`Completed`
      (`KismetArrayLibrary.Array_Clear` (`self.Components`))
      (bind _output_get (set `self.Components` (`SceneComponent.GetChildrenComponents` (`self.DefaultSceneRoot`) true)))
      (bind _returnvalue (`KismetMaterialLibrary.CreateDynamicMaterialInstance` "/Game/0000_Pritch/02_Assets/3D_Assets/Grass/M_Grass_FlowerMaster_1.M_Grass_FlowerMaster_1"))
      (set `self.Material` _returnvalue)
      (for _array_element _output_get
        (bind _asstatic_mesh_component (cast `StaticMeshComponent` _array_element))
        (`PrimitiveComponent.SetMaterial` _asstatic_mesh_component 0 (`self.Material`))))))